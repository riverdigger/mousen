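; BP_Spell_Volley is a timed area spell that deals damage over time and slows what enters its mesh, then destroys itself after its lifespan.
; On overlap, the entering actor's BP_PC_Mousen instigator controller starts tick damage, crediting player controller 0, and stops it on exit.
; Actors implementing I_Status_Slow also receive a timed slow message, sent only on the server.
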(event OnComponentBeginOverlap(StaticMesh)
  (params (OverlappedComponent :type Primitive%20Component%20Object%20Reference) (OtherActor :type Actor%20Object%20Reference) (OtherComp :type Primitive%20Component%20Object%20Reference) (OtherBodyIndex :type Integer) (bFromSweep :type Boolean) (SweepResult :type Hit%20Result%20Structure%20%28by%20ref%29))
  (bind _asbp_pc_mousen (Utilities|Casting|CastToBP_PC_Mousen (Game|GetInstigatorController OtherActor)))
  (Default|ApplyTickDamage _asbp_pc_mousen OtherActor (Variables|Default|GetDamage) (Variables|Default|GetTickRate) (Variables|Default|GetAs%20BP%20PC%20Mousen) (Variables|Default|GetInstigator))
  (if (Utilities|DoesObjectImplementInterface OtherActor "/Game/Spells/StatusEffects/I_Status_Slow.I_Status_Slow_C")
    (if (Networking|IsServer)
      (Class|IStatusSlow|OnSlowed(Message) OtherActor (Variables|Default|GetSlowStatusEffect) (Variables|Default|GetSlowLifespan) (Variables|Default|GetSlowAmount)))))

(event OnComponentEndOverlap(StaticMesh)
  (params (OverlappedComponent :type Primitive%20Component%20Object%20Reference) (OtherActor :type Actor%20Object%20Reference) (OtherComp :type Primitive%20Component%20Object%20Reference) (OtherBodyIndex :type Integer))
  (bind _asbp_pc_mousen (Utilities|Casting|CastToBP_PC_Mousen (Game|GetInstigatorController OtherActor)))
  (Default|StopTickDamage _asbp_pc_mousen))

(event EventBeginPlay
  (bind _asbp_pc_mousen (Utilities|Casting|CastToBP_PC_Mousen (Game|GetPlayerController 0)))
  (Variables|Default|SetAs%20BP%20PC%20Mousen _asbp_pc_mousen)
  (Utilities|FlowControl|Delay (Variables|Default|GetLifespan))
  (Actor|DestroyActor))

(fn ConstructionScript)