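; BP_Spell_Shield is a shield spell actor; its graphs handle only lifetime cleanup, with no shield effect logic.
; On BeginPlay it caches player controller 0 as BP_PC_Mousen and the instigator's BP_PS_Mousen player state.
; ServerBindings hooks that controller's player-state reset event to CleanupResources, which destroys the actor.
; The movement and projectile movement component getters are empty stubs.
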(event Custom|CleanupResources
  (Actor|DestroyActor))

(event Custom|Server%20Bindings
  (EventDispatchers|BindEventtoPSPlayerReset (Variables|Default|GetAs%20BP%20PC%20Mousen) (delegate Custom|CleanupResources)))

(event EventBeginPlay
  (bind _asbp_pc_mousen (Utilities|Casting|CastToBP_PC_Mousen (Game|GetPlayerController 0)))
  (Variables|Default|SetAs%20BP%20PC%20Mousen _asbp_pc_mousen)
  (Variables|Default|SetAs%20BP%20PS%20Mousen (.AsBP%20PS%20Mousen (Utilities|Casting|CastToBP_PS_Mousen (Variables|/Script/Engine.Pawn|GetPlayerState (Variables|Default|GetInstigator)))))
  (CallFunction|ServerBindings))

(fn ConstructionScript)

(fn GetMovementComponent
  (return 0))

(fn GetProjectileMovementComponent
  (return 0))