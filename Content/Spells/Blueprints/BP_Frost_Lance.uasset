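; Frost Lance spell projectile that damages enemy-team actors on direct hit and in an expanding burst.
; It breaks on impact or after a travel timer scaled by the caster's reach modifier, hiding meshes, playing Niagara, then destroying itself.
; A timeline grows the burst sphere, whose damage scales inversely with distance.
; Damage is server-only and once per actor; other projectiles receive a collision message instead of breaking it.
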(event OnSystemFinished(Niagara)
  (params (PSystem :type Niagara%20Component%20Object%20Reference))
  (Actor|DestroyActor))

(event OnComponentBeginOverlap(Sphere)
  (params (OverlappedComponent :type Primitive%20Component%20Object%20Reference) (OtherActor :type Actor%20Object%20Reference) (OtherComp :type Primitive%20Component%20Object%20Reference) (OtherBodyIndex :type Integer) (bFromSweep :type Boolean) (SweepResult :type Hit%20Result%20Structure%20%28by%20ref%29))
  (if (and (!= OtherActor (Variables|Default|GetInstigator)) (!= OtherActor self))
    (if (Utilities|DoesObjectImplementInterface OtherActor "/Game/ThirdPerson/Blueprints/Gameplay/I_Damage.I_Damage_C")
      (if (!= (Math|Conversions|ToInteger(Byte) (Variables|/Game/ThirdPerson/Blueprints/Gameplay/BP_PS_Mousen.BP_PS_Mousen_C|GetPlayerTeam (.AsBP%20PS%20Mousen (Utilities|Casting|CastToBP_PS_Mousen (Variables|/Script/Engine.Pawn|GetPlayerState (Variables|Default|GetInstigator)))))) (Math|Conversions|ToInteger(Byte) (Variables|/Game/ThirdPerson/Blueprints/Gameplay/BP_PS_Mousen.BP_PS_Mousen_C|GetPlayerTeam (.AsBP%20PS%20Mousen (Utilities|Casting|CastToBP_PS_Mousen (Variables|/Script/Engine.Pawn|GetPlayerState (.AsBP%20Third%20Person%20Character (Utilities|Casting|CastToBP_ThirdPersonCharacter OtherActor))))))))
        (if (Networking|IsServer)
          (if (not (Utilities|Array|ContainsItem (Variables|Default|GetHitActors) OtherActor))
            (CallFunction|ServerApplyDamage :DamagedActor OtherActor :Damage (Variables|Default|GetDamage) :Instigated%20By (Variables|Default|GetAs%20BP%20PC%20Mousen) :DamageCauser (Variables|Default|GetInstigator) :Damage%20Type%20Class "/Script/Engine.DamageType")
            (Utilities|Array|AddUnique (Variables|Default|GetHitActors) OtherActor)
            (CallFunction|BreakSelf))))
      (elif (Utilities|DoesObjectImplementInterface OtherActor "/Game/ThirdPerson/Blueprints/Gameplay/I_Projectile.I_Projectile_C")
        (Class|IProjectile|ApplyCollision(Message) OtherActor self (Variables|Default|GetProjectileMovement))
        (else
          (CallFunction|BreakSelf))))))

(event OnComponentBeginOverlap(ExpandingSphere)
  (params (OverlappedComponent :type Primitive%20Component%20Object%20Reference) (OtherActor :type Actor%20Object%20Reference) (OtherComp :type Primitive%20Component%20Object%20Reference) (OtherBodyIndex :type Integer) (bFromSweep :type Boolean) (SweepResult :type Hit%20Result%20Structure%20%28by%20ref%29))
  (if (and (!= OtherActor (Variables|Default|GetInstigator)) (!= OtherActor self))
    (if (Utilities|DoesObjectImplementInterface OtherActor "/Game/ThirdPerson/Blueprints/Gameplay/I_Damage.I_Damage_C")
      (if (!= (Math|Conversions|ToInteger(Byte) (Variables|/Game/ThirdPerson/Blueprints/Gameplay/BP_PS_Mousen.BP_PS_Mousen_C|GetPlayerTeam (.AsBP%20PS%20Mousen (Utilities|Casting|CastToBP_PS_Mousen (Variables|/Script/Engine.Pawn|GetPlayerState (Variables|Default|GetInstigator)))))) (Math|Conversions|ToInteger(Byte) (Variables|/Game/ThirdPerson/Blueprints/Gameplay/BP_PS_Mousen.BP_PS_Mousen_C|GetPlayerTeam (.AsBP%20PS%20Mousen (Utilities|Casting|CastToBP_PS_Mousen (Variables|/Script/Engine.Pawn|GetPlayerState (.AsBP%20Third%20Person%20Character (Utilities|Casting|CastToBP_ThirdPersonCharacter OtherActor))))))))
        (if (Networking|IsServer)
          (if (not (Utilities|Array|ContainsItem (Variables|Default|GetHitActors) OtherActor))
            (CallFunction|ServerApplyDamage :DamagedActor OtherActor :Damage (* (/ (/ 1.9e+02 (Transformation|GetDistanceTo OtherActor self)) 2.0) (Variables|Default|GetDamage)) :Instigated%20By (Variables|Default|GetAs%20BP%20PC%20Mousen) :DamageCauser (Variables|Default|GetInstigator) :Damage%20Type%20Class "/Script/Engine.DamageType")
            (Utilities|Array|AddUnique (Variables|Default|GetHitActors) OtherActor)))))))

(event Custom|Server%20Apply%20Damage
  (params (DamagedActor :type Actor%20Object%20Reference) (Damage :type Float%20%28double-precision%29) (Hit%20Direction :type Vector) (Hit%20Info :type Hit%20Result%20Structure) (Instigated%20By :type Controller%20Object%20Reference) (DamageCauser :type Actor%20Object%20Reference) (Damage%20Type%20Class :type Damage%20Type%20Class%20Reference))
  (Default|ApplyPointDamage (Variables|Default|GetAs%20BP%20PC%20Mousen) DamagedActor Damage Hit%20Direction Hit%20Info Instigated%20By DamageCauser Damage%20Type%20Class))

(event Custom|Expand%20Sphere
  (bind _scale (Timeline|Expand%20Sphere%20Timeline PlayFromStart)
    (:Update
      (Transformation|SetWorldScale3D (Variables|Default|GetExpandingSphere) (Math|Vector|MakeVector _scale _scale _scale)))))

(event Custom|Break%20Self
  (bind _niagara (Variables|Default|GetNiagara))
  (bind _staticmesh (Variables|Default|GetStaticMesh))
  (if (not (Variables|Default|GetAlreadyBroken?))
    (Collision|SetCollisionEnabled (Variables|Default|GetSphere) "NoCollision")
    (Components|Movement|StopMovementImmediately (Variables|Default|GetProjectileMovement))
    (Utilities|FlowControl|Sequence
      (:then_0
        (Utilities|IsValid _staticmesh
          (:Is%20Valid
            (Components|DestroyComponent _staticmesh)
            (Components|DestroyComponent (Variables|Default|GetStaticMesh1))
            (Components|DestroyComponent (Variables|Default|GetStaticMesh2)))))
      (:then_1
        (Utilities|IsValid _niagara
          (:Is%20Valid
            (Components|Activation|Activate _niagara true))))
      (:then_2
        (CallFunction|ExpandSphere)))))

(event EventBeginPlay
  (bind _asbp_pc_mousen (Utilities|Casting|CastToBP_PC_Mousen (Game|GetPlayerController 0)))
  (Variables|Default|SetAs%20BP%20PC%20Mousen _asbp_pc_mousen)
  (Variables|Default|SetAs%20BP%20Third%20Person%20Magic (.AsBP%20Third%20Person%20Magic (Utilities|Casting|CastToBP_ThirdPerson_Magic (Variables|Default|GetInstigator))))
  (Utilities|IsValid (Variables|/Game/ThirdPerson/Blueprints/Magic/BP_ThirdPerson_Magic.BP_ThirdPerson_Magic_C|GetSpellSpawn (Variables|Default|GetAs%20BP%20Third%20Person%20Magic))
    (:Is%20Valid
      (Utilities|Time|SetTimerbyEvent (delegate Custom|Break%20Self) (* (Variables|Default|GetTravelTime) (Variables|/Game/ThirdPerson/Blueprints/Gameplay/BP_PS_Mousen.BP_PS_Mousen_C|GetFireballReachModifier (.AsBP%20PS%20Mousen (Utilities|Casting|CastToBP_PS_Mousen (Variables|/Script/Engine.Pawn|GetPlayerState (Variables|Default|GetInstigator))))))))))

(event EventFinishCollision
  (params (Collided%20With :type Actor%20Object%20Reference))
  (Components|Movement|StopMovementImmediately (Variables|Default|GetProjectileMovement))
  (Actor|DestroyActor))

(event EventDisableCollision
  (params (Delay :type Float%20%28double-precision%29))
  (Variables|Default|SetAlreadyBroken? true)
  (Collision|SetCollisionEnabled (Variables|Default|GetSphere) "NoCollision")
  (Collision|SetCollisionEnabled (Variables|Default|GetExpandingSphere) "NoCollision")
  (Utilities|FlowControl|Delay Delay)
  (Class|IProjectile|FinishCollision(Message) self))

(fn ConstructionScript)

(fn GetMovementComponent
  (return 0))

(fn GetProjectileMovement
  (return 0))

(fn GetProjectileMovementComponent
  (return 0))