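; Shield spell actor that orbits a shield mesh around its Instigator while spinning to face outward along its forward vector.
; Each Tick places it at a set distance from the Instigator and advances its yaw by the full-rotation time and direction.
; When the OwnerShield reports destruction, a timeline drives the mesh's Color Intensity material parameter and the actor destroys itself after a short delay.
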(event Custom|CleanupResources
  (CallFunction|ServerUpdateColor)
  (Utilities|FlowControl|Delay 0.1)
  (Actor|DestroyActor))

(event Custom|Server%20Bindings
  (EventDispatchers|BindEventtoShieldDestroyed (Variables|Default|GetOwnerShield) (delegate Custom|CleanupResources)))

(event Custom|Server%20Update%20Color
  (bind _alpha (Timeline|Timeline PlayFromStart)
    (:Update
      (Rendering|Material|SetScalarParameterValueonMaterials (Variables|Default|GetShieldMesh) "Color Intensity" _alpha))))

(event EventBeginPlay
  (CallFunction|ServerBindings))

(event EventTick
  (params (DeltaSeconds :type Float%20%28single-precision%29))
  (Transformation|SetActorLocation (+ (Transformation|GetActorLocation (Variables|Actor|GetInstigator)) (* (Math|Vector|Normalize (Transformation|GetActorForwardVector)) (Variables|Default|GetDistanceFromCenter))) false false)
  (Transformation|AddActorLocalRotation (Math|Rotator|MakeRotator 0.0 0.0 (* (* (/ 3.6e+02 (Variables|Default|GetTimeToRotateFully)) DeltaSeconds) (Variables|Default|GetDirection))) false false))

(fn ConstructionScript)