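; Tremors spell actor that emits a repeating ground pulse, slowing enemy-team characters it overlaps.
; One timeline scales the actor outward, then a second animates the material's HeightFalloff before shrinking and disabling it until a timer restarts the cycle.
; While enabled, overlaps skip the instigator and teammates, and the server sends a slow status to targets implementing I_Status_Invincible.
; It destroys itself when the instigator dies or the player state resets.
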(event OnComponentBeginOverlap(StaticMesh)
  (params (OverlappedComponent :type Primitive%20Component%20Object%20Reference) (OtherActor :type Actor%20Object%20Reference) (OtherComp :type Primitive%20Component%20Object%20Reference) (OtherBodyIndex :type Integer) (bFromSweep :type Boolean) (SweepResult :type Hit%20Result%20Structure%20%28by%20ref%29))
  (if (Variables|Default|GetEnabled?)
    (if (not (== OtherActor (Variables|Default|GetInstigator)))
      (if (not (== (Math|Conversions|ToInteger(Byte) (Variables|/Game/ThirdPerson/Blueprints/Gameplay/BP_PS_Mousen.BP_PS_Mousen_C|GetPlayerTeam (.AsBP%20PS%20Mousen (Utilities|Casting|CastToBP_PS_Mousen (Variables|/Script/Engine.Pawn|GetPlayerState (.AsBP%20Third%20Person%20Character (Utilities|Casting|CastToBP_ThirdPersonCharacter OtherActor))))))) (Math|Conversions|ToInteger(Byte) (Variables|/Game/ThirdPerson/Blueprints/Gameplay/BP_PS_Mousen.BP_PS_Mousen_C|GetPlayerTeam (.AsBP%20PS%20Mousen (Utilities|Casting|CastToBP_PS_Mousen (Variables|/Script/Engine.Pawn|GetPlayerState (Variables|Default|GetInstigator))))))))
        (if (Utilities|DoesObjectImplementInterface OtherActor "/Game/Spells/StatusEffects/Interfaces/I_Status_Invincible.I_Status_Invincible_C")
          (if (Networking|IsServer)
            (Class|IStatusSlow|OnSlowed(Message) OtherActor "/Game/Spells/StatusEffects/Blueprints/BP_Status_Effect_Slowed.BP_Status_Effect_Slowed_C" 2.0 (Variables|Default|GetSlowAmount))))))))

(event Custom|CleanupResources
  (Actor|DestroyActor))

(event Custom|Server%20Bindings
  (EventDispatchers|BindEventtoPSPlayerReset (Variables|Default|GetAs%20BP%20PC%20Mousen) (delegate Custom|CleanupResources))
  (EventDispatchers|BindEventtoPlayerDied (.AsBP%20Third%20Person%20Character (Utilities|Casting|CastToBP_ThirdPersonCharacter (Variables|Default|GetInstigator))) (delegate Custom|CleanupResources)))

(event Custom|Server%20Pulse%20Outwards
  (Rendering|Material|SetScalarParameterValueonMaterials (Variables|Default|GetStaticMesh) "HeightFalloff" 1.0)
  (bind _alpha (Timeline|Timeline PlayFromStart)
    (:Update
      (Transformation|SetActorScale3D self (Math|Vector|Lerp(Vector) (Variables|Default|GetStartScale) (Variables|Default|GetEndScale) _alpha)))
    (:Finished
      (CallFunction|ServerDisable))))

(event Custom|Server%20Restart%20Pulse
  (Variables|Default|SetEnabled? true)
  (CallFunction|ServerPulseOutwards))

(event Custom|ServerDisable
  (bind _alpha (Timeline|Disable PlayFromStart)
    (:Update
      (Rendering|Material|SetScalarParameterValueonMaterials (Variables|Default|GetStaticMesh) "HeightFalloff" _alpha))
    (:Finished
      (Variables|Default|SetEnabled? false)
      (Transformation|SetActorScale3D self "0.010000,0.010000,0.010000")
      (Utilities|Time|SetTimerbyEvent (delegate Custom|Server%20Restart%20Pulse) 3.0))))

(event EventBeginPlay
  (bind _asbp_pc_mousen (Utilities|Casting|CastToBP_PC_Mousen (Game|GetPlayerController 0)))
  (Variables|Default|SetAs%20BP%20PC%20Mousen _asbp_pc_mousen)
  (CallFunction|ServerPulseOutwards)
  (CallFunction|ServerBindings))

(fn ConstructionScript)