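; Protection dome spell actor that makes its caster and/or teammates invincible while inside, depending on its targeting flags.
; On mesh overlap, the server sends eligible actors an invincible status through I_Status_Invincible and tracks them in AffectedActors.
; Leaving the dome removes the status, and the caster leaving destroys the dome.
; It also expires after its Lifespan, clearing the status from remaining affected actors when destroyed.
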(event OnComponentBeginOverlap(StaticMesh)
  (params (OverlappedComponent :type Primitive%20Component%20Object%20Reference) (OtherActor :type Actor%20Object%20Reference) (OtherComp :type Primitive%20Component%20Object%20Reference) (OtherBodyIndex :type Integer) (bFromSweep :type Boolean) (SweepResult :type Hit%20Result%20Structure%20%28by%20ref%29))
  (if (== OtherActor (Variables|Default|GetInstigator))
    (if (Variables|Default|GetAffectsCaster?)
      (if (Utilities|DoesObjectImplementInterface OtherActor "/Game/Spells/StatusEffects/Interfaces/I_Status_Invincible.I_Status_Invincible_C") :!label _label
        (if (Networking|IsServer)
          (Class|IStatusInvincible|OnInvincible(Message) OtherActor "/Game/Spells/StatusEffects/Blueprints/BP_Status_Effect_Invincible.BP_Status_Effect_Invincible_C" (Variables|Default|GetInvincibleLifespan))
          (Utilities|Array|AddUnique (Variables|Default|GetAffectedActors) OtherActor))))
    (elif (== (Math|Conversions|ToInteger(Byte) (Variables|/Game/ThirdPerson/Blueprints/Gameplay/BP_PS_Mousen.BP_PS_Mousen_C|GetPlayerTeam (.AsBP%20PS%20Mousen (Utilities|Casting|CastToBP_PS_Mousen (Variables|/Script/Engine.Pawn|GetPlayerState (.AsBP%20Third%20Person%20Character (Utilities|Casting|CastToBP_ThirdPersonCharacter OtherActor))))))) (Math|Conversions|ToInteger(Byte) (Variables|/Game/ThirdPerson/Blueprints/Gameplay/BP_PS_Mousen.BP_PS_Mousen_C|GetPlayerTeam (.AsBP%20PS%20Mousen (Utilities|Casting|CastToBP_PS_Mousen (Variables|/Script/Engine.Pawn|GetPlayerState (Variables|Default|GetInstigator)))))))
      (if (Variables|Default|GetAffectsTeammates?)
        (goto _label)))))

(event OnComponentEndOverlap(StaticMesh)
  (params (OverlappedComponent :type Primitive%20Component%20Object%20Reference) (OtherActor :type Actor%20Object%20Reference) (OtherComp :type Primitive%20Component%20Object%20Reference) (OtherBodyIndex :type Integer))
  (bind _returnvalue (Utilities|Array|RemoveItem (Variables|Default|GetAffectedActors) OtherActor))
  (if _returnvalue
    (Class|IStatusInvincible|OnUnInvincible(Message) OtherActor "/Game/Spells/StatusEffects/Blueprints/BP_Status_Effect_Invincible.BP_Status_Effect_Invincible_C")
    (if (== OtherActor (Variables|Default|GetInstigator))
      (Actor|DestroyActor))))

(event EventDestroyed
  (for _array_element (Variables|Default|GetAffectedActors)
    (Class|IStatusInvincible|OnUnInvincible(Message) _array_element "/Game/Spells/StatusEffects/Blueprints/BP_Status_Effect_Invincible.BP_Status_Effect_Invincible_C")))

(event EventBeginPlay
  (bind _asbp_pc_mousen (Utilities|Casting|CastToBP_PC_Mousen (Game|GetPlayerController 0)))
  (Variables|Default|SetAs%20BP%20PC%20Mousen _asbp_pc_mousen)
  (Utilities|FlowControl|Delay (Variables|Default|GetLifespan))
  (Actor|DestroyActor))

(fn ConstructionScript)