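; Frozen Orb spell actor that marks the spot where a launched orb stops and becomes a storm.
; On authority at BeginPlay, it spawns BP_Spell_Frozen_Orb_Movement at its owner's location, aimed at itself.
; When that projectile overlaps the Sphere, it halts, attaches to this actor and enables its storm.
; Sphere collision is switched off, and both actors are destroyed after Lifetime.
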(event OnComponentBeginOverlap(Sphere)
  (params (OverlappedComponent :type Primitive%20Component%20Object%20Reference) (OtherActor :type Actor%20Object%20Reference) (OtherComp :type Primitive%20Component%20Object%20Reference) (OtherBodyIndex :type Integer) (bFromSweep :type Boolean) (SweepResult :type Hit%20Result%20Structure%20%28by%20ref%29))
  (bind _frozenorbmovementactor (Variables|Default|GetFrozenOrbMovementActor))
  ;[1 1 1] When Orb hits something
  (if (== OtherActor _frozenorbmovementactor)
    (Components|Movement|StopMovementImmediately (Variables|/Game/Spells/Blueprints/BP_Spell_Frozen_Orb_Movement.BP_Spell_Frozen_Orb_Movement_C|GetProjectileMovement _frozenorbmovementactor))
    (Collision|SetCollisionEnabled (Variables|Default|GetSphere) "NoCollision")
    (Transformation|AttachActorToActor OtherActor self "None" "KeepWorld" "KeepWorld" "KeepWorld" true)
    (Default|EnableStorm (Variables|Default|GetFrozenOrbMovementActor))
    (Utilities|FlowControl|Delay (Variables|Default|GetLifetime))
    (Actor|DestroyActor OtherActor)
    (Actor|DestroyActor)))

(event EventBeginPlay
  (bind _returnvalue (Components|GetOwner))
  (bind _returnvalue_2 (Transformation|GetActorLocation _returnvalue))
  (Networking|SwitchHasAuthority
    (:Authority
      (bind _returnvalue_3 (Game|SpawnActorfromClass "/Game/Spells/Blueprints/BP_Spell_Frozen_Orb_Movement.BP_Spell_Frozen_Orb_Movement_C" (Math|Transform|MakeTransform _returnvalue_2 (Math|Rotator|FindLookatRotation _returnvalue_2 (Transformation|GetActorLocation)) "1.000000,1.000000,1.000000") "Undefined" self (Variables|Default|GetInstigator)))
      (Variables|Default|SetFrozenOrbMovementActor _returnvalue_3))))

(fn ConstructionScript)