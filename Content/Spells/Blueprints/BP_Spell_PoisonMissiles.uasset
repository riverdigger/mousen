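; Poison Missiles spell actor that launches a staggered volley of missiles from its instigator's location.
; On BeginPlay it reads the player state's chunky-missile flag, choosing one chunky missile or six regular ones, and sets its lifespan.
; Only the server runs the delayed DoN loop, which calls a spawn event with randomized, roughly upward pitch for each missile.
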(event Custom|Server%20Spawn%20Spell%20Missile
  (params (SpawnTransform :type Transform) (Chunky? :type Boolean))
  (Game|SpawnActorfromClass (select Chunky? "/Game/Spells/Blueprints/BP_Spell_Chunky_Missile.BP_Spell_Chunky_Missile_C" "/Game/Spells/Blueprints/BP_Spell_Missile.BP_Spell_Missile_C") SpawnTransform "Undefined" 0 (Variables|Default|GetInstigator)))

(event EventBeginPlay
  (bind _asbp_pc_mousen (Utilities|Casting|CastToBP_PC_Mousen (Game|GetPlayerController 0)))
  (Variables|Default|SetAs%20BP%20PC%20Mousen _asbp_pc_mousen)
  (Variables|Default|SetAs%20BP%20PS%20Mousen (.AsBP%20PS%20Mousen (Utilities|Casting|CastToBP_PS_Mousen (Variables|/Script/Engine.Pawn|GetPlayerState (Variables|Default|GetInstigator)))))
  (Variables|Default|SetN (Math|Integer|SelectInt 1 6 (Variables|/Game/ThirdPerson/Blueprints/Gameplay/BP_PS_Mousen.BP_PS_Mousen_C|GetHasChunkyMissile? (Variables|Default|GetAs%20BP%20PS%20Mousen))))
  (Transformation|SetActorRotation (Math|Rotator|FindLookatRotation (Transformation|GetActorLocation) (Transformation|GetActorForwardVector (Variables|Default|GetInstigator))))
  (Actor|SetLifeSpan (Variables|Default|GetLifespan))
  (if (Networking|IsServer)
    (Utilities|FlowControl|DoN (Variables|Default|GetN) :!label _label
      (:Exit
        (CallFunction|ServerSpawnSpellMissile (Math|Transform|MakeTransform (Transformation|GetActorLocation (Variables|Default|GetInstigator)) (Math|Rotator|MakeRotator 0.0 (Math|Random|RandomFloatinRange 1.1e+02 7e+01) 0.0) "1.000000,1.000000,1.000000") (Variables|/Game/ThirdPerson/Blueprints/Gameplay/BP_PS_Mousen.BP_PS_Mousen_C|GetHasChunkyMissile? (Variables|Default|GetAs%20BP%20PS%20Mousen)))
        (Utilities|FlowControl|Delay 0.1)
        (goto _label)))))

(fn ConstructionScript)

(fn GetMovementComponent
  (return 0))

(fn GetProjectileMovementComponent
  (return 0))