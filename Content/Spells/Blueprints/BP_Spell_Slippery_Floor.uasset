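; BP_Spell_Slippery_Floor is a spell actor that applies the Charmed status to enemy players who begin overlapping its collision.
; The overlap skips the Instigator, requires the I_Status_Charmed interface and compares PlayerState teams before sending the charm message.
; Charm duration is a base time plus the target's, not the caster's, PacifyCharmedDuration.
; On BeginPlay it binds to player controller 0's PlayerState reset event to destroy itself.
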(event OnComponentBeginOverlap(Colission)
  (params (OverlappedComponent :type Primitive%20Component%20Object%20Reference) (OtherActor :type Actor%20Object%20Reference) (OtherComp :type Primitive%20Component%20Object%20Reference) (OtherBodyIndex :type Integer) (bFromSweep :type Boolean) (SweepResult :type Hit%20Result%20Structure%20%28by%20ref%29))
  (bind _asbp_third_person_character (Utilities|Casting|CastToBP_ThirdPersonCharacter OtherActor))
  (bind _playerstate (Variables|/Script/Engine.Pawn|GetPlayerState _asbp_third_person_character))
  (bind _asbp_ps_mousen (Utilities|Casting|CastToBP_PS_Mousen _playerstate))
  (if (!= OtherActor (Variables|Default|GetInstigator))
    (if (Utilities|DoesObjectImplementInterface OtherActor "/Game/Spells/StatusEffects/Interfaces/I_Status_Charmed.I_Status_Charmed_C")
      (if (!= (Math|Conversions|ToInteger(Byte) (Variables|/Game/ThirdPerson/Blueprints/Gameplay/BP_PS_Mousen.BP_PS_Mousen_C|GetPlayerTeam (.AsBP%20PS%20Mousen (Utilities|Casting|CastToBP_PS_Mousen (Variables|/Script/Engine.Pawn|GetPlayerState (Variables|Default|GetInstigator)))))) (Math|Conversions|ToInteger(Byte) (Variables|/Game/ThirdPerson/Blueprints/Gameplay/BP_PS_Mousen.BP_PS_Mousen_C|GetPlayerTeam _asbp_ps_mousen)))
        (Class|IStatusCharmed|OnCharmed(Message) OtherActor "/Game/Spells/StatusEffects/Blueprints/BP_Status_Effect_Charmed.BP_Status_Effect_Charmed_C" (+ 2.0 (Variables|/Game/ThirdPerson/Blueprints/Gameplay/BP_PS_Mousen.BP_PS_Mousen_C|GetPacifyCharmedDuration _asbp_ps_mousen)))))))

(event Custom|CleanupResources
  (Actor|DestroyActor))

(event Custom|Server%20Bindings
  (EventDispatchers|BindEventtoPSPlayerReset (Variables|Default|GetAs%20BP%20PC%20Mousen) (delegate Custom|CleanupResources)))

(event EventBeginPlay
  (bind _asbp_pc_mousen (Utilities|Casting|CastToBP_PC_Mousen (Game|GetPlayerController 0)))
  (Variables|Default|SetAs%20BP%20PC%20Mousen _asbp_pc_mousen)
  (Variables|Default|SetAs%20BP%20PS%20Mousen (.AsBP%20PS%20Mousen (Utilities|Casting|CastToBP_PS_Mousen (Variables|/Script/Engine.Pawn|GetPlayerState (Variables|Default|GetInstigator)))))
  (CallFunction|ServerBindings))

(fn ConstructionScript)

(fn GetMovementComponent
  (return 0))

(fn GetProjectileMovementComponent
  (return 0))