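; Bubble spell actor that glides out along the caster's camera forward on a timeline, then becomes an active, bobbing launch pad for characters.
; Overlaps trigger a multicast launch using player controller 0's velocity, with a brief per-actor cooldown.
; Server-side pops play a sound and spend charges, shrinking the bubble until it is destroyed at zero, on lifetime expiry or on player reset.
; The instigator's JetStream perk alters lifetime and launch strength.
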(event OnComponentBeginOverlap(Sphere)
  (params (OverlappedComponent :type Primitive%20Component%20Object%20Reference) (OtherActor :type Actor%20Object%20Reference) (OtherComp :type Primitive%20Component%20Object%20Reference) (OtherBodyIndex :type Integer) (bFromSweep :type Boolean) (SweepResult :type Hit%20Result%20Structure%20%28by%20ref%29))
  (if (Variables|Default|GetActive)
    (CallFunction|ServerPop OtherActor)))

(event Custom|CleanupResources
  (Actor|DestroyActor))

(event Custom|Server%20Pulse%20Forwards
  (bind _alpha (Timeline|Timeline PlayFromStart)
    (:Update
      (Transformation|SetActorLocation self (Math|Vector|Lerp(Vector) (Variables|Default|GetStartPoint) (Variables|Default|GetEndPoint) _alpha) true false))
    (:Finished
      (Variables|Default|SetActive true)
      (for _array_element (Collision|GetOverlappingActors (Variables|Default|GetSphere) 0 :!class /Script/Engine.PrimitiveComponent)
        (CallFunction|ServerPop _array_element)))))

(event Custom|Multicast%20Apply%20Impulse
  (params (Actor :type Actor%20Object%20Reference))
  (bind _as_bp_pc_mousen (Variables|Default|GetAs%20BP%20PC%20Mousen))
  (bind _instigator (Variables|Default|GetInstigator))
  (bind _returnvalue (Transformation|GetVelocity _as_bp_pc_mousen))
  (bind _playerstate (Variables|/Script/Engine.Pawn|GetPlayerState _instigator))
  (bind _asbp_ps_mousen (Utilities|Casting|CastToBP_PS_Mousen _playerstate))
  (bind _hasjetstream_ (Variables|/Game/ThirdPerson/Blueprints/Gameplay/BP_PS_Mousen.BP_PS_Mousen_C|GetHasJetStream? _asbp_ps_mousen))
  (bind _returnvalue_2 (select _hasjetstream_ 1.75e+03 1.25e+03))
  (bind _returnvalue_3 (* _returnvalue _returnvalue_2))
  (bind _ascharacter (Utilities|Casting|CastToCharacter Actor))
  (Character|LaunchCharacter _ascharacter (Math|Vector|MakeVector (.x _returnvalue_3) (.y _returnvalue_3) (select _hasjetstream_ 2.5e+03 (.z (Variables|Default|GetLaunchVelocity)))) true true))

(event Custom|Server%20Bindings
  (EventDispatchers|BindEventtoPSPlayerReset (Variables|Default|GetAs%20BP%20PC%20Mousen) (delegate Custom|CleanupResources)))

(event Custom|Multicast%20Sound
  (Audio|SpawnSoundAttached "/Game/Sounds/Character/Magic/Bubble/MS_Bubble_Pop.MS_Bubble_Pop" (Variables|Default|GetSphere) "None" "0, 0, 0" "0, 0, 0" "KeepRelativeOffset" false 1.0 1.0 0.0 0 0))

(event Custom|Server%20Shrink
  (params (A :type Integer))
  (bind _scale (Timeline|Shrink PlayFromStart)
    (:Update
      (Transformation|SetWorldScale3D (Variables|Default|GetSphere) (* (* (Variables|Default|GetStartingScale) (/ (+ (Variables|Default|GetCurrentCharges) 1) (Variables|Default|GetMaxCharges))) _scale)))
    (:Finished
      (if (<= A 0)
        (Variables|Default|SetActive false)
        (Actor|DestroyActor)))))

(event Custom|Server%20Pop
  (params (Actor :type Actor%20Object%20Reference%20%28by%20ref%29))
  (if (not (Utilities|Array|ContainsItem (Variables|Default|GetAffectedActors) Actor))
    (CallFunction|MulticastApplyImpulse Actor)
    (if (Networking|IsServer)
      (CallFunction|MulticastSound)
      (Utilities|Array|Add (Variables|Default|GetAffectedActors) Actor)
      (bind _result (Math|Integer|DecrementInt (Variables|Default|GetCurrentCharges))
        (:%20%20
          (CallFunction|ServerShrink _result)
          (Utilities|FlowControl|Delay 0.2)
          (Utilities|Array|RemoveItem (Variables|Default|GetAffectedActors) Actor))))))

(event EventBeginPlay
  (bind _asbp_pc_mousen (Utilities|Casting|CastToBP_PC_Mousen (Game|GetPlayerController 0)))
  (Variables|Default|SetAs%20BP%20PC%20Mousen _asbp_pc_mousen)
  (bind _camera (Class|ICharacter|GetCamera(Message) (.AsBP%20Third%20Person%20Character (Utilities|Casting|CastToBP_ThirdPersonCharacter (Variables|Default|GetInstigator)))))
  (Variables|Default|SetThirdPersonCamera _camera)
  (Variables|Default|SetStartPoint (Transformation|GetActorLocation))
  (Variables|Default|SetEndPoint (+ (* (Math|Vector|GetForwardVector (Variables|Default|GetThirdPersonCamera)) 8e+02) (Transformation|GetWorldLocation (Variables|Default|GetThirdPersonCamera))))
  (CallFunction|ServerPulseForwards)
  (CallFunction|ServerBindings)
  (Utilities|FlowControl|Delay (Math|Float|SelectFloat 3e+01 (Variables|Default|GetLifetime) (Variables|/Game/ThirdPerson/Blueprints/Gameplay/BP_PS_Mousen.BP_PS_Mousen_C|GetHasJetStream? (.AsBP%20PS%20Mousen (Utilities|Casting|CastToBP_PS_Mousen (Variables|/Script/Engine.Pawn|GetPlayerState (Variables|Default|GetInstigator)))))))
  (Actor|DestroyActor))

(event EventTick
  (params (DeltaSeconds :type Float%20%28single-precision%29))
  (bind _output_get (Variables|Default|SetRunningTime (+ DeltaSeconds (Variables|Default|GetRunningTime))))
  (Transformation|SetRelativeLocationAndRotation (Variables|Default|GetSphere) (Math|Vector|Lerp(Vector) "0.000000,0.000000,15.000000" "0.000000,0.000000,-15.000000" (+ (* (Math|Trig|Sin(Radians) _output_get) 0.5) 0.5)) (Math|Rotator|MakeRotator 0.0 0.0 (* (+ (* (Math|Trig|Sin(Radians) _output_get) 0.5) 0.5) 1.8e+02)) false false))

(fn ConstructionScript)