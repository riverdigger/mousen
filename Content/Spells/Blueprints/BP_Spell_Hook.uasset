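; Hook spell projectile for the melee character, tethered to the caster by a cable, that damages and drags in enemy players.
; Server-side overlap filters by team; shields block the pull, projectiles receive a collision message, and other surfaces launch casters who have Hookshot.
; At range limit or after contact, a distance-scaled timeline returns the hook, lerping victims to a traced point before the caster's camera.
; Ending stuns the victim and restores the weapon.
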(event OnComponentBeginOverlap(Box)
  (params (OverlappedComponent :type Primitive%20Component%20Object%20Reference) (OtherActor :type Actor%20Object%20Reference) (OtherComp :type Primitive%20Component%20Object%20Reference) (OtherBodyIndex :type Integer) (bFromSweep :type Boolean) (SweepResult :type Hit%20Result%20Structure%20%28by%20ref%29))
  (if (Networking|IsServer)
    (if (not (Variables|Default|GetIsReturning?))
      (if (!= OtherActor (Variables|Default|GetInstigator))
        (if (Utilities|DoesObjectImplementInterface OtherActor "/Game/Spells/StatusEffects/Interfaces/I_Status_Launch.I_Status_Launch_C")
          (if (!= (Math|Conversions|ToInteger(Byte) (Variables|/Game/ThirdPerson/Blueprints/Gameplay/BP_PS_Mousen.BP_PS_Mousen_C|GetPlayerTeam (.AsBP%20PS%20Mousen (Utilities|Casting|CastToBP_PS_Mousen (Variables|/Script/Engine.Pawn|GetPlayerState (Variables|Default|GetInstigator)))))) (Math|Conversions|ToInteger(Byte) (Variables|/Game/ThirdPerson/Blueprints/Gameplay/BP_PS_Mousen.BP_PS_Mousen_C|GetPlayerTeam (.AsBP%20PS%20Mousen (Utilities|Casting|CastToBP_PS_Mousen (Variables|/Script/Engine.Pawn|GetPlayerState (.AsBP%20Third%20Person%20Character (Utilities|Casting|CastToBP_ThirdPersonCharacter OtherActor))))))))
            (CallFunction|ServerUpdateHookedActor OtherActor))
          (Collision|SetCollisionEnabled (Variables|Default|GetBox) "NoCollision" :!label _label)
          (CallFunction|ServerReturnHook)
          (elif (Utilities|DoesObjectImplementInterface OtherActor "/Game/ThirdPerson/Blueprints/Gameplay/I_Projectile.I_Projectile_C")
            (Class|IProjectile|ApplyCollision(Message) OtherActor self (Variables|Default|GetProjectileMovement))
            (CallFunction|ServerReturnHook)
            (elif (Variables|/Game/ThirdPerson/Blueprints/Gameplay/BP_PS_Mousen.BP_PS_Mousen_C|GetHasHookshot? (.AsBP%20PS%20Mousen (Utilities|Casting|CastToBP_PS_Mousen (Variables|/Script/Engine.Pawn|GetPlayerState (.AsBP%20Third%20Person%20Character (Utilities|Casting|CastToBP_ThirdPersonCharacter (Variables|Default|GetInstigator)))))))
              (CallFunction|OCLaunchCharacter)
              (CallFunction|MulticastStopMovement)
              (Variables|Default|SetIsReturning? true)
              (Utilities|FlowControl|Delay 0.5)
              (CallFunction|ServerReturnHook)
              (else
                (goto _label)))))))))

(event Custom|OC%20Launch%20Character
  (bind _self self)
  (bind _instigator (Variables|Default|GetInstigator))
  (bind _returnvalue (Transformation|GetActorLocation _self))
  (bind _asbp_third_person_character (Utilities|Casting|CastToBP_ThirdPersonCharacter _instigator))
  (bind _returnvalue_2 (Transformation|GetActorLocation _asbp_third_person_character))
  (bind _returnvalue_3 (- _returnvalue _returnvalue_2))
  (bind _returnvalue_4 (Math|Vector|VectorLength _returnvalue_3))
  (Development|PrintString (Utilities|String|ToString(Float) _returnvalue_4))
  (Character|LaunchCharacter _asbp_third_person_character (+ (* (Math|Vector|Normalize _returnvalue_3) (Math|Float|MapRangeClamped _returnvalue_4 0.0 1.7e+03 2.5e+03 2.85e+03)) "0.000000,0.000000,750.000000") true true))

(event Custom|Server%20Return%20Hook
  (bind _instigator (Variables|Default|GetInstigator))
  (bind _returnvalue (Transformation|GetActorLocation _instigator))
  (CallFunction|MulticastStopMovement)
  (Variables|Default|SetIsReturning? true)
  (Variables|Default|SetReturn%20Start%20Point (Transformation|GetActorLocation))
  (Utilities|FlowControl|Delay 0.15)
  (Components|Timeline|SetPlayRate (Variables|Default|GetReturn%20to%20Instigator) (/ 7.5e+02 (Math|Vector|Distance(Vector) (Variables|Default|GetReturn%20Start%20Point) (Transformation|GetActorLocation (Variables|Default|GetInstigator)))))
  (bind _alpha (Timeline|Return%20to%20Instigator PlayFromStart)
    (:Update
      (Utilities|IsValid (Variables|Default|GetInstigator)
        (:Is%20Valid
          (Transformation|SetActorLocation (Math|Vector|Lerp(Vector) (Variables|Default|GetReturn%20Start%20Point) (Transformation|GetActorLocation (Variables|Default|GetInstigator)) _alpha) false false)
          (Variables|/Script/Engine.MovementComponent|SetVelocity (Variables|Default|GetProjectileMovement) (Math|Vector|Normalize (- (Variables|Default|GetReturn%20Start%20Point) (Math|Vector|Lerp(Vector) (Variables|Default|GetReturn%20Start%20Point) (Transformation|GetActorLocation (Variables|Default|GetInstigator)) _alpha))))
          (bind _camera (Class|ICharacter|GetCamera(Message) _instigator))
          (Utilities|IsValid (Variables|Default|GetHooked%20Actor)
            (:Is%20Valid
              (bind _count (Class|IStatusEffectOwner|GetStatusEffectCount(Message) (Variables|Default|GetHooked%20Actor) "Launched"))
              (if (>= _count 1)
                (bind (_outhit _returnvalue_2) (Collision|LineTraceByChannel _returnvalue (+ _returnvalue (* (Math|Vector|Normalize (Math|Vector|GetForwardVector _camera)) 195.0)) "TraceTypeQuery1" false (Variables|Default|GetIgnoredActors) "None"))
                (Transformation|SetActorLocation (Variables|Default|GetHooked%20Actor) (Math|Vector|Lerp(Vector) (Variables|Default|GetReturn%20Start%20Point) (Math|Vector|SelectVector (.ImpactPoint (Collision|BreakHitResult _outhit)) (+ _returnvalue (* (Math|Vector|Normalize (Math|Vector|GetForwardVector _camera)) 195.0)) _returnvalue_2) _alpha) false false)
                (else
                  (Variables|Default|SetHooked%20Actor 0))))))
        (:Is%20Not%20Valid
          (CallFunction|AbandonHook))))
    (:Finished
      (CallFunction|EndHook))))

(event Custom|Multicast%20Stop%20Movement
  (Components|Movement|StopMovementImmediately (Variables|Default|GetProjectileMovement)))

(event Custom|Multicast%20Reset%20Sword
  (Variables|/Game/ThirdPerson/Blueprints/Melee/BP_ThirdPerson_Melee.BP_ThirdPerson_Melee_C|SetIsHooking? (.AsBP%20Third%20Person%20Melee (Utilities|Casting|CastToBP_ThirdPerson_Melee (Variables|Default|GetInstigator))) false)
  (Rendering|SetVisibility (Variables|/Game/ThirdPerson/Blueprints/Melee/BP_ThirdPerson_Melee.BP_ThirdPerson_Melee_C|GetWeaponActor (.AsBP%20Third%20Person%20Melee (Utilities|Casting|CastToBP_ThirdPerson_Melee (Variables|Default|GetInstigator)))) true false))

(event Custom|Multicast%20Play%20Sound
  (Audio|SpawnSoundAttached "/Game/Sounds/Character/Melee/Hook/MS_Hook_Impact.MS_Hook_Impact" (Variables|Default|GetBox) "None" "0, 0, 0" "0, 0, 0" "KeepRelativeOffset" false 1.0 1.0 0.0 0 0))

(event Custom|Abandon%20Hook
  (bind _instigator (Variables|Default|GetInstigator))
  (bind _returnvalue (Transformation|GetActorLocation _instigator))
  (CallFunction|EndHook)
  (bind _alpha (Timeline|Return%20to%20Instigator Stop)
    (:Update
      (Utilities|IsValid (Variables|Default|GetInstigator)
        (:Is%20Valid
          (Transformation|SetActorLocation (Math|Vector|Lerp(Vector) (Variables|Default|GetReturn%20Start%20Point) (Transformation|GetActorLocation (Variables|Default|GetInstigator)) _alpha) false false)
          (Variables|/Script/Engine.MovementComponent|SetVelocity (Variables|Default|GetProjectileMovement) (Math|Vector|Normalize (- (Variables|Default|GetReturn%20Start%20Point) (Math|Vector|Lerp(Vector) (Variables|Default|GetReturn%20Start%20Point) (Transformation|GetActorLocation (Variables|Default|GetInstigator)) _alpha))))
          (bind _camera (Class|ICharacter|GetCamera(Message) _instigator))
          (Utilities|IsValid (Variables|Default|GetHooked%20Actor)
            (:Is%20Valid
              (bind _count (Class|IStatusEffectOwner|GetStatusEffectCount(Message) (Variables|Default|GetHooked%20Actor) "Launched"))
              (if (>= _count 1)
                (bind (_outhit _returnvalue_2) (Collision|LineTraceByChannel _returnvalue (+ _returnvalue (* (Math|Vector|Normalize (Math|Vector|GetForwardVector _camera)) 195.0)) "TraceTypeQuery1" false (Variables|Default|GetIgnoredActors) "None"))
                (Transformation|SetActorLocation (Variables|Default|GetHooked%20Actor) (Math|Vector|Lerp(Vector) (Variables|Default|GetReturn%20Start%20Point) (Math|Vector|SelectVector (.ImpactPoint (Collision|BreakHitResult _outhit)) (+ _returnvalue (* (Math|Vector|Normalize (Math|Vector|GetForwardVector _camera)) 195.0)) _returnvalue_2) _alpha) false false)
                (else
                  (Variables|Default|SetHooked%20Actor 0))))))
        (:Is%20Not%20Valid
          (CallFunction|AbandonHook))))
    (:Finished
      (CallFunction|EndHook))))

(event Custom|End%20Hook
  (Class|IStatusLaunch|OnUnLaunch(Message) (Variables|Default|GetHooked%20Actor) "/Game/Spells/StatusEffects/Blueprints/BP_Status_Effect_Launched.BP_Status_Effect_Launched_C" false self)
  (Class|IStatusStun|OnStun(Message) (Variables|Default|GetHooked%20Actor) "/Game/Spells/StatusEffects/Blueprints/BP_Status_Effect_Stunned.BP_Status_Effect_Stunned_C" 0.4 self)
  (CallFunction|MulticastResetSword)
  (Actor|DestroyActor))

(event Custom|Server%20Update%20Hooked%20Actor
  (params (Hooked%20Actor :type Actor%20Object%20Reference))
  (Variables|Default|SetLastKnownVector (Transformation|GetActorForwardVector))
  (bind _output_get (Variables|Default|SetHooked%20Actor Hooked%20Actor))
  (bind _hasshield_ (Class|ICharacter|GetHasShield(Message) _output_get))
  (if _hasshield_
    (Class|IDamage|ApplyServerPointDamage(Message) :self Hooked%20Actor :DamagedActor _output_get :BaseDamage (Variables|Default|GetDamage) :InstigatedBy (Variables|Default|GetAs%20BP%20PC%20Mousen) :DamageCauser (Variables|Default|GetInstigator) :DamageType "/Script/Engine.DamageType")
    (Variables|Default|SetHooked%20Actor 0)
    (else
      (Class|IStatusLaunch|OnLaunch(Message) _output_get "/Game/Spells/StatusEffects/Blueprints/BP_Status_Effect_Launched.BP_Status_Effect_Launched_C" 9999.0 "0, 0, 0" false self)
      (Class|IDamage|ApplyServerPointDamage(Message) :self _output_get :DamagedActor Hooked%20Actor :BaseDamage (Variables|Default|GetDamage) :InstigatedBy (Variables|Default|GetAs%20BP%20PC%20Mousen) :DamageCauser (Variables|Default|GetInstigator) :DamageType "/Script/Engine.DamageType")
      (if (Networking|IsServer)
        (CallFunction|MulticastPlaySound)))))

(event EventBeginPlay
  (bind _instigator (Variables|Default|GetInstigator))
  (Variables|Default|SetIgnoredActors (Utilities|Array|MakeArray (Variables|Default|GetInstigator)))
  (Rendering|SetVisibility (Variables|/Game/ThirdPerson/Blueprints/Melee/BP_ThirdPerson_Melee.BP_ThirdPerson_Melee_C|GetWeaponActor (.AsBP%20Third%20Person%20Melee (Utilities|Casting|CastToBP_ThirdPerson_Melee (Variables|Default|GetInstigator)))) false false)
  (Variables|Default|SetStart%20Point (Transformation|GetActorLocation))
  (bind _asbp_pc_mousen (Utilities|Casting|CastToBP_PC_Mousen (Game|GetPlayerController 0)))
  (Variables|Default|SetAs%20BP%20PC%20Mousen _asbp_pc_mousen)
  (Variables|Default|SetAs%20BP%20PS%20Mousen (.AsBP%20PS%20Mousen (Utilities|Casting|CastToBP_PS_Mousen (Variables|/Script/Engine.Pawn|GetPlayerState _instigator))))
  (Class|CableComponent|SetAttachEndto (Variables|Default|GetCable) _instigator "None" "pelvis"))

(event EventTick
  (params (DeltaSeconds :type Float%20%28single-precision%29))
  (Utilities|FlowControl|Sequence
    (:then_0
      (Utilities|FlowControl|DoOnce false
        (:Completed
          (Audio|SpawnSoundAttached "/Game/Sounds/Character/Melee/Hook/MS_Hook.MS_Hook" (Variables|Default|GetStaticMesh) "None" "0, 0, 0" "0, 0, 0" "KeepRelativeOffset" true 1.0 1.0 0.0 0 0))))
    (:then_1
      (if (and (>= (Math|Vector|Distance(Vector) (Transformation|GetActorLocation) (Variables|Default|GetStart%20Point)) (* (Variables|Default|GetRange) (Variables|/Game/ThirdPerson/Blueprints/Gameplay/BP_PS_Mousen.BP_PS_Mousen_C|GetHookReachModifier (.AsBP%20PS%20Mousen (Utilities|Casting|CastToBP_PS_Mousen (Variables|/Script/Engine.Pawn|GetPlayerState (Variables|Default|GetInstigator))))))) (not (Variables|Default|GetIsReturning?)))
        (CallFunction|ServerReturnHook)))))

(fn ConstructionScript)

(fn GetMovementComponent
  (return 0))

(fn GetProjectileMovementComponent
  (return (Variables|Default|GetProjectileMovement)))