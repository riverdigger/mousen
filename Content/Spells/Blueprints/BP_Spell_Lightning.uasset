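; BP_Spell_Lightning is a continuous lightning beam spell that damages targets, with optional stun and chain lightning from player-state upgrades.
; Each tick it traces from camera, then spell spawn, with a sphere-trace fallback for soft homing, ignoring same-team actors.
; Two beam emitters converge on damageable hits or scatter randomly around the aim point.
; Server-side looping timers apply damage, stun and chain-checker spawns, while events drive reticle feedback.
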(event Custom|Server%20Apply%20Damage
  (params (DamagedActor :type Actor%20Object%20Reference) (Damage :type Float%20%28double-precision%29) (Hit%20Direction :type Vector) (Hit%20Info :type Hit%20Result%20Structure) (Instigated%20By :type Controller%20Object%20Reference) (DamageCauser :type Actor%20Object%20Reference) (Damage%20Type%20Class :type Damage%20Type%20Class%20Reference))
  (Default|ApplyPointDamage (Variables|Default|GetAs%20BP%20PC%20Mousen) DamagedActor Damage Hit%20Direction Hit%20Info Instigated%20By DamageCauser Damage%20Type%20Class))

(event Custom|OC%20Reset%20Reticle
  (Default|ResetMagicReticle (Variables|/Game/ThirdPerson/Blueprints/Gameplay/BP_PC_Mousen.BP_PC_Mousen_C|GetAs%20BP%20HUD%20Mousen (Variables|Default|GetAs%20BP%20PC%20Mousen))))

(event Custom|Server%20Tick%20Damage
  (bind _localhitactor (Variables|Default|GetLocalHitActor))
  (CallFunction|ServerApplyDamage :DamagedActor (Variables|Default|GetLocalHitActor) :Damage (Variables|Default|GetDamage) :Hit%20Direction (Variables|Default|GetLocalImpactNormal) :Instigated%20By (Variables|Default|GetAs%20BP%20PC%20Mousen) :DamageCauser (Variables|Default|GetInstigator) :Damage%20Type%20Class "/Script/Engine.DamageType")
  (Class|IDamage|ShakeCamera(Message) (Variables|Default|GetInstigator))
  (if (Variables|/Game/ThirdPerson/Blueprints/Gameplay/BP_PS_Mousen.BP_PS_Mousen_C|GetHasChainLightning? (Variables|Default|GetAs%20BP%20PS%20Mousen))
    (Game|SpawnActorfromClass "/Game/Spells/Blueprints/BP_Lightning_Chain_Checker.BP_Lightning_Chain_Checker_C" (Transformation|GetActorTransform _localhitactor) "Undefined" "MultiplyWithRoot" 0 (Variables|Default|GetIgnoredActors) _localhitactor (Variables|Default|GetDistance) (Variables|Default|GetInstigator))))

(event Custom|Update%20Ignored%20Actors
  (bind _outactors (Actor|GetAllActorswithTag (Utilities|Name|EnumtoName (Variables|/Game/ThirdPerson/Blueprints/Gameplay/BP_PS_Mousen.BP_PS_Mousen_C|GetPlayerTeam (.AsBP%20PS%20Mousen (Utilities|Casting|CastToBP_PS_Mousen (Variables|/Script/Engine.Pawn|GetPlayerState (Variables|Default|GetAs%20BP%20Third%20Person%20Magic))))))))
  (bind _output_get (Variables|Default|SetIgnoredActors _outactors))
  (Utilities|Array|AddUnique _output_get (Variables|Default|GetInstigator)))

(event Custom|Server%20Apply%20Stun
  (bind _as_bp_ps_mousen (Variables|Default|GetAs%20BP%20PS%20Mousen))
  (if (Utilities|DoesObjectImplementInterface (Variables|Default|GetLocalHitActor) "/Game/Spells/StatusEffects/Interfaces/I_Status_Stun.I_Status_Stun_C")
    (Class|IStatusStun|OnStun(Message) (Variables|Default|GetLocalHitActor) "/Game/Spells/StatusEffects/Blueprints/BP_Status_Effect_Stunned.BP_Status_Effect_Stunned_C" (+ (Variables|/Game/ThirdPerson/Blueprints/Gameplay/BP_PS_Mousen.BP_PS_Mousen_C|GetLightningStunDuration _as_bp_ps_mousen) (Variables|/Game/ThirdPerson/Blueprints/Gameplay/BP_PS_Mousen.BP_PS_Mousen_C|GetPacifyStunLightningDuration _as_bp_ps_mousen)))))

(event Custom|OC%20Shrink%20Reticle
  (Default|ShrinkMagicReticle (Variables|/Game/ThirdPerson/Blueprints/Gameplay/BP_PC_Mousen.BP_PC_Mousen_C|GetAs%20BP%20HUD%20Mousen (Variables|Default|GetAs%20BP%20PC%20Mousen))))

(event Custom|Reset%20Reticle
  (if (Variables|Default|GetHasConnected?)
    (Utilities|FlowControl|DoOnce false
      (:Completed
        (CallFunction|OCResetReticle)))))

(event EventBeginPlay
  (bind _asbp_pc_mousen (Utilities|Casting|CastToBP_PC_Mousen (Game|GetPlayerController 0)))
  (Variables|Default|SetAs%20BP%20PC%20Mousen _asbp_pc_mousen)
  (bind _output_get (Variables|Default|SetAs%20BP%20Third%20Person%20Magic (.AsBP%20Third%20Person%20Magic (Utilities|Casting|CastToBP_ThirdPerson_Magic (Variables|Default|GetInstigator)))))
  (bind _output_get_2 (Variables|Default|SetAs%20BP%20PS%20Mousen (.AsBP%20PS%20Mousen (Utilities|Casting|CastToBP_PS_Mousen (Variables|/Script/Engine.Pawn|GetPlayerState _output_get)))))
  (bind _output_get_3 (Variables|Default|SetDistance (Variables|/Game/ThirdPerson/Blueprints/Gameplay/BP_PS_Mousen.BP_PS_Mousen_C|GetLightningRange _output_get_2)))
  (CallFunction|UpdateIgnoredActors))

(event EventTick
  (params (DeltaSeconds :type Float%20%28single-precision%29))
  (bind _as_bp_third_person_magic (Variables|Default|GetAs%20BP%20Third%20Person%20Magic))
  (bind _as_bp_third_person_magic_2 (Variables|Default|GetAs%20BP%20Third%20Person%20Magic))
  (bind _as_bp_ps_mousen (Variables|Default|GetAs%20BP%20PS%20Mousen))
  (bind _camerastartpoint (Variables|/Game/ThirdPerson/Blueprints/Magic/BP_ThirdPerson_Magic.BP_ThirdPerson_Magic_C|GetCameraStartPoint _as_bp_third_person_magic))
  (bind _spellspawn (Variables|/Game/ThirdPerson/Blueprints/Magic/BP_ThirdPerson_Magic.BP_ThirdPerson_Magic_C|GetSpellSpawn _as_bp_third_person_magic_2))
  (bind _returnvalue (Transformation|GetWorldLocation _camerastartpoint))
  (Variables|Default|SetLocalIsHitting false)
  (Variables|Default|SetLocalImpactPoint "0, 0, 0")
  (Variables|Default|SetLocalImpactNormal "0, 0, 0")
  (Variables|Default|SetLocalHitActor 0)
  (Math|Integer|IncrementInt (Variables|Default|GetTickCount)
    (:%20%20
      ;[0.04246 0.05443 1 1 80] Set start and end point
      (Utilities|IsValid _spellspawn
        (:Is%20Valid
          _)
        (:Is%20Not%20Valid
          _))
      (Variables|Default|SetStartPoint (Transformation|GetWorldLocation _spellspawn))
      (bind _camera (Default|GetCamera (Variables|Default|GetAs%20BP%20Third%20Person%20Magic)))
      (Variables|Default|SetEndPoint (+ _returnvalue (* (Math|Vector|GetForwardVector _camera) (Variables|Default|GetDistance))))
      ;[1 1 1 1 80] Camera Line Trace to check if crosshair is hitting, if it is, use that hit, else use the max value for the trace
      (bind (_outhit _returnvalue_2) (Collision|LineTraceByChannel _returnvalue (Variables|Default|GetEndPoint) "TraceTypeQuery1" false (Variables|Default|GetIgnoredActors) "None" true "(R=0.120979,G=1.000000,B=0.277371,A=1.000000)" "(R=0.947917,G=0.365343,B=0.918246,A=1.000000)"))
      (if _returnvalue_2
        (Variables|Default|SetEndPoint (.ImpactPoint (Collision|BreakHitResult _outhit)))
        (else
          (Variables|Default|SetEndPoint (.TraceEnd (Collision|BreakHitResult _outhit)))))
      ;[1 1 1 1 80] Line Trace from player to end point, if it hit's something then save the hit info and shoot lightning, else check a sphere trace
      (bind (_outhit_2 _returnvalue_3) (Collision|LineTraceByChannel (Transformation|GetWorldLocation (Variables|/Game/ThirdPerson/Blueprints/Magic/BP_ThirdPerson_Magic.BP_ThirdPerson_Magic_C|GetSpellSpawn (Variables|Default|GetAs%20BP%20Third%20Person%20Magic))) (Variables|Default|GetEndPoint) "TraceTypeQuery1" false (Variables|Default|GetIgnoredActors) "None" true "(R=0.000000,G=0.118403,B=1.000000,A=1.000000)" "(R=0.925733,G=1.000000,B=0.091299,A=1.000000)"))
      (bind _output_get (Variables|Default|SetLocalIsLineTraceHittingSomething _returnvalue_3))
      (if _output_get
        ;;[1 1 1 1 30] We are hitting player
        (if (Utilities|DoesObjectImplementInterface (.HitActor (Collision|BreakHitResult _outhit_2)) "/Game/ThirdPerson/Blueprints/Gameplay/I_Damage.I_Damage_C")
          (Variables|Default|SetLocalIsHitting true)
          (Variables|Default|SetLocalImpactPoint (.ImpactPoint (Collision|BreakHitResult _outhit_2)))
          (Variables|Default|SetLocalImpactNormal (.ImpactNormal (Collision|BreakHitResult _outhit_2)))
          (Variables|Default|SetLocalHitActor (.HitActor (Collision|BreakHitResult _outhit_2)))
          (else
            ;[1 1 1 1 80] Sphere trace for "homing", if sphere hits a player check if the line trace hit was closer (if not don't hit), if yes then shoot lightning at hit
            (bind (_outhit_3 _returnvalue_4) (Collision|SphereTraceByChannel (Transformation|GetWorldLocation (Variables|/Game/ThirdPerson/Blueprints/Magic/BP_ThirdPerson_Magic.BP_ThirdPerson_Magic_C|GetSpellSpawn (Variables|Default|GetAs%20BP%20Third%20Person%20Magic))) (Variables|Default|GetEndPoint) 1.3e+02 "TraceTypeQuery4" false (Variables|Default|GetIgnoredActors) "None" :!label _label))
            (if _returnvalue_4
              (if (Variables|Default|GetLocalIsLineTraceHittingSomething)
                (if (<= (Math|Vector|Distance(Vector) (Transformation|GetWorldLocation (Variables|/Script/Engine.Actor|GetRootComponent (Variables|Default|GetAs%20BP%20Third%20Person%20Magic))) (.ImpactPoint (Collision|BreakHitResult _outhit_3))) (Math|Vector|Distance(Vector) (Transformation|GetWorldLocation (Variables|/Script/Engine.Actor|GetRootComponent (Variables|Default|GetAs%20BP%20Third%20Person%20Magic))) (.ImpactPoint (Collision|BreakHitResult _outhit_2))))
                  (Variables|Default|SetLocalIsHitting true :!label _label_2)
                  (Variables|Default|SetLocalImpactPoint (.ImpactPoint (Collision|BreakHitResult _outhit_3)))
                  (Variables|Default|SetLocalImpactNormal (.ImpactNormal (Collision|BreakHitResult _outhit_3)))
                  (Variables|Default|SetLocalHitActor (.HitActor (Collision|BreakHitResult _outhit_3)))
                  (else
                    (Variables|Default|SetLocalIsHitting false :!label _label_3)))
                (else
                  (goto _label_2)))
              (else
                (goto _label_3)))))
        (else
          (goto _label)))
      ;[1 1 1 1 80] If the target can take damage, focus the streams, else hide focus point
      (if (Variables|Default|GetLocalIsHitting)
        (if (Utilities|DoesObjectImplementInterface (Variables|Default|GetLocalHitActor) "/Game/ThirdPerson/Blueprints/Gameplay/I_Damage.I_Damage_C")
          (Variables|Default|SetEndPoint (Variables|Default|GetLocalImpactPoint))
          (Rendering|SetVisibility (Variables|Default|GetSparks) true false)
          (Rendering|SetVisibility (Variables|Default|GetStaticMesh) true false)
          (Transformation|SetWorldLocation (Variables|Default|GetSparks) (Variables|Default|GetEndPoint) false false)
          (Transformation|SetWorldLocation (Variables|Default|GetStaticMesh) (Variables|Default|GetEndPoint) false false)
          (else
            (Rendering|SetVisibility (Variables|Default|GetSparks) false false :!label _label_4)
            (Rendering|SetVisibility (Variables|Default|GetStaticMesh) false false)))
        (else
          (goto _label_4)))
      (Utilities|FlowControl|Sequence
        (:then_0
          ;[1 1 1 1 80] Set second beam start and end depending on if target takes damage
          (Class|ParticleSystemComponent|SetBeamSourceTangent (Variables|Default|GetLightning) 0 (* (Variables|Default|GetLocalImpactNormal) (Math|Conversions|ToFloat(Integer) (Math|Random|RandomIntegerinRange 30 50))))
          (Class|ParticleSystemComponent|SetBeamSourcePoint (Variables|Default|GetLightning) 0 (Variables|Default|GetStartPoint))
          (if (Variables|Default|GetLocalIsHitting)
            (if (Utilities|DoesObjectImplementInterface (Variables|Default|GetLocalHitActor) "/Game/ThirdPerson/Blueprints/Gameplay/I_Damage.I_Damage_C")
              (Class|ParticleSystemComponent|SetBeamTargetPoint (Variables|Default|GetLightning) 0 (Variables|Default|GetEndPoint))
              (else
                (Class|ParticleSystemComponent|SetBeamTargetPoint (Variables|Default|GetLightning) 0 (Math|Random|RandomPointinBoundingBox (Variables|Default|GetEndPoint) "400.000000,400.000000,400.000000") :!label _label_5)))
            (else
              (goto _label_5))))
        (:then_1
          ;[1 1 1 1 80] Set second beam start and end depending on if target takes damage
          (Class|ParticleSystemComponent|SetBeamSourceTangent (Variables|Default|GetLightning) 1 (* (Variables|Default|GetLocalImpactNormal) (Math|Conversions|ToFloat(Integer) (select (== (Math|Integer|%(Integer) (Variables|Default|GetTickCount) 35) 0) (Math|Random|RandomIntegerinRange 80 100) (Math|Random|RandomIntegerinRange 30 50)))))
          (Class|ParticleSystemComponent|SetBeamSourcePoint (Variables|Default|GetLightning) 1 (Variables|Default|GetStartPoint))
          (if (Variables|Default|GetLocalIsHitting)
            (if (Utilities|DoesObjectImplementInterface (Variables|Default|GetLocalHitActor) "/Game/ThirdPerson/Blueprints/Gameplay/I_Damage.I_Damage_C")
              (Class|ParticleSystemComponent|SetBeamTargetPoint (Variables|Default|GetLightning) 1 (Variables|Default|GetEndPoint))
              (else
                (Class|ParticleSystemComponent|SetBeamTargetPoint (Variables|Default|GetLightning) 1 (Math|Random|RandomPointinBoundingBox (Variables|Default|GetEndPoint) "400.000000,400.000000,400.000000") :!label _label_6)))
            (else
              (goto _label_6))))
        (:then_2
          ;[1 1 1 1 30] Confirm there is a hit actor and it can take damage from the server
          (Utilities|IsValid (Variables|Default|GetLocalHitActor)
            (:Is%20Valid
              (if (Utilities|DoesObjectImplementInterface (Variables|Default|GetLocalHitActor) "/Game/ThirdPerson/Blueprints/Gameplay/I_Damage.I_Damage_C")
                (if (Networking|IsServer)
                  (Utilities|FlowControl|Sequence
                    (:then_0
                      (if (not (Utilities|Time|IsTimerActivebyHandle (Variables|Default|GetMaintainedTimer)))
                        (if (Variables|/Game/ThirdPerson/Blueprints/Gameplay/BP_PS_Mousen.BP_PS_Mousen_C|GetHasMaintained? _as_bp_ps_mousen)
                          (bind _returnvalue_5 (Utilities|Time|SetTimerbyEvent (delegate Custom|Server%20Apply%20Stun) (Variables|/Game/ThirdPerson/Blueprints/Gameplay/BP_PS_Mousen.BP_PS_Mousen_C|GetLightningHitTimeTilStun _as_bp_ps_mousen) true))
                          (Variables|Default|SetMaintainedTimer _returnvalue_5))))
                    (:then_1
                      (if (not (Utilities|Time|IsTimerActivebyHandle (Variables|Default|GetTickDamageTimer)))
                        (bind _returnvalue_6 (Utilities|Time|SetTimerbyEvent (delegate Custom|Server%20Tick%20Damage) (Variables|Default|GetTickRate) true))
                        (Variables|Default|SetTickDamageTimer _returnvalue_6)
                        (Variables|Default|SetHasConnected? true)
                        (CallFunction|OCShrinkReticle)
                        (Utilities|FlowControl|DoOnce false) ; enters at Reset
                      ))))
                (else
                  (CallFunction|ResetReticle :!label _label_7)
                  (Utilities|Time|ClearandInvalidateTimerbyHandle (Variables|Default|GetMaintainedTimer))
                  (Utilities|Time|ClearandInvalidateTimerbyHandle (Variables|Default|GetTickDamageTimer)))))
            (:Is%20Not%20Valid
              (goto _label_7))))))))

(event EventDestroyed
  (if (Variables|Default|GetHasConnected?)
    (if (Variables|Default|GetLocalIsHitting)
      (CallFunction|OCResetReticle))))

(fn ConstructionScript)

(fn GetMovementComponent
  (return 0))

(fn GetProjectileMovementComponent
  (return 0))