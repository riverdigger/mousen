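; Frozen orb spell Blueprint that creates an expanding storm zone to freeze actors overlapping it.
; EnableStorm shows the tinted particle effect, enables sphere query collision and runs a timeline growing both from zero scale.
; On overlap, the server sends a frozen status message with a lifespan to actors implementing the freeze interface, skipping the instigator unless AffectsCaster is set.
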(event OnComponentBeginOverlap(SphereZone)
  (params (OverlappedComponent :type Primitive%20Component%20Object%20Reference) (OtherActor :type Actor%20Object%20Reference) (OtherComp :type Primitive%20Component%20Object%20Reference) (OtherBodyIndex :type Integer) (bFromSweep :type Boolean) (SweepResult :type Hit%20Result%20Structure%20%28by%20ref%29))
  (if (Utilities|DoesObjectImplementInterface OtherActor "/Game/Spells/StatusEffects/Interfaces/I_Status_Freeze.I_Status_Freeze_C")
    (if (== (Variables|Default|GetInstigator) OtherActor)
      (if (Variables|Default|GetAffectsCaster?)
        (if (Networking|IsServer) :!label _label
          (Class|IStatusFreeze|OnFrozen(Message) OtherActor (Variables|Default|GetFrozenStatusEffect) (Variables|Default|GetFrozenLifespan))))
      (else
        (goto _label)))))

(event Custom|Expand%20Zone
  (bind _alpha (Timeline|Grow%20Zone PlayFromStart)
    (:Update
      (Transformation|SetRelativeScale3D (Variables|Default|GetParticleSystem) (Math|Vector|Lerp(Vector) "0, 0, 0" (Variables|Default|GetParticleSystemScale) _alpha))
      (Transformation|SetRelativeScale3D (Variables|Default|GetSphereZone) (Math|Vector|Lerp(Vector) "0, 0, 0" (Variables|Default|GetSphereZoneScale) _alpha)))))

(fn ConstructionScript
  (Transformation|SetRelativeScale3D (Variables|Default|GetSphereZone) "0, 0, 0")
  (Transformation|SetRelativeScale3D (Variables|Default|GetParticleSystem) "0, 0, 0"))

(fn EnableStorm
  (bind _particlesystem (Variables|Default|GetParticleSystem))
  (Effects|Components|ParticleSystem|SetColorParameter _particlesystem "color" "(R=0.088542,G=0.911790,B=1.000000,A=1.000000)")
  (Rendering|SetVisibility _particlesystem true false)
  (Transformation|SetWorldRotation _particlesystem "0,1.000000, 0" false false)
  (Collision|SetCollisionEnabled (Variables|Default|GetSphereZone) "QueryOnly")
  (CallFunction|ExpandZone))