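; BP_Spell_Invisibility is a timed spell actor that makes overlapping characters invisible.
; On StaticMesh overlap it filters for the instigator or same-team characters, gated by AffectsCaster and AffectsTeammates.
; Valid targets implementing I_Status_Invisible receive the invisible status effect and duration through a server-only interface message.
; It caches player controller 0 as the effect's InstigatedBy, then destroys itself after its Lifespan.
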(event OnComponentBeginOverlap(StaticMesh)
  (params (OverlappedComponent :type Primitive%20Component%20Object%20Reference) (OtherActor :type Actor%20Object%20Reference) (OtherComp :type Primitive%20Component%20Object%20Reference) (OtherBodyIndex :type Integer) (bFromSweep :type Boolean) (SweepResult :type Hit%20Result%20Structure%20%28by%20ref%29))
  (if (== OtherActor (Variables|Default|GetInstigator))
    (if (Variables|Default|GetAffectsCaster?)
      (if (Utilities|DoesObjectImplementInterface OtherActor "/Game/Spells/StatusEffects/Interfaces/I_Status_Invisible.I_Status_Invisible_C") :!label _label
        (if (Networking|IsServer)
          (Class|IStatusInvisible|OnInvisible(Message) OtherActor "/Game/Spells/StatusEffects/Blueprints/BP_Status_Effect_Invisible.BP_Status_Effect_Invisible_C" (Variables|Default|GetInvisibleLifespan) (Variables|Default|GetAs%20BP%20PC%20Mousen) (Variables|Default|GetInstigator)))))
    (elif (== (Math|Conversions|ToInteger(Byte) (Variables|/Game/ThirdPerson/Blueprints/Gameplay/BP_PS_Mousen.BP_PS_Mousen_C|GetPlayerTeam (.AsBP%20PS%20Mousen (Utilities|Casting|CastToBP_PS_Mousen (Variables|/Script/Engine.Pawn|GetPlayerState (.AsBP%20Third%20Person%20Character (Utilities|Casting|CastToBP_ThirdPersonCharacter OtherActor))))))) (Math|Conversions|ToInteger(Byte) (Variables|/Game/ThirdPerson/Blueprints/Gameplay/BP_PS_Mousen.BP_PS_Mousen_C|GetPlayerTeam (.AsBP%20PS%20Mousen (Utilities|Casting|CastToBP_PS_Mousen (Variables|/Script/Engine.Pawn|GetPlayerState (Variables|Default|GetInstigator)))))))
      (if (Variables|Default|GetAffectsTeammates?)
        (goto _label)))))

(event EventBeginPlay
  (bind _asbp_pc_mousen (Utilities|Casting|CastToBP_PC_Mousen (Game|GetPlayerController 0)))
  (Variables|Default|SetAs%20BP%20PC%20Mousen _asbp_pc_mousen)
  (Utilities|FlowControl|Delay (Variables|Default|GetLifespan))
  (Actor|DestroyActor))

(fn ConstructionScript)