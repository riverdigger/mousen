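; BP_Spell_Charm_Wall is a spell actor: a moving wall that charms opposing players and heals teammates it overlaps.
; A multicast timeline sweeps it forward from spawn, scales the mesh toward the owner's PacifyWallLength, then destroys it.
; On the server, overlaps compare PlayerTeam, then send interface messages, adding the target's own PacifyCharmedDuration to charm lifespan.
; The caster is healed only if AffectsCaster is set.
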(event OnComponentBeginOverlap(StaticMesh)
  (params (OverlappedComponent :type Primitive%20Component%20Object%20Reference) (OtherActor :type Actor%20Object%20Reference) (OtherComp :type Primitive%20Component%20Object%20Reference) (OtherBodyIndex :type Integer) (bFromSweep :type Boolean) (SweepResult :type Hit%20Result%20Structure%20%28by%20ref%29))
  (bind _asbp_third_person_character (Utilities|Casting|CastToBP_ThirdPersonCharacter OtherActor))
  (bind _playerstate (Variables|/Script/Engine.Pawn|GetPlayerState _asbp_third_person_character))
  (bind _asbp_ps_mousen (Utilities|Casting|CastToBP_PS_Mousen _playerstate))
  (if (Utilities|DoesObjectImplementInterface OtherActor "/Game/Spells/StatusEffects/Interfaces/I_Status_Charmed.I_Status_Charmed_C")
    (if (Networking|IsServer)
      (if (!= (Variables|/Game/ThirdPerson/Blueprints/Gameplay/BP_PS_Mousen.BP_PS_Mousen_C|GetPlayerTeam _asbp_ps_mousen) (Math|Conversions|ToInteger(Byte) (Variables|/Game/ThirdPerson/Blueprints/Gameplay/BP_PS_Mousen.BP_PS_Mousen_C|GetPlayerTeam (.AsBP%20PS%20Mousen (Utilities|Casting|CastToBP_PS_Mousen (Variables|/Script/Engine.Pawn|GetPlayerState (.AsBP%20Third%20Person%20Character (Utilities|Casting|CastToBP_ThirdPersonCharacter (Components|GetOwner)))))))))
        (Class|IStatusCharmed|OnCharmed(Message) OtherActor "/Game/Spells/StatusEffects/Blueprints/BP_Status_Effect_Charmed.BP_Status_Effect_Charmed_C" (+ (Variables|Default|GetCharmedDuration) (Variables|/Game/ThirdPerson/Blueprints/Gameplay/BP_PS_Mousen.BP_PS_Mousen_C|GetPacifyCharmedDuration _asbp_ps_mousen)))
        (else
          ;[1 1 1] Wave of Healing
          (if true
            (if (== OtherActor (Variables|Default|GetInstigator))
              (if (Variables|Default|GetAffectsCaster?)
                (Class|HealthInterface|Heal(Message) OtherActor (Variables|Default|GetHealingAmount) :!label _label))
              (else
                (goto _label)))))))))

(event Custom|Server%20Pulse%20Forwards
  (CallFunction|MulticastPulseForwards))

(event Custom|Multicast%20Pulse%20Forwards
  (bind _alpha (Timeline|PulseForwards PlayFromStart)
    (:Update
      (Transformation|SetActorLocation self (Math|Vector|Lerp(Vector) (Variables|Default|GetStartPoint) (Variables|Default|GetEndPoint) _alpha) true false)
      (Transformation|SetWorldScale3D (Variables|Default|GetStaticMesh) (Math|Vector|Lerp(Vector) (Variables|Default|GetStartScale) (Variables|Default|GetEndScale) _alpha)))
    (:Finished
      (Actor|DestroyActor))))

(event EventBeginPlay
  (Variables|Default|SetStartPoint (Transformation|GetActorLocation))
  (Variables|Default|SetEndPoint (+ (Transformation|GetActorLocation) (* (Transformation|GetActorForwardVector) 1.2e+03)))
  (Variables|Default|SetStartScale (Transformation|GetWorldScale (Variables|Default|GetStaticMesh)))
  (Variables|Default|SetEndScale (Variables|/Game/ThirdPerson/Blueprints/Gameplay/BP_PS_Mousen.BP_PS_Mousen_C|GetPacify%20Wall%20Length (.AsBP%20PS%20Mousen (Utilities|Casting|CastToBP_PS_Mousen (Variables|/Script/Engine.Pawn|GetPlayerState (.AsBP%20Third%20Person%20Character (Utilities|Casting|CastToBP_ThirdPersonCharacter (Components|GetOwner))))))))
  (CallFunction|ServerPulseForwards))

(event EventTick
  (params (DeltaSeconds :type Float%20%28single-precision%29))
  (Utilities|FlowControl|DoOnce false
    (:Completed
      (Audio|SpawnSoundAttached "/Game/Sounds/Character/Magic/CharmWave/CharmWall_MS.CharmWall_MS" (Variables|Default|GetStaticMesh) "None" "0, 0, 0" "0, 0, 0" "KeepRelativeOffset" true 1.0 1.0 0.0 0 0))))

(fn ConstructionScript)