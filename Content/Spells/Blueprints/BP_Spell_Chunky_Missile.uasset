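; Homing spell missile that chases enemies with a steeply ramping turn acceleration.
; Every quarter second it retargets to the nearest "Homing"-tagged, non-team actor in line of sight and exponentially raises homing acceleration.
; On overlap, the server damages I_Damage actors through the caster's controller and destroys the missile; other hits also destroy it, except certain missiles and the caster's own objects.
; Destruction, including lifespan expiry, multicasts an ice burst.
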(event OnComponentBeginOverlap(Capsule)
  (params (OverlappedComponent :type Primitive%20Component%20Object%20Reference) (OtherActor :type Actor%20Object%20Reference) (OtherComp :type Primitive%20Component%20Object%20Reference) (OtherBodyIndex :type Integer) (bFromSweep :type Boolean) (SweepResult :type Hit%20Result%20Structure%20%28by%20ref%29))
  (bind _instigator (Variables|/Script/Engine.Actor|GetInstigator OtherActor))
  (if (Utilities|DoesObjectImplementInterface OtherActor "/Game/ThirdPerson/Blueprints/Gameplay/I_Damage.I_Damage_C")
    (if (!= OtherActor (Variables|Default|GetInstigator))
      (if (Networking|IsServer)
        (CallFunction|ServerApplyDamage :DamagedActor OtherActor :Damage (Variables|Default|GetDamage) :Instigated%20By (Variables|Default|GetAs%20BP%20PC%20Mousen) :DamageCauser (Variables|Default|GetInstigator))
        (Actor|DestroyActor)))
    (elif (not (or (== (Utilities|GetClass OtherActor) "/Game/Spells/Blueprints/BP_Spell_Missile.BP_Spell_Missile_C") (== (Utilities|GetClass OtherActor) "/Game/Spells/Blueprints/BP_Spell_MagicMissiles.BP_Spell_MagicMissiles_C")))
      (Utilities|IsValid _instigator
        (:Is%20Valid
          (if (!= (.AsBP%20PS%20Mousen (Utilities|Casting|CastToBP_PS_Mousen (Variables|/Script/Engine.Pawn|GetPlayerState _instigator))) (Variables|Default|GetAs%20BP%20PS%20Mousen))
            (if (Networking|IsServer) :!label _label
              (Actor|DestroyActor))))
        (:Is%20Not%20Valid
          (goto _label))))))

(event Custom|Server%20Apply%20Damage
  (params (DamagedActor :type Actor%20Object%20Reference) (Damage :type Float%20%28double-precision%29) (Hit%20Direction :type Vector) (Hit%20Info :type Hit%20Result%20Structure) (Instigated%20By :type Controller%20Object%20Reference) (DamageCauser :type Actor%20Object%20Reference) (Damage%20Type%20Class :type Damage%20Type%20Class%20Reference))
  (Default|ApplyPointDamage (Variables|Default|GetAs%20BP%20PC%20Mousen) DamagedActor Damage Hit%20Direction Hit%20Info Instigated%20By DamageCauser Damage%20Type%20Class))

(event Custom|Go%20To%20Target
  (bind _projectilemovement (Variables|Default|GetProjectileMovement))
  (bind _homing_target (CallFunction|FindHomingTarget))
  (Variables|/Script/Engine.ProjectileMovementComponent|SetHomingTargetComponent _projectilemovement _homing_target)
  (Variables|/Script/Engine.ProjectileMovementComponent|SetbIsHomingProjectile _projectilemovement true))

(event Custom|Server%20Spawn%20Emitter
  (params (Location :type Vector))
  (CallFunction|MulticastSpawnEmitter Location))

(event Custom|Multicast%20Spawn%20Emitter
  (params (Location :type Vector))
  (Effects|SpawnEmitteratLocation "/Game/ExternalFreeContent/Realistic_Starter_VFX_Pack_Vol2/Particles/Hit/P_Ice.P_Ice" Location))

(event EventBeginPlay
  (bind _asbp_pc_mousen (Utilities|Casting|CastToBP_PC_Mousen (Game|GetPlayerController 0)))
  (Variables|Default|SetAs%20BP%20PC%20Mousen _asbp_pc_mousen)
  (Variables|Default|SetAs%20BP%20PS%20Mousen (.AsBP%20PS%20Mousen (Utilities|Casting|CastToBP_PS_Mousen (Variables|/Script/Engine.Pawn|GetPlayerState (Variables|Default|GetInstigator)))))
  (Actor|SetLifeSpan (Variables|Default|GetLifespan))
  (CallFunction|GotoTarget :!label _label)
  (Math|Integer|IncrementInt (Variables|Default|GetLoopCount)
    (:%20%20
      (Variables|/Script/Engine.ProjectileMovementComponent|SetHomingAccelerationMagnitude (Variables|Default|GetProjectileMovement) (* 2e+02 (Math|Float|Power 1.45 (Math|Conversions|ToFloat(Integer) (Variables|Default|GetLoopCount)))))
      (Utilities|FlowControl|Delay 0.25)
      (goto _label))))

(event EventDestroyed
  (CallFunction|ServerSpawnEmitter (Transformation|GetActorLocation)))

(fn ConstructionScript)

(fn FindHomingTarget
  (bind _outactors (Actor|GetAllActorsOfClasswithTag "/Script/Engine.Actor" "Homing"))
  (for _array_element _outactors
    (if (not (Actor|ActorHasTag _array_element (Utilities|Name|EnumtoName (Variables|/Game/ThirdPerson/Blueprints/Gameplay/BP_PS_Mousen.BP_PS_Mousen_C|GetPlayerTeam (Variables|Default|GetAs%20BP%20PS%20Mousen)))))
      (if (!= _array_element (Variables|Default|GetInstigator))
        (bind _outhit (Collision|SphereTraceByChannel (Transformation|GetActorLocation) (Transformation|GetActorLocation _array_element) 15.0 "TraceTypeQuery1" false (Utilities|Array|MakeArray (Variables|Default|GetInstigator)) "None"))
        (if (== (.HitActor (Collision|BreakHitResult _outhit)) _array_element)
          (if (< (Math|Vector|VectorLength (- (Transformation|GetActorLocation _array_element) (Transformation|GetActorLocation))) (Variables|Default|GetClosestDistance))
            (Variables|Default|SetClosestDistance (Math|Vector|VectorLength (- (Transformation|GetActorLocation _array_element) (Transformation|GetActorLocation))))
            (Variables|Default|SetHomingTarget _array_element))))))
  (Utilities|IsValid (Variables|Default|GetHomingTarget)
    (:Is%20Valid
      (return (Actor|GetComponentbyClass (Variables|Default|GetHomingTarget) "/Script/Engine.CapsuleComponent")))
    (:Is%20Not%20Valid
      (return 0))))

(fn GetMovementComponent
  (return 0))

(fn GetProjectileMovementComponent
  (return (Variables|Default|GetProjectileMovement)))