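; Helper actor for the lightning chain spell that finds damageable actors within a sphere and spawns chain lightning to them.
; Overlapping actors that implement I_Damage are skipped if listed in IgnoredActors, which gains the checker and its HitActor on BeginPlay.
; A visibility trace must hit the candidate directly before BP_Spell_Lightning_Chain spawns with the impact data and owner's instigator.
; The construction script sets the search radius.
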(event OnComponentBeginOverlap(Sphere)
  (params (OverlappedComponent :type Primitive%20Component%20Object%20Reference) (OtherActor :type Actor%20Object%20Reference) (OtherComp :type Primitive%20Component%20Object%20Reference) (OtherBodyIndex :type Integer) (bFromSweep :type Boolean) (SweepResult :type Hit%20Result%20Structure%20%28by%20ref%29))
  (if (Utilities|DoesObjectImplementInterface OtherActor "/Game/ThirdPerson/Blueprints/Gameplay/I_Damage.I_Damage_C")
    (Variables|Default|SetHittingIgnoredActor? false)
    (for _array_element (Variables|Default|GetIgnoredActors)
      (if (== _array_element OtherActor)
        (Variables|Default|SetHittingIgnoredActor? true)))
    (if (not (Variables|Default|GetHittingIgnoredActor?))
      (bind (_outhit _returnvalue) (Collision|LineTraceByChannel (Transformation|GetActorLocation) (Transformation|GetActorLocation OtherActor) "TraceTypeQuery1" false (Variables|Default|GetIgnoredActors) "None"))
      (if _returnvalue
        (if (== (.HitActor (Collision|BreakHitResult _outhit)) OtherActor)
          (Game|SpawnActorfromClass "/Game/Spells/Blueprints/BP_Spell_Lightning_Chain.BP_Spell_Lightning_Chain_C" (Transformation|GetActorTransform) "Undefined" "MultiplyWithRoot" 0 (Transformation|GetActorLocation) (.ImpactPoint (Collision|BreakHitResult _outhit)) (.ImpactNormal (Collision|BreakHitResult _outhit)) (.HitActor (Collision|BreakHitResult _outhit)) (Game|GetInstigator (Components|GetOwner))))))))

(event EventBeginPlay
  (Utilities|Array|AddUnique (Variables|Default|GetIgnoredActors) self)
  (Utilities|Array|AddUnique (Variables|Default|GetIgnoredActors) (Variables|Default|GetHitActor)))

(fn ConstructionScript
  (Components|Sphere|SetSphereRadius (Variables|Default|GetSphere) (Variables|Default|GetIn%20Sphere%20Radius) true))