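; Projectile spike owned by BP_Spell_Cage that forms one post of the cage spell's fence and destroys itself when the cage is destroyed.
; On overlap, or at lifespan end if still unlanded, it freezes and reports completion; spikes already landed when the timer fires register as valid.
; Multicast events set the neighbor behind and, if their height gap is small enough, draw four persistent debug sphere traces between fence points, with hit results unused.
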(event OnComponentBeginOverlap(Capsule)
  (params (OverlappedComponent :type Primitive%20Component%20Object%20Reference) (OtherActor :type Actor%20Object%20Reference) (OtherComp :type Primitive%20Component%20Object%20Reference) (OtherBodyIndex :type Integer) (bFromSweep :type Boolean) (SweepResult :type Hit%20Result%20Structure%20%28by%20ref%29))
  (bind _projectilemovement (Variables|Default|GetProjectileMovement))
  (Components|Movement|StopMovementImmediately _projectilemovement)
  (Variables|/Script/Engine.ProjectileMovementComponent|SetProjectileGravityScale _projectilemovement 0.0)
  (Variables|Default|SetHasCollided? true)
  (Default|UpdateCompletedSpikes (Variables|Default|GetSpellCage)))

(event Custom|CleanupResources
  (Actor|DestroyActor))

(event Custom|Multicast%20Set%20Neighbor
  (params (NeighborBehind :type BP%20Spell%20Cage%20Spike%20Object%20Reference))
  (Variables|Default|SetNeighborBehind NeighborBehind))

(event Custom|Server%20Set%20Neighbor
  (params (NeighborBehind :type BP%20Spell%20Cage%20Spike%20Object%20Reference))
  (CallFunction|MulticastSetNeighbor NeighborBehind))

(event Custom|Server%20Activate%20Fence
  (CallFunction|MulticastActivateFence))

(event Custom|Multicast%20Activate%20Fence
  (bind _returnvalue (Transformation|GetActorLocation))
  (bind _neighborbehind (Variables|Default|GetNeighborBehind))
  (bind _returnvalue_2 (Transformation|GetActorLocation _neighborbehind))
  (bind _returnvalue_3 (- (.z _returnvalue_2) (.z _returnvalue)))
  (bind _returnvalue_4 (Math|Float|Absolute(Float) _returnvalue_3))
  (Development|PrintString (Utilities|String|ToString(Float) _returnvalue_4))
  (if (not (>= _returnvalue_4 3.7e+02))
    (Collision|SphereTraceByChannel (Transformation|GetWorldLocation (Variables|Default|GetFencePoint1)) (Transformation|GetWorldLocation (Variables|BP_Spell_Cage_Spike_C|GetFencePoint1 (Variables|Default|GetNeighborBehind))) 15.0 "TraceTypeQuery1" false 0 "Persistent" true "(R=0.000000,G=0.124772,B=1.000000,A=1.000000)")
    (Collision|SphereTraceByChannel (Transformation|GetWorldLocation (Variables|Default|GetFencePoint2)) (Transformation|GetWorldLocation (Variables|BP_Spell_Cage_Spike_C|GetFencePoint2 (Variables|Default|GetNeighborBehind))) 15.0 "TraceTypeQuery1" false 0 "Persistent" true "(R=0.000000,G=0.124772,B=1.000000,A=1.000000)")
    (Collision|SphereTraceByChannel (Transformation|GetWorldLocation (Variables|Default|GetFencePoint3)) (Transformation|GetWorldLocation (Variables|BP_Spell_Cage_Spike_C|GetFencePoint3 (Variables|Default|GetNeighborBehind))) 15.0 "TraceTypeQuery1" false 0 "Persistent" true "(R=0.000000,G=0.124772,B=1.000000,A=1.000000)")
    (Collision|SphereTraceByChannel (Transformation|GetWorldLocation (Variables|Default|GetFencePoint4)) (Transformation|GetWorldLocation (Variables|BP_Spell_Cage_Spike_C|GetFencePoint4 (Variables|Default|GetNeighborBehind))) 15.0 "TraceTypeQuery1" false 0 "Persistent" true "(R=0.000000,G=0.124772,B=1.000000,A=1.000000)")))

(event Custom|Server%20Bindings
  (EventDispatchers|BindEventtoCageDestroyed (Variables|Default|GetSpellCage) (delegate Custom|CleanupResources)))

(event Custom|Destroy%20Self
  (bind _projectilemovement (Variables|Default|GetProjectileMovement))
  (if (not (Variables|Default|GetHasCollided?))
    (Components|Movement|StopMovementImmediately _projectilemovement)
    (Variables|/Script/Engine.ProjectileMovementComponent|SetProjectileGravityScale _projectilemovement 0.0)
    (Variables|Default|SetHasCollided? true)
    (Default|UpdateCompletedSpikes (Variables|Default|GetSpellCage))
    (else
      (Default|UpdateTotalValidSpikes (Variables|Default|GetSpellCage) self))))

(event EventBeginPlay
  (Variables|Default|SetSpellCage (.AsBP%20Spell%20Cage (Utilities|Casting|CastToBP_Spell_Cage (Components|GetOwner))))
  (CallFunction|ServerBindings)
  (Utilities|Time|SetTimerbyEvent (delegate Custom|Destroy%20Self) (Variables|Default|GetLifespan)))

(fn ConstructionScript
  (|CallParentFunction))