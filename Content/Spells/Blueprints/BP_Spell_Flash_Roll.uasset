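; Flash Roll spell projectile for the Ranger: rolls its caster and stuns enemy players caught in its flash sphere.
; On spawn, a timeline sweeps the caster along the camera's forward vector by the player state's FlashRollLength, clearing IsRolling near the end.
; A timer halts the projectile, removes its mesh and fires Niagara, later disabling the sphere.
; Sphere overlaps apply stun server-side through an interface, once per opposing-team actor.
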(event OnComponentBeginOverlap(Sphere)
  (params (OverlappedComponent :type Primitive%20Component%20Object%20Reference) (OtherActor :type Actor%20Object%20Reference) (OtherComp :type Primitive%20Component%20Object%20Reference) (OtherBodyIndex :type Integer) (bFromSweep :type Boolean) (SweepResult :type Hit%20Result%20Structure%20%28by%20ref%29))
  (if (!= OtherActor (Variables|Default|GetInstigator))
    (if (Utilities|DoesObjectImplementInterface OtherActor "/Game/Spells/StatusEffects/Interfaces/I_Status_Stun.I_Status_Stun_C")
      (if (!= (Math|Conversions|ToInteger(Byte) (Variables|/Game/ThirdPerson/Blueprints/Gameplay/BP_PS_Mousen.BP_PS_Mousen_C|GetPlayerTeam (.AsBP%20PS%20Mousen (Utilities|Casting|CastToBP_PS_Mousen (Variables|/Script/Engine.Pawn|GetPlayerState (Variables|Default|GetInstigator)))))) (Math|Conversions|ToInteger(Byte) (Variables|/Game/ThirdPerson/Blueprints/Gameplay/BP_PS_Mousen.BP_PS_Mousen_C|GetPlayerTeam (.AsBP%20PS%20Mousen (Utilities|Casting|CastToBP_PS_Mousen (Variables|/Script/Engine.Pawn|GetPlayerState (.AsBP%20Third%20Person%20Character (Utilities|Casting|CastToBP_ThirdPersonCharacter OtherActor))))))))
        (if (== (Utilities|Array|FindItem (Variables|Default|GetAlreadyAffectedActors) OtherActor) -1)
          (Utilities|Array|AddUnique (Variables|Default|GetAlreadyAffectedActors) OtherActor)
          (if (Networking|IsServer)
            (Class|IStatusStun|OnStun(Message) OtherActor "/Game/Spells/StatusEffects/Blueprints/BP_Status_Effect_Stunned.BP_Status_Effect_Stunned_C" (Variables|Default|GetStunDuration))))))))

(event OnSystemFinished(Niagara)
  (params (PSystem :type Niagara%20Component%20Object%20Reference))
  (Actor|DestroyActor))

(event Custom|Roll%20Backwards
  (params (Character :type BP%20Third%20Person%20Ranger%20Object%20Reference))
  (Variables|/Game/ThirdPerson/Blueprints/Ranger/BP_ThirdPerson_Ranger.BP_ThirdPerson_Ranger_C|SetIsRolling? Character true)
  (bind _camera (Default|GetCamera Character))
  (bind _output_get (Variables|Default|SetStart%20Point (Transformation|GetActorLocation Character)))
  (Variables|Default|SetEnd%20Point (Math|Vector|MakeVector (.x (+ _output_get (* (Math|Vector|MakeVector (.x (Math|Vector|GetForwardVector _camera)) (.y (Math|Vector|GetForwardVector _camera)) (.z (Math|Vector|GetForwardVector _camera))) (Variables|/Game/ThirdPerson/Blueprints/Gameplay/BP_PS_Mousen.BP_PS_Mousen_C|GetFlashRollLength (.AsBP%20PS%20Mousen (Utilities|Casting|CastToBP_PS_Mousen (Variables|/Script/Engine.Pawn|GetPlayerState (.AsBP%20Third%20Person%20Character (Utilities|Casting|CastToBP_ThirdPersonCharacter (Components|GetOwner)))))))))) (.y (+ _output_get (* (Math|Vector|MakeVector (.x (Math|Vector|GetForwardVector _camera)) (.y (Math|Vector|GetForwardVector _camera)) (.z (Math|Vector|GetForwardVector _camera))) (Variables|/Game/ThirdPerson/Blueprints/Gameplay/BP_PS_Mousen.BP_PS_Mousen_C|GetFlashRollLength (.AsBP%20PS%20Mousen (Utilities|Casting|CastToBP_PS_Mousen (Variables|/Script/Engine.Pawn|GetPlayerState (.AsBP%20Third%20Person%20Character (Utilities|Casting|CastToBP_ThirdPersonCharacter (Components|GetOwner)))))))))) (.z (+ _output_get (* (Math|Vector|MakeVector (.x (Math|Vector|GetForwardVector _camera)) (.y (Math|Vector|GetForwardVector _camera)) (.z (Math|Vector|GetForwardVector _camera))) (Variables|/Game/ThirdPerson/Blueprints/Gameplay/BP_PS_Mousen.BP_PS_Mousen_C|GetFlashRollLength (.AsBP%20PS%20Mousen (Utilities|Casting|CastToBP_PS_Mousen (Variables|/Script/Engine.Pawn|GetPlayerState (.AsBP%20Third%20Person%20Character (Utilities|Casting|CastToBP_ThirdPersonCharacter (Components|GetOwner))))))))))))
  (Components|Timeline|SetPlayRate (Variables|Default|GetRollBackwardsTimeline) 2.0)
  (CallFunction|FlipBaclwards Character))

(event Custom|Server%20Stop%20Roll
  (Audio|Components|Audio|Stop (Variables|Default|GetRollBackwardsTimeline)))

(event Custom|Flip%20Baclwards
  (params (Target :type BP%20Third%20Person%20Ranger%20Object%20Reference))
  (bind _alpha (Timeline|RollBackwardsTimeline PlayFromStart)
    (:Update
      (if (>= _alpha 0.6)
        (Variables|/Game/ThirdPerson/Blueprints/Ranger/BP_ThirdPerson_Ranger.BP_ThirdPerson_Ranger_C|SetIsRolling? Target false))
      (Transformation|SetActorLocation Target (Math|Vector|Lerp(Vector) (Variables|Default|GetStart%20Point) (Variables|Default|GetEnd%20Point) _alpha) true false))))

(event Custom|Break%20Self
  (bind _niagara (Variables|Default|GetNiagara))
  (bind _projectilemovement (Variables|Default|GetProjectileMovement))
  (bind _staticmesh (Variables|Default|GetStaticMesh))
  (Components|Movement|StopMovementImmediately _projectilemovement)
  (Variables|/Script/Engine.ProjectileMovementComponent|SetProjectileGravityScale _projectilemovement 0.0)
  (Utilities|FlowControl|Sequence
    (:then_0
      (Utilities|IsValid _staticmesh
        (:Is%20Valid
          (Components|DestroyComponent _staticmesh))))
    (:then_1
      (Utilities|IsValid _niagara
        (:Is%20Valid
          (Components|Activation|Activate _niagara true)
          (Utilities|FlowControl|Delay (Variables|Default|GetLifespan))
          (Collision|SetCollisionEnabled (Variables|Default|GetSphere) "NoCollision"))))))

(event EventBeginPlay
  (bind _asbp_pc_mousen (Utilities|Casting|CastToBP_PC_Mousen (Game|GetPlayerController 0)))
  (Variables|Default|SetAs%20BP%20PC%20Mousen _asbp_pc_mousen)
  (bind _output_get (Variables|Default|SetAs%20BP%20Third%20Person%20Ranger (.AsBP%20Third%20Person%20Ranger (Utilities|Casting|CastToBP_ThirdPerson_Ranger (Variables|Default|GetInstigator)))))
  (CallFunction|RollBackwards _output_get)
  (Utilities|IsValid (Variables|/Game/ThirdPerson/Blueprints/Ranger/BP_ThirdPerson_Ranger.BP_ThirdPerson_Ranger_C|GetSpellSpawn (Variables|Default|GetAs%20BP%20Third%20Person%20Ranger))
    (:Is%20Valid
      (Utilities|Time|SetTimerbyEvent (delegate Custom|Break%20Self) (Variables|Default|GetThrownLifespan)))))

(fn ConstructionScript)

(fn GetMovementComponent
  (return 0))

(fn GetProjectileMovementComponent
  (return 0))