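; Magic Missiles spell spawner that travels out from its spawn point, then fires a timed volley of six BP_Spell_Missile actors.
; A forward sphere trace sets the endpoint, offset from any wall hit, and a timeline lerps the spawner there.
; On arrival it shows its mesh and faces the nearest "Homing"-tagged actor in line of sight, falling back to its Instigator.
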(event EventBeginPlay
  (bind _returnvalue (Transformation|GetActorForwardVector))
  (bind _returnvalue_2 (Transformation|GetActorLocation))
  (bind _returnvalue_3 (* _returnvalue 7.5e+02))
  (bind _returnvalue_4 (+ _returnvalue_2 _returnvalue_3))
  ;[1 1 1 1 241] Spawn Spawner and face the correct way
  (bind _asbp_pc_mousen (Utilities|Casting|CastToBP_PC_Mousen (Game|GetPlayerController 0)))
  (Variables|Default|SetAs%20BP%20PC%20Mousen _asbp_pc_mousen)
  (Variables|Default|SetStartPoint _returnvalue_2)
  ;;[1 1 1 1 74] if collide, move away from wall
  (bind (_outhit _returnvalue_5) (Collision|SphereTraceByChannel _returnvalue_2 _returnvalue_4 5e+01 "TraceTypeQuery1" false (Utilities|Array|MakeArray (Variables|Default|GetInstigator)) "None"))
  (if _returnvalue_5
    (Variables|Default|SetEndPoint (+ (.ImpactPoint (Collision|BreakHitResult _outhit)) (* (.ImpactNormal (Collision|BreakHitResult _outhit)) 6e+01)))
    (bind _distancemultiplier (Timeline|Move%20Towards%20Point%20Timeline Play)
      (:Update
        (Transformation|SetActorLocation (Math|Vector|Lerp(Vector) (Variables|Default|GetStartPoint) (Variables|Default|GetEndPoint) _distancemultiplier) true false))
      (:Finished
        (Rendering|SetVisibility (Variables|Default|GetStaticMesh) true false)
        (bind _homing_target (CallFunction|FindHomingTarget))
        (Utilities|IsValid _homing_target
          (:Is%20Valid
            (Transformation|SetActorRotation (Math|Rotator|FindLookatRotation (Transformation|GetActorLocation) (Transformation|GetWorldLocation _homing_target))))
          (:Is%20Not%20Valid
            (Transformation|SetActorRotation (Math|Rotator|FindLookatRotation (Transformation|GetActorLocation) (Transformation|GetActorLocation (Variables|Default|GetInstigator))))))
        (Actor|SetLifeSpan (Variables|Default|GetLifespan))
        (Utilities|FlowControl|DoN 6 :!label _label
          (:Exit
            (Game|SpawnActorfromClass "/Game/Spells/Blueprints/BP_Spell_Missile.BP_Spell_Missile_C" (Transformation|GetActorTransform) "Undefined" 0 0)
            (Utilities|FlowControl|Delay 0.35)
            (goto _label)))))
    (else
      (Variables|Default|SetEndPoint _returnvalue_4)
      (Timeline|Move%20Towards%20Point%20Timeline PlayFromStart))))

(fn ConstructionScript)

(fn FindHomingTarget
  (bind _outactors (Actor|GetAllActorsOfClasswithTag "/Script/Engine.Actor" "Homing"))
  (for _array_element _outactors
    (if (!= _array_element (Variables|Default|GetInstigator))
      (bind _outhit (Collision|SphereTraceByChannel (Transformation|GetActorLocation) (Transformation|GetActorLocation _array_element) 15.0 "TraceTypeQuery1" false (Utilities|Array|MakeArray (Variables|Default|GetInstigator)) "None"))
      (if (== (.HitActor (Collision|BreakHitResult _outhit)) _array_element)
        (if (< (Math|Vector|VectorLength (- (Transformation|GetActorLocation _array_element) (Transformation|GetActorLocation))) (Variables|Default|GetClosestDistance))
          (Variables|Default|SetClosestDistance (Math|Vector|VectorLength (- (Transformation|GetActorLocation _array_element) (Transformation|GetActorLocation))))
          (Variables|Default|SetHomingTarget _array_element)))))
  (Utilities|IsValid (Variables|Default|GetHomingTarget)
    (:Is%20Valid
      (return (Actor|GetComponentbyClass (Variables|Default|GetHomingTarget) "/Script/Engine.CapsuleComponent")))
    (:Is%20Not%20Valid
      (return 0))))

(fn GetMovementComponent
  (return 0))

(fn GetProjectileMovementComponent
  (return 0))