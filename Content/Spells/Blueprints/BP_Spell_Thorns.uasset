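; BP_Spell_Thorns is a thorns spell actor that attaches a thorns Niagara effect to its owner's mesh.
; On BeginPlay it fetches that mesh from the owner through GetMeshMessage and spawns the attached system.
; It also binds to the BP_PC_Mousen player reset event and destroys itself when that fires.
; The movement component getters return nothing, and no damage logic is present.
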(event Custom|CleanupResources
  (Actor|DestroyActor))

(event Custom|Server%20Bindings
  (EventDispatchers|BindEventtoPSPlayerReset (Variables|Default|GetAs%20BP%20PC%20Mousen) (delegate Custom|CleanupResources)))

(event EventBeginPlay
  (bind _asbp_pc_mousen (Utilities|Casting|CastToBP_PC_Mousen (Game|GetPlayerController 0)))
  (Variables|Default|SetAs%20BP%20PC%20Mousen _asbp_pc_mousen)
  (CallFunction|ServerBindings)
  (bind _mesh (Class|IStatusEffectOwner|GetMesh(Message) (Components|GetOwner)))
  (Niagara|SpawnSystemAttached "/Game/Items/FX/NS_Thorns_Attached.NS_Thorns_Attached" _mesh "None" "0, 0, 0" "0, 0, 0" "KeepRelativeOffset" false))

(fn ConstructionScript)

(fn GetMovementComponent
  (return 0))

(fn GetProjectileMovementComponent
  (return 0))