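; Short-lived chain lightning spell actor that draws a beam between a start and end point and strikes the hit actor.
; BeginPlay caches the caster's player state, gathers same-team actors and the instigator into IgnoredActors, and sets both beam emitters, which Tick keeps updated.
; With a valid hit, the server applies stun if HasMaintained, deals point damage via the player controller, then destroys the actor after a brief delay.
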(event Custom|Server%20Apply%20Damage
  (params (DamagedActor :type Actor%20Object%20Reference) (Damage :type Float%20%28double-precision%29) (Hit%20Direction :type Vector) (Hit%20Info :type Hit%20Result%20Structure) (Instigated%20By :type Controller%20Object%20Reference) (DamageCauser :type Actor%20Object%20Reference) (Damage%20Type%20Class :type Damage%20Type%20Class%20Reference))
  (Default|ApplyPointDamage (Variables|Default|GetAs%20BP%20PC%20Mousen) DamagedActor Damage Hit%20Direction Hit%20Info Instigated%20By DamageCauser Damage%20Type%20Class))

(event Custom|Server%20Tick%20Damage
  (CallFunction|ServerApplyDamage :DamagedActor (Variables|Default|GetHitActor) :Damage (Variables|Default|GetDamage) :Hit%20Direction (Variables|Default|GetLocalImpactNormal) :Instigated%20By (Variables|Default|GetAs%20BP%20PC%20Mousen) :DamageCauser (Variables|Default|GetInstigator) :Damage%20Type%20Class "/Script/Engine.DamageType"))

(event Custom|Server%20Update%20Ignored%20Actors
  (bind _outactors (Actor|GetAllActorswithTag (Utilities|Name|EnumtoName (Variables|/Game/ThirdPerson/Blueprints/Gameplay/BP_PS_Mousen.BP_PS_Mousen_C|GetPlayerTeam (.AsBP%20PS%20Mousen (Utilities|Casting|CastToBP_PS_Mousen (Variables|/Script/Engine.Pawn|GetPlayerState (Variables|Default|GetAs%20BP%20Third%20Person%20Magic))))))))
  (bind _output_get (Variables|Default|SetIgnoredActors _outactors))
  (Utilities|Array|AddUnique _output_get (Variables|Default|GetInstigator)))

(event Custom|Server%20Apply%20Stun
  (bind _as_bp_ps_mousen (Variables|Default|GetAs%20BP%20PS%20Mousen))
  (if (Utilities|DoesObjectImplementInterface (Variables|Default|GetHitActor) "/Game/Spells/StatusEffects/Interfaces/I_Status_Stun.I_Status_Stun_C")
    (Class|IStatusStun|OnStun(Message) (Variables|Default|GetHitActor) "/Game/Spells/StatusEffects/Blueprints/BP_Status_Effect_Stunned.BP_Status_Effect_Stunned_C" (+ (Variables|/Game/ThirdPerson/Blueprints/Gameplay/BP_PS_Mousen.BP_PS_Mousen_C|GetLightningStunDuration _as_bp_ps_mousen) (Variables|/Game/ThirdPerson/Blueprints/Gameplay/BP_PS_Mousen.BP_PS_Mousen_C|GetPacifyStunLightningDuration _as_bp_ps_mousen)))))

(event Custom|Begin%20Destroy
  (Utilities|FlowControl|Delay 0.2)
  (Actor|DestroyActor))

(event EventBeginPlay
  (bind _asbp_pc_mousen (Utilities|Casting|CastToBP_PC_Mousen (Game|GetPlayerController 0)))
  (Variables|Default|SetAs%20BP%20PC%20Mousen _asbp_pc_mousen)
  (bind _output_get (Variables|Default|SetAs%20BP%20Third%20Person%20Magic (.AsBP%20Third%20Person%20Magic (Utilities|Casting|CastToBP_ThirdPerson_Magic (Variables|Default|GetInstigator)))))
  (Variables|Default|SetAs%20BP%20PS%20Mousen (.AsBP%20PS%20Mousen (Utilities|Casting|CastToBP_PS_Mousen (Variables|/Script/Engine.Pawn|GetPlayerState _output_get))))
  (CallFunction|ServerUpdateIgnoredActors)
  (Utilities|FlowControl|Sequence
    (:then_0
      ;[1 1 1 1 80] Set second beam start and end
      (Class|ParticleSystemComponent|SetBeamSourceTangent (Variables|Default|GetLightning) 0 "0, 0, 0")
      (Class|ParticleSystemComponent|SetBeamSourcePoint (Variables|Default|GetLightning) 0 (Variables|Default|GetStartPoint))
      (Class|ParticleSystemComponent|SetBeamTargetPoint (Variables|Default|GetLightning) 0 (Variables|Default|GetEndPoint)))
    (:then_1
      ;[1 1 1 1 80] Set second beam start and end
      (Class|ParticleSystemComponent|SetBeamSourceTangent (Variables|Default|GetLightning) 1 (Variables|Default|GetLocalImpactNormal))
      (Class|ParticleSystemComponent|SetBeamSourcePoint (Variables|Default|GetLightning) 1 (Variables|Default|GetStartPoint))
      (Class|ParticleSystemComponent|SetBeamTargetPoint (Variables|Default|GetLightning) 1 (Variables|Default|GetEndPoint)))
    (:then_2
      ;[1 1 1 1 30] Confirm there is a hit actor and it can take damage from the server
      (Utilities|IsValid (Variables|Default|GetHitActor)
        (:Is%20Valid
          (if (Networking|IsServer)
            (Utilities|FlowControl|Sequence
              (:then_0
                (if (Variables|/Game/ThirdPerson/Blueprints/Gameplay/BP_PS_Mousen.BP_PS_Mousen_C|GetHasMaintained? (Variables|Default|GetAs%20BP%20PS%20Mousen))
                  (CallFunction|ServerApplyStun)))
              (:then_1
                (CallFunction|ServerTickDamage))
              (:then_2
                (CallFunction|BeginDestroy)))))
        (:Is%20Not%20Valid
          (CallFunction|BeginDestroy))))))

(event EventTick
  (params (DeltaSeconds :type Float%20%28single-precision%29))
  ;[1 1 1 1 80] Set second beam start and end
  (Class|ParticleSystemComponent|SetBeamSourceTangent (Variables|Default|GetLightning) 0 "0, 0, 0")
  (Class|ParticleSystemComponent|SetBeamSourcePoint (Variables|Default|GetLightning) 0 (Variables|Default|GetStartPoint))
  (Class|ParticleSystemComponent|SetBeamTargetPoint (Variables|Default|GetLightning) 0 (Variables|Default|GetEndPoint))
  ;[1 1 1 1 80] Set second beam start and end
  (Class|ParticleSystemComponent|SetBeamSourceTangent (Variables|Default|GetLightning) 1 (Variables|Default|GetLocalImpactNormal))
  (Class|ParticleSystemComponent|SetBeamSourcePoint (Variables|Default|GetLightning) 1 (Variables|Default|GetStartPoint))
  (Class|ParticleSystemComponent|SetBeamTargetPoint (Variables|Default|GetLightning) 1 (Variables|Default|GetEndPoint)))

(fn ConstructionScript)

(fn GetMovementComponent
  (return 0))

(fn GetProjectileMovementComponent
  (return 0))