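; Spell actor: a fiery cube that orbits its instigator and damages enemy-team players on contact.
; Tick spins the actor's yaw and places it along its forward vector from the caster.
; Overlaps with I_Damage targets apply server-side point damage through player controller 0, then disable the cube briefly, with multicasts toggling Niagara fire and material.
; It destroys itself when the caster dies or the player-state reset event fires.
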(event OnComponentBeginOverlap(Collision)
  (params (OverlappedComponent :type Primitive%20Component%20Object%20Reference) (OtherActor :type Actor%20Object%20Reference) (OtherComp :type Primitive%20Component%20Object%20Reference) (OtherBodyIndex :type Integer) (bFromSweep :type Boolean) (SweepResult :type Hit%20Result%20Structure%20%28by%20ref%29))
  (if (Variables|Default|GetCanDamage?)
    (if (!= OtherActor (Variables|Default|GetInstigator))
      (if (Utilities|DoesObjectImplementInterface OtherActor "/Game/ThirdPerson/Blueprints/Gameplay/I_Damage.I_Damage_C")
        (if (!= (Math|Conversions|ToInteger(Byte) (Variables|/Game/ThirdPerson/Blueprints/Gameplay/BP_PS_Mousen.BP_PS_Mousen_C|GetPlayerTeam (.AsBP%20PS%20Mousen (Utilities|Casting|CastToBP_PS_Mousen (Variables|/Script/Engine.Pawn|GetPlayerState (Variables|Default|GetInstigator)))))) (Math|Conversions|ToInteger(Byte) (Variables|/Game/ThirdPerson/Blueprints/Gameplay/BP_PS_Mousen.BP_PS_Mousen_C|GetPlayerTeam (.AsBP%20PS%20Mousen (Utilities|Casting|CastToBP_PS_Mousen (Variables|/Script/Engine.Pawn|GetPlayerState (.AsBP%20Third%20Person%20Character (Utilities|Casting|CastToBP_ThirdPersonCharacter OtherActor))))))))
          (if (Networking|IsServer)
            (CallFunction|ServerApplyDamage :DamagedActor OtherActor :Damage (Variables|Default|GetDamage) :Instigated%20By (Variables|Default|GetAs%20BP%20PC%20Mousen) :DamageCauser (Variables|Default|GetInstigator))
            (CallFunction|ServerTurnOffCube)
            (Utilities|Time|SetTimerbyEvent (delegate Custom|Server%20Restart%20Cube) 2.0)))))))

(event Custom|Server%20Apply%20Damage
  (params (DamagedActor :type Actor%20Object%20Reference) (Damage :type Float%20%28double-precision%29) (Hit%20Direction :type Vector) (Hit%20Info :type Hit%20Result%20Structure) (Instigated%20By :type Controller%20Object%20Reference) (DamageCauser :type Actor%20Object%20Reference) (Damage%20Type%20Class :type Damage%20Type%20Class%20Reference))
  (Default|ApplyPointDamage (Variables|Default|GetAs%20BP%20PC%20Mousen) DamagedActor Damage Hit%20Direction Hit%20Info Instigated%20By DamageCauser Damage%20Type%20Class))

(event Custom|Server%20Bindings
  (EventDispatchers|BindEventtoPSPlayerReset (Variables|Default|GetAs%20BP%20PC%20Mousen) (delegate Custom|CleanupResources))
  (bind _asbp_third_person_character (Utilities|Casting|CastToBP_ThirdPersonCharacter (Variables|Default|GetInstigator)))
  (EventDispatchers|BindEventtoPlayerDied _asbp_third_person_character (delegate Custom|CleanupResources)))

(event Custom|CleanupResources
  (Actor|DestroyActor))

(event Custom|Multicast%20Restart%20Cube
  (Components|Activation|Activate (Variables|Default|GetNiagaraProjectileFire) true)
  (Rendering|Material|SetMaterial (Variables|Default|GetStaticMesh) 0 0))

(event Custom|Server%20Restart%20Cube
  (Variables|Default|SetCanDamage? true)
  (CallFunction|MulticastRestartCube))

(event Custom|Server%20Turn%20Off%20Cube
  (Variables|Default|SetCanDamage? false)
  (CallFunction|MulticastTurnOffCube))

(event Custom|Multicast%20Turn%20Off%20Cube
  (Components|Activation|Deactivate (Variables|Default|GetNiagaraProjectileFire))
  (Rendering|Material|SetMaterial (Variables|Default|GetStaticMesh) 0 0))

(event EventBeginPlay
  (Variables|Default|SetCubeMaterials (Rendering|Material|GetMaterials (Variables|Default|GetStaticMesh)))
  (bind _asbp_pc_mousen (Utilities|Casting|CastToBP_PC_Mousen (Game|GetPlayerController 0)))
  (Variables|Default|SetAs%20BP%20PC%20Mousen _asbp_pc_mousen)
  (Variables|Default|SetAs%20BP%20PS%20Mousen (.AsBP%20PS%20Mousen (Utilities|Casting|CastToBP_PS_Mousen (Variables|/Script/Engine.Pawn|GetPlayerState (Variables|Default|GetInstigator)))))
  (CallFunction|ServerBindings))

(event EventTick
  (params (DeltaSeconds :type Float%20%28single-precision%29))
  (Transformation|SetActorLocation (+ (Transformation|GetActorLocation (Variables|Default|GetInstigator)) (* (Math|Vector|Normalize (Transformation|GetActorForwardVector)) (Variables|Default|GetDistanceFromCenter))) false false)
  (Transformation|AddActorLocalRotation (Math|Rotator|MakeRotator 0.0 0.0 (* (* (/ 3.6e+02 (Variables|Default|GetTimeToRotateFully)) DeltaSeconds) (Variables|Default|GetDirection))) false false))

(event EventResetMaterial
  (params (Actor%20Component :type Actor%20Component%20Object%20Reference) (Actor :type Actor%20Object%20Reference))
  (Rendering|SetVisibility (Variables|Default|GetNiagaraProjectileFire) true false)
  (for (_array_element _array_index) (Variables|Default|GetCubeMaterials)
    (Rendering|Material|SetMaterial (Variables|Default|GetStaticMesh) _array_index _array_element)))

(event EventSetMaterial
  (params (Actor :type Actor%20Object%20Reference) (Owner%20Material :type Material%20Instance%20Object%20Reference) (Others%20Material :type Material%20Instance%20Object%20Reference))
  (Rendering|SetVisibility (Variables|Default|GetNiagaraProjectileFire) false false))

(fn ConstructionScript)

(fn GetCharacterMovement
  (return 0))

(fn GetMesh
  (return (Variables|Default|GetStaticMesh)))

(fn GetMovementComponent
  (return 0))

(fn GetPhysicalComponent
  (return 0))

(fn GetProjectileMovementComponent
  (return 0))

(fn GetSkeletalMesh
  (return 0))

(fn GetStatusEffectCount
  (params (Name :type Name :default "None"))
  (return 0))

(fn HasStatusEffectsThatPreventAttacking
  (return false))

(fn HasStatusEffectsThatPreventCasting
  (return false))

(fn HasStatusEffectsThatPreventJumping
  (return false))

(fn HasStatusEffectsThatPreventMovement
  (return false))

(fn HasStatusEffectsThatPreventSliding
  (return false))