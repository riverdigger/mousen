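; Wall spell actor that pushes out in front of the caster's camera, slowing enemies and intercepted projectiles.
; A timeline lerps it to the target point; with the Tower Shield item it then keeps tracking the camera's position and rotation.
; Overlap applies a server-side slow to opposing-team actors.
; ApplyCollision disables projectile collision and caps speed, repositioning fast ones via a backward trace with color pulse and impact sound.
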(event OnComponentBeginOverlap(StaticMeshCollision)
  (params (OverlappedComponent :type Primitive%20Component%20Object%20Reference) (OtherActor :type Actor%20Object%20Reference) (OtherComp :type Primitive%20Component%20Object%20Reference) (OtherBodyIndex :type Integer) (bFromSweep :type Boolean) (SweepResult :type Hit%20Result%20Structure%20%28by%20ref%29))
  (if (Utilities|DoesObjectImplementInterface OtherActor "/Game/Spells/StatusEffects/Interfaces/I_Status_Slow.I_Status_Slow_C")
    (if (Networking|IsServer)
      (if (!= (Variables|/Game/ThirdPerson/Blueprints/Gameplay/BP_PS_Mousen.BP_PS_Mousen_C|GetPlayerTeam (.AsBP%20PS%20Mousen (Utilities|Casting|CastToBP_PS_Mousen (Variables|/Script/Engine.Pawn|GetPlayerState (.AsBP%20Third%20Person%20Character (Utilities|Casting|CastToBP_ThirdPersonCharacter OtherActor)))))) (Math|Conversions|ToInteger(Byte) (Variables|/Game/ThirdPerson/Blueprints/Gameplay/BP_PS_Mousen.BP_PS_Mousen_C|GetPlayerTeam (.AsBP%20PS%20Mousen (Utilities|Casting|CastToBP_PS_Mousen (Variables|/Script/Engine.Pawn|GetPlayerState (.AsBP%20Third%20Person%20Character (Utilities|Casting|CastToBP_ThirdPersonCharacter (Components|GetOwner)))))))))
        (Class|IStatusSlow|OnSlowed(Message) OtherActor "/Game/Spells/StatusEffects/Blueprints/BP_Status_Effect_Slowed.BP_Status_Effect_Slowed_C" 1.0 0.45)))))

(event Custom|Server%20Pulse%20Forwards
  ;[1 1 1] Begin Play
  (bind _alpha (Timeline|Timeline PlayFromStart)
    (:Update
      (if (Variables|Default|GetHas%20Tower%20Shield?)
        (Transformation|SetActorLocationAndRotation (Math|Vector|Lerp(Vector) (Variables|Default|GetStartPoint) (Variables|Default|GetEndPoint) _alpha) (Transformation|GetWorldRotation (Variables|Default|GetThirdPersonCamera)))
        (else
          (Transformation|SetActorLocation self (Math|Vector|Lerp(Vector) (Variables|Default|GetStartPoint) (Variables|Default|GetEndPoint) _alpha) true false))))
    (:Finished
      (Variables|Default|SetFinishedTimeline true))))

(event Custom|Multicast%20Play%20Sound
  ;[1 1 1] Begin Play
  (Audio|SpawnSoundAttached "/Game/Sounds/Character/Melee/ProjectileWall/MS_Projectile_Wall.MS_Projectile_Wall" (Variables|Default|GetStaticMesh) "None" "0, 0, 0" "0, 0, 0" "KeepRelativeOffset" false 1.0 1.0 0.0 0 0))

(event Custom|Server%20Update%20Color
  (bind _alpha (Timeline|ColorImpact PlayFromStart)
    (:Update
      (Rendering|Material|SetScalarParameterValueonMaterials (Variables|Default|GetStaticMesh) "Color Intensity" _alpha))))

(event Custom|Multicast%20Play%20Impact%20Sound
  ;[1 1 1] Begin Play
  (Audio|SpawnSoundAttached "/Game/Sounds/Character/Melee/ProjectileWall/MS_Projectile_Wall_Impact.MS_Projectile_Wall_Impact" (Variables|Default|GetStaticMesh) "None" "0, 0, 0" "0, 0, 0" "KeepRelativeOffset" false 1.0 1.0 0.0 0 0))

(event EventBeginPlay
  ;[1 1 1] Begin Play
  (bind _output_get (Variables|Default|SetThirdPersonCharacter (.AsBP%20Third%20Person%20Character (Utilities|Casting|CastToBP_ThirdPersonCharacter (Variables|Default|GetInstigator)))))
  (Variables|Default|SetHas%20Tower%20Shield? (Variables|/Game/ThirdPerson/Blueprints/Gameplay/BP_PS_Mousen.BP_PS_Mousen_C|GetHasTowerShield? (.AsBP%20PS%20Mousen (Utilities|Casting|CastToBP_PS_Mousen (Variables|/Script/Engine.Pawn|GetPlayerState _output_get)))))
  (bind _camera (Class|ICharacter|GetCamera(Message) _output_get))
  (Variables|Default|SetThirdPersonCamera _camera)
  (Variables|Default|SetStartPoint (Transformation|GetActorLocation))
  (Variables|Default|SetEndPoint (+ (* (Math|Vector|GetForwardVector (Variables|Default|GetThirdPersonCamera)) 7.5e+02) (Transformation|GetWorldLocation (Variables|Default|GetThirdPersonCamera))))
  (CallFunction|ServerPulseForwards)
  (CallFunction|MulticastPlaySound))

(event EventApplyCollision
  (params (Projectile :type Actor%20Object%20Reference) (Projectile%20Movement :type Projectile%20Movement%20Component%20Object%20Reference))
  (bind _returnvalue (Transformation|GetActorLocation Projectile))
  (bind _velocity (Variables|/Script/Engine.MovementComponent|GetVelocity Projectile%20Movement))
  (bind _returnvalue_2 (Math|Vector|Normalize _velocity))
  (Class|IProjectile|DisableCollision(Message) Projectile 2.0)
  (if (> (Math|Vector|VectorLength _velocity) 7.5e+02)
    (Variables|/Script/Engine.ProjectileMovementComponent|SetMaxSpeed Projectile%20Movement 75.0)
    (bind (_outhit _returnvalue_3) (Collision|LineTraceByChannel _returnvalue (+ _returnvalue (* _returnvalue_2 -4e+02)) "TraceTypeQuery1" false 0 "None" false))
    (Transformation|SetActorLocation Projectile (Math|Vector|SelectVector (- (.ImpactPoint (Collision|BreakHitResult _outhit)) (* _returnvalue_2 1e+02)) (Transformation|GetActorLocation) _returnvalue_3) false false)
    (CallFunction|ServerUpdateColor)
    (CallFunction|MulticastPlayImpactSound)
    (else
      (Variables|/Script/Engine.ProjectileMovementComponent|SetMaxSpeed Projectile%20Movement 75.0))))

(event EventTick
  (params (DeltaSeconds :type Float%20%28single-precision%29))
  (bind _thirdpersoncamera (Variables|Default|GetThirdPersonCamera))
  (bind _thirdpersoncamera_2 (Variables|Default|GetThirdPersonCamera))
  ;[1 1 1] Event tick
  ;;[1 1 1] Has item?
  (if (Variables|Default|GetHas%20Tower%20Shield?)
    (Variables|Default|SetEndPoint (+ (* (Math|Vector|GetForwardVector _thirdpersoncamera_2) 7.5e+02) (Transformation|GetWorldLocation _thirdpersoncamera_2)))
    (if (Variables|Default|GetFinishedTimeline)
      (Transformation|SetActorLocationAndRotation (+ (* (Math|Vector|GetForwardVector _thirdpersoncamera) 7.5e+02) (Transformation|GetWorldLocation _thirdpersoncamera)) (Transformation|GetWorldRotation _thirdpersoncamera_2)))))

(fn ConstructionScript)

(fn GetProjectileMovement
  (return 0))