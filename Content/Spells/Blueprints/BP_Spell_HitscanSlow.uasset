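; Hitscan lightning beam spell actor that continuously damages what it hits, fired from the caster's spell spawn point along the camera's forward vector.
; Each tick it shrinks its range toward a minimum, sphere-traces, then moves the sparks, mesh and two jittered beam emitters to the resulting endpoint.
; On the server, hit actors implementing I_Damage take point damage every tick.
; An older delay-looped trace is disconnected, and no slow effect appears here.
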(event Custom|Server%20Apply%20Damage
  (params (DamagedActor :type Actor%20Object%20Reference) (Damage :type Float%20%28double-precision%29) (Hit%20Direction :type Vector) (Hit%20Info :type Hit%20Result%20Structure) (Instigated%20By :type Controller%20Object%20Reference) (DamageCauser :type Actor%20Object%20Reference) (Damage%20Type%20Class :type Damage%20Type%20Class%20Reference))
  (Default|ApplyPointDamage (Variables|Default|GetAs%20BP%20PC%20Mousen) DamagedActor Damage Hit%20Direction Hit%20Info Instigated%20By DamageCauser Damage%20Type%20Class))

(event EventBeginPlay
  (bind _asbp_pc_mousen (Utilities|Casting|CastToBP_PC_Mousen (Game|GetPlayerController 0)))
  (Variables|Default|SetAs%20BP%20PC%20Mousen _asbp_pc_mousen)
  (Variables|Default|SetAs%20BP%20Third%20Person%20Magic (.AsBP%20Third%20Person%20Magic (Utilities|Casting|CastToBP_ThirdPerson_Magic (Variables|Default|GetInstigator)))))

(event EventTick
  (params (DeltaSeconds :type Float%20%28single-precision%29))
  (bind _lightning (Variables|Default|GetLightning))
  (bind _as_bp_third_person_magic (Variables|Default|GetAs%20BP%20Third%20Person%20Magic))
  (bind _lightning_2 (Variables|Default|GetLightning))
  (Variables|Default|SetStartPoint (Transformation|GetWorldLocation (Variables|/Game/ThirdPerson/Blueprints/Magic/BP_ThirdPerson_Magic.BP_ThirdPerson_Magic_C|GetSpellSpawn (Variables|Default|GetAs%20BP%20Third%20Person%20Magic))))
  (if (> (Variables|Default|GetDistance) 1e+02)
    (Variables|Default|SetDistance (- (Variables|Default|GetDistance) 2.0)))
  (Variables|Default|SetEndPoint (+ (Transformation|GetWorldLocation (Variables|/Game/ThirdPerson/Blueprints/Magic/BP_ThirdPerson_Magic.BP_ThirdPerson_Magic_C|GetSpellSpawn _as_bp_third_person_magic)) (* (Math|Vector|GetForwardVector (Variables|/Script/Mousen.MousenCharacter|GetFollowCamera _as_bp_third_person_magic)) (Variables|Default|GetDistance))))
  (bind (_outhit _returnvalue) (Collision|SphereTraceByChannel (Variables|Default|GetStartPoint) (Variables|Default|GetEndPoint) 25.0 "TraceTypeQuery1" false (Utilities|Array|MakeArray (Variables|Default|GetInstigator)) "None"))
  (if _returnvalue
    (Variables|Default|SetEndPoint (.ImpactPoint (Collision|BreakHitResult _outhit))))
  (Transformation|SetWorldLocation (Variables|Default|GetSparks) (Variables|Default|GetEndPoint) false false)
  (Transformation|SetWorldLocation (Variables|Default|GetStaticMesh) (Variables|Default|GetEndPoint) false false)
  (Utilities|FlowControl|Sequence
    (:then_0
      (Class|ParticleSystemComponent|SetBeamSourceTangent _lightning_2 0 (Math|Vector|MakeVector 1.0 0.0 (Math|Conversions|ToFloat(Integer) (Math|Random|RandomIntegerinRange -20 20))))
      (Class|ParticleSystemComponent|SetBeamSourcePoint _lightning_2 0 (Variables|Default|GetStartPoint))
      (Class|ParticleSystemComponent|SetBeamTargetPoint _lightning_2 0 (Variables|Default|GetEndPoint)))
    (:then_1
      (Class|ParticleSystemComponent|SetBeamSourceTangent _lightning 1 (Math|Vector|MakeVector 1.0 0.0 (Math|Conversions|ToFloat(Integer) (Math|Random|RandomIntegerinRange -20 20))))
      (Class|ParticleSystemComponent|SetBeamSourcePoint _lightning 1 (Variables|Default|GetStartPoint))
      (Class|ParticleSystemComponent|SetBeamTargetPoint _lightning 1 (Variables|Default|GetEndPoint)))
    (:then_2
      (if (Utilities|DoesObjectImplementInterface (.HitActor (Collision|BreakHitResult _outhit)) "/Game/ThirdPerson/Blueprints/Gameplay/I_Damage.I_Damage_C")
        (if (Networking|IsServer)
          (CallFunction|ServerApplyDamage :DamagedActor (.HitActor (Collision|BreakHitResult _outhit)) :Damage (Variables|Default|GetDamage) :Hit%20Direction (.ImpactNormal (Collision|BreakHitResult _outhit)) :Instigated%20By (Variables|Default|GetAs%20BP%20PC%20Mousen) :DamageCauser (Variables|Default|GetInstigator) :Damage%20Type%20Class "/Script/Engine.DamageType"))))))

(fn ConstructionScript)

(fn GetMovementComponent
  (return 0))

(fn GetProjectileMovementComponent
  (return 0))