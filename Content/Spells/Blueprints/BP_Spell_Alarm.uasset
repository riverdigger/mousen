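; Alarm trap spell that reveals characters entering its sphere, filtered by caster and team flags, and unmarks them on exit.
; A server-side overlap applies the seen overlay, adds a stun with the caster's trap upgrade, multicasts a sound and starts delayed self-destruction.
; A second sphere sets emissive and shows a HUD prompt for non-teammates, whose timed interaction destroys the trap.
; The caster's player-reset event also destroys it.
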(event OnComponentBeginOverlap(InteractSphere)
  (params (OverlappedComponent :type Primitive%20Component%20Object%20Reference) (OtherActor :type Actor%20Object%20Reference) (OtherComp :type Primitive%20Component%20Object%20Reference) (OtherBodyIndex :type Integer) (bFromSweep :type Boolean) (SweepResult :type Hit%20Result%20Structure%20%28by%20ref%29))
  (bind _asbp_third_person_character (Utilities|Casting|CastToBP_ThirdPersonCharacter OtherActor))
  (bind _can_interact (Default|CanInteract self _asbp_third_person_character))
  (if _can_interact
    (CallFunction|ServerSetVisibility)
    (Utilities|IsValid (Pawn|GetLocalViewingPlayerController _asbp_third_person_character)
      (:Is%20Valid
        (Default|ShowInteract (.AsBP%20HUD%20Mousen (Utilities|Casting|CastToBP_HUD_Mousen (HUD|GetHUD (Pawn|GetLocalViewingPlayerController _asbp_third_person_character)))) (Transformation|GetWorldLocation (Variables|Default|GetInteractPoint)))))))

(event OnComponentEndOverlap(InteractSphere)
  (params (OverlappedComponent :type Primitive%20Component%20Object%20Reference) (OtherActor :type Actor%20Object%20Reference) (OtherComp :type Primitive%20Component%20Object%20Reference) (OtherBodyIndex :type Integer))
  (bind _asbp_third_person_character (Utilities|Casting|CastToBP_ThirdPersonCharacter OtherActor))
  (Utilities|IsValid (Pawn|GetLocalViewingPlayerController _asbp_third_person_character)
    (:Is%20Valid
      (Default|HideInteract (.AsBP%20HUD%20Mousen (Utilities|Casting|CastToBP_HUD_Mousen (HUD|GetHUD (Pawn|GetLocalViewingPlayerController _asbp_third_person_character))))))))

(event OnComponentBeginOverlap(Sphere)
  (params (OverlappedComponent :type Primitive%20Component%20Object%20Reference) (OtherActor :type Actor%20Object%20Reference) (OtherComp :type Primitive%20Component%20Object%20Reference) (OtherBodyIndex :type Integer) (bFromSweep :type Boolean) (SweepResult :type Hit%20Result%20Structure%20%28by%20ref%29))
  (bind _as_bp_ps_mousen (Variables|Default|GetAs%20BP%20PS%20Mousen))
  (if (Networking|IsServer)
    (if (== OtherActor (Variables|Default|GetInstigator))
      (if (Variables|Default|GetAffectsCaster?)
        (if true :!label _label
          (Class|IStatusSeen|OnSeen(Message) OtherActor 0 (Variables|Default|GetOverlayMaterial) 9999.0 self)
          (if (Variables|/Game/ThirdPerson/Blueprints/Gameplay/BP_PS_Mousen.BP_PS_Mousen_C|GetHasTrapUpgrade? _as_bp_ps_mousen)
            (Class|IStatusStun|OnStun(Message) OtherActor "/Game/Spells/StatusEffects/Blueprints/BP_Status_Effect_Stunned.BP_Status_Effect_Stunned_C" (Variables|/Game/ThirdPerson/Blueprints/Gameplay/BP_PS_Mousen.BP_PS_Mousen_C|GetTrapStunDuration _as_bp_ps_mousen) self))
          (CallFunction|ServerStartAlarm)
          (Variables|Default|SetRecentActor OtherActor)
          (Utilities|FlowControl|DoOnce false
            (:Completed
              (Utilities|FlowControl|Sequence
                (:then_0
                  (Utilities|FlowControl|Delay (Variables|Default|GetDelayedLifespan))
                  (Actor|DestroyActor self)))))))
      (elif (!= (Math|Conversions|ToInteger(Byte) (Variables|/Game/ThirdPerson/Blueprints/Gameplay/BP_PS_Mousen.BP_PS_Mousen_C|GetPlayerTeam (.AsBP%20PS%20Mousen (Utilities|Casting|CastToBP_PS_Mousen (Variables|/Script/Engine.Pawn|GetPlayerState (.AsBP%20Third%20Person%20Character (Utilities|Casting|CastToBP_ThirdPersonCharacter OtherActor))))))) (Math|Conversions|ToInteger(Byte) (Variables|/Game/ThirdPerson/Blueprints/Gameplay/BP_PS_Mousen.BP_PS_Mousen_C|GetPlayerTeam (.AsBP%20PS%20Mousen (Utilities|Casting|CastToBP_PS_Mousen (Variables|/Script/Engine.Pawn|GetPlayerState (Variables|Default|GetInstigator)))))))
        (goto _label)
        (elif (Variables|Default|GetAffectsTeammates?)
          (goto _label))))))

(event OnComponentEndOverlap(Sphere)
  (params (OverlappedComponent :type Primitive%20Component%20Object%20Reference) (OtherActor :type Actor%20Object%20Reference) (OtherComp :type Primitive%20Component%20Object%20Reference) (OtherBodyIndex :type Integer))
  (if (Networking|IsServer)
    (Class|IStatusSeen|OnUnSeen(Message) OtherActor 0 self)))

(event Custom|CleanupResources
  (Actor|DestroyActor))

(event Custom|Server%20Start%20Alarm
  (CallFunction|MulticastStartAlarm))

(event Custom|Multicast%20Start%20Alarm
  (Audio|PlaySoundatLocation "/Engine/VREditor/Sounds/VR_teleport.VR_teleport" (Transformation|GetActorLocation self) "0, 0, 0" 1.0 1.0 0.0 0 0 0 0))

(event Custom|Server%20Bindings
  (EventDispatchers|BindEventtoPSPlayerReset (Variables|Default|GetAs%20BP%20PC%20Mousen) (delegate Custom|CleanupResources)))

(event Custom|Multicast%20Set%20Visibility
  (Rendering|Material|SetScalarParameterValueonMaterials (Variables|Default|GetCylinder) "Emissive" 0.05))

(event Custom|Server%20Set%20Visibility
  (CallFunction|MulticastSetVisibility))

(event Custom|Multicast%20Set%20Rotation
  (params (Target :type Scene%20Component%20Object%20Reference) (NewRotation :type Rotator))
  (Transformation|SetWorldRotation Target NewRotation false false))

(event Custom|Server%20Set%20Rotation
  (params (Target :type Scene%20Component%20Object%20Reference) (NewRotation :type Rotator))
  (CallFunction|MulticastSetRotation Target NewRotation))

(event EventBeginPlay
  (bind _asbp_pc_mousen (Utilities|Casting|CastToBP_PC_Mousen (Pawn|GetController (Variables|Default|GetInstigator))))
  (bind _output_get (Variables|Default|SetAs%20BP%20PC%20Mousen _asbp_pc_mousen))
  (Variables|Default|SetAs%20BP%20PS%20Mousen (.AsBP%20PS%20Mousen (Utilities|Casting|CastToBP_PS_Mousen (Variables|/Script/Engine.Controller|GetPlayerState _output_get))))
  (CallFunction|ServerBindings))

(event EventInteract
  (params (Player :type Character%20Object%20Reference))
  (Actor|DestroyActor self))

(fn ConstructionScript)

(fn CanInteract
  (params (Player%20Character :type Character%20Object%20Reference))
  (bind _asbp_third_person_character (Utilities|Casting|CastToBP_ThirdPersonCharacter Player%20Character)
    (:then
      (bind _asbp_ps_mousen (Utilities|Casting|CastToBP_PS_Mousen (Variables|/Script/Engine.Pawn|GetPlayerState _asbp_third_person_character))
        (:then
          (if (Utilities|Enum|NotEqual(Enum) (Variables|/Game/ThirdPerson/Blueprints/Gameplay/BP_PS_Mousen.BP_PS_Mousen_C|GetPlayerTeam _asbp_ps_mousen) (Variables|/Game/ThirdPerson/Blueprints/Gameplay/BP_PS_Mousen.BP_PS_Mousen_C|GetPlayerTeam (Variables|Default|GetAs%20BP%20PS%20Mousen)))
            _
            (else
              (return false))))
        (:CastFailed
          _)))
    (:CastFailed
      _))
  (return true))

(fn GetInteractTimeSeconds
  (return 1.75 false))