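; BP_Spell_Tornado is a timed tornado spell actor that throws characters it touches into the air.
; Capsule overlaps call MulticastApplyImpulse, which casts to Character and launches it straight up with a fixed velocity, overriding only Z.
; BeginPlay caches the first player controller as BP_PC_Mousen, unused elsewhere here, then destroys the actor after Lifetime.
; A failed controller cast skips that timed destruction.
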(event OnComponentBeginOverlap(Capsule)
  (params (OverlappedComponent :type Primitive%20Component%20Object%20Reference) (OtherActor :type Actor%20Object%20Reference) (OtherComp :type Primitive%20Component%20Object%20Reference) (OtherBodyIndex :type Integer) (bFromSweep :type Boolean) (SweepResult :type Hit%20Result%20Structure%20%28by%20ref%29))
  (CallFunction|MulticastApplyImpulse OtherActor))

(event Custom|Multicast%20Apply%20Impulse
  (params (Actor :type Actor%20Object%20Reference))
  (bind _ascharacter (Utilities|Casting|CastToCharacter Actor))
  (Character|LaunchCharacter _ascharacter "0, 0,1750.000000" false true))

(event EventBeginPlay
  (bind _asbp_pc_mousen (Utilities|Casting|CastToBP_PC_Mousen (Game|GetPlayerController 0)))
  (Variables|Default|SetAs%20BP%20PC%20Mousen _asbp_pc_mousen)
  (Utilities|FlowControl|Delay (Variables|Default|GetLifetime))
  (Actor|DestroyActor))

(fn ConstructionScript)