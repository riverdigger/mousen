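; BP_Spell_Cage_Pillar is one projectile pillar of the cage spell, owned by a BP_Spell_Cage.
; On box overlap it stops; the server reports a completed spike, enables rock collision and moves two gates vertically via timeline.
; A Lifespan timer stops and reports any pillar that never collided, without destroying it.
; It destroys itself with the cage and receives its neighbor reference by multicast; ServerActivateFence is empty.
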(event OnComponentBeginOverlap(Box)
  (params (OverlappedComponent :type Primitive%20Component%20Object%20Reference) (OtherActor :type Actor%20Object%20Reference) (OtherComp :type Primitive%20Component%20Object%20Reference) (OtherBodyIndex :type Integer) (bFromSweep :type Boolean) (SweepResult :type Hit%20Result%20Structure%20%28by%20ref%29))
  (bind _gate (Variables|Default|GetGate))
  (bind _projectilemovement (Variables|Default|GetProjectileMovement))
  (bind _gate1 (Variables|Default|GetGate1))
  (bind _relativelocation (Variables|/Script/Engine.SceneComponent|GetRelativeLocation _gate))
  (bind _relativelocation_2 (Variables|/Script/Engine.SceneComponent|GetRelativeLocation _gate1))
  (Components|Movement|StopMovementImmediately _projectilemovement)
  (Variables|/Script/Engine.ProjectileMovementComponent|SetProjectileGravityScale _projectilemovement 0.0)
  (if (Networking|IsServer)
    (Variables|Default|SetHasCollided? true)
    (Default|UpdateCompletedSpikes (Variables|Default|GetSpellCage))
    (Collision|SetCollisionEnabled (Variables|Default|GetRockStaticMesh) "QueryAndPhysics")
    (bind (_direction _sizepercentage _barheight) (Timeline|Shrink%20Timeline PlayFromStart)
      (:Update
        (Transformation|SetRelativeLocation _gate (Math|Vector|MakeVector (.x _relativelocation) (.y _relativelocation) _barheight) true false)
        (Transformation|SetRelativeLocation _gate1 (Math|Vector|MakeVector (.x _relativelocation_2) (.y _relativelocation_2) _barheight) true false)))))

(event Custom|CleanupResources
  (Actor|DestroyActor))

(event Custom|Multicast%20Set%20Neighbor
  (params (NeighborBehind :type BP%20Spell%20Cage%20Spike%20Object%20Reference))
  (Variables|Default|SetNeighborBehind NeighborBehind))

(event Custom|Server%20Set%20Neighbor
  (params (NeighborBehind :type BP%20Spell%20Cage%20Spike%20Object%20Reference))
  (CallFunction|MulticastSetNeighbor NeighborBehind))

(event Custom|Server%20Activate%20Fence)

(event Custom|Server%20Bindings
  (EventDispatchers|BindEventtoCageDestroyed (Variables|Default|GetSpellCage) (delegate Custom|CleanupResources)))

(event Custom|Destroy%20Self
  (bind _projectilemovement (Variables|Default|GetProjectileMovement))
  (if (not (Variables|Default|GetHasCollided?))
    (Components|Movement|StopMovementImmediately _projectilemovement)
    (Variables|/Script/Engine.ProjectileMovementComponent|SetProjectileGravityScale _projectilemovement 0.0)
    (Variables|Default|SetHasCollided? true)
    (Default|UpdateCompletedSpikes (Variables|Default|GetSpellCage))))

(event EventBeginPlay
  (Variables|Default|SetSpellCage (.AsBP%20Spell%20Cage (Utilities|Casting|CastToBP_Spell_Cage (Components|GetOwner))))
  (CallFunction|ServerBindings)
  (Utilities|Time|SetTimerbyEvent (delegate Custom|Destroy%20Self) (Variables|Default|GetLifespan)))

(fn ConstructionScript
  (|CallParentFunction))