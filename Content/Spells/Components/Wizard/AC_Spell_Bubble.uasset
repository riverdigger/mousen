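; Wizard spell component for the Bubble spell, fired directly from the first magic spell input.
; On initialization it rebuilds its spell data, granting one extra max and initial count when the player state has Hurricane.
; On input it checks count and castability through owner messages, restarts the cast montage sped up, cancels other spells, then sets and immediately casts itself before running post-cast logic.
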(event Input|EnhancedActionEvents|EnhancedInputActionIA_Magic_SpellOne
  (params (ActionValue :type Boolean) (ElapsedSeconds :type Float%20%28double-precision%29) (TriggeredSeconds :type Float%20%28double-precision%29) (InputAction :type Input%20Action%20Object%20Reference :default "/Game/Inputs/Magic/IA_Magic_SpellOne.IA_Magic_SpellOne"))
  (bind _returnvalue (Components|GetOwner))
  (bind _returnvalue_2 (Components|GetOwner))
  (bind _returnvalue_3 (Components|GetOwner))
  (:Started
    (bind _spell_count (Class|ISpellcaster|GetSpellCount(Message) _returnvalue (Variables|Default|GetSpell%20Components)))
    (bind _can_cast (Class|ISpellcaster|CanCast(Message) _returnvalue _spell_count))
    (if _can_cast
      (Class|ISpellcaster|SpellcastingStopMontage(Message) _returnvalue_2 "/Game/FrogNomad/Animations/Standing_2H_Magic_Attack_01_Montage.Standing_2H_Magic_Attack_01_Montage")
      (Class|ISpellcaster|SpellcastingPlayMontage(Message) _returnvalue_2 "/Game/FrogNomad/Animations/Standing_2H_Magic_Attack_01_Montage.Standing_2H_Magic_Attack_01_Montage" 3.0)
      (Class|ISpellcaster|CancelAllSpells(Message) _returnvalue_3)
      (Class|ISpellcaster|SetActiveSpell(Message) _returnvalue_3 (Variables|Default|GetSpell%20Components))
      (Class|ISpellcaster|CastActiveSpell(Message) (Components|GetOwner))
      (CallFunction|PostSpellCast))))

(event EventInitializeSpellComponent
  (bind _player_state (Class|ICharacter|GetPlayerState(Message) (Components|GetOwner)))
  (bind _asbp_ps_mousen (Utilities|Casting|CastToBP_PS_Mousen _player_state))
  (Variables|Default|SetSpell%20Components (Utilities|Struct|MakeS_Spell_Components (.Name (Utilities|Struct|BreakS_Spell_Components (Variables|Default|GetSpell%20Components))) (.Class (Utilities|Struct|BreakS_Spell_Components (Variables|Default|GetSpell%20Components))) (.Indicator (Utilities|Struct|BreakS_Spell_Components (Variables|Default|GetSpell%20Components))) (.IndicatorType (Utilities|Struct|BreakS_Spell_Components (Variables|Default|GetSpell%20Components))) (.Cooldown (Utilities|Struct|BreakS_Spell_Components (Variables|Default|GetSpell%20Components))) (.Image (Utilities|Struct|BreakS_Spell_Components (Variables|Default|GetSpell%20Components))) (Math|Integer|SelectInt (+ (.MaxCount (Utilities|Struct|BreakS_Spell_Components (Variables|Default|GetSpell%20Components))) 1) (.MaxCount (Utilities|Struct|BreakS_Spell_Components (Variables|Default|GetSpell%20Components))) (Variables|/Game/ThirdPerson/Blueprints/Gameplay/BP_PS_Mousen.BP_PS_Mousen_C|GetHasHurricane? _asbp_ps_mousen)) (Math|Integer|SelectInt (+ (.InitialCount (Utilities|Struct|BreakS_Spell_Components (Variables|Default|GetSpell%20Components))) 1) (.InitialCount (Utilities|Struct|BreakS_Spell_Components (Variables|Default|GetSpell%20Components))) (Variables|/Game/ThirdPerson/Blueprints/Gameplay/BP_PS_Mousen.BP_PS_Mousen_C|GetHasHurricane? _asbp_ps_mousen)) (.InputAction (Utilities|Struct|BreakS_Spell_Components (Variables|Default|GetSpell%20Components))) (.CastingRange (Utilities|Struct|BreakS_Spell_Components (Variables|Default|GetSpell%20Components))) (.Type (Utilities|Struct|BreakS_Spell_Components (Variables|Default|GetSpell%20Components))))))