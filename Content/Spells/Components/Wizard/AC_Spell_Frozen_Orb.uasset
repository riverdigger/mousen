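; Wizard spell component for Frozen Orb, driven by the SpellThree input action and talking to its owner through message calls.
; Started checks castability, makes the spell active and starts its indicator, which Ongoing updates.
; Canceled casts if castable with a valid indicator, playing montage and server sound before PostSpellCast; otherwise it stops the indicator.
; Triggered cancels all spells through a DoOnce that resets only when Started cannot cast.
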(event Input|EnhancedActionEvents|EnhancedInputActionIA_Magic_SpellThree
  (params (ActionValue :type Boolean) (ElapsedSeconds :type Float%20%28double-precision%29) (TriggeredSeconds :type Float%20%28double-precision%29) (InputAction :type Input%20Action%20Object%20Reference :default "/Game/Inputs/Magic/IA_Magic_SpellThree.IA_Magic_SpellThree"))
  (bind _returnvalue (Components|GetOwner))
  (bind _returnvalue_2 (Components|GetOwner))
  (bind _returnvalue_3 (Components|GetOwner))
  (bind _returnvalue_4 (Components|GetOwner))
  (:Triggered
    (Utilities|FlowControl|DoOnce false :!label _label
      (:Completed
        (Class|ISpellcaster|CancelAllSpells(Message) (Components|GetOwner)))))
  (:Started
    (bind _spell_count (Class|ISpellcaster|GetSpellCount(Message) _returnvalue_2 (Variables|Default|GetSpell%20Components)))
    (bind _can_cast (Class|ISpellcaster|CanCast(Message) _returnvalue_2 _spell_count))
    (if _can_cast
      (Class|ISpellcaster|CancelAllSpells(Message) _returnvalue_4)
      (Class|ISpellcaster|SetActiveSpell(Message) _returnvalue_4 (Variables|Default|GetSpell%20Components))
      (Class|ISpellcaster|StartSpellIndicator(Message) (Components|GetOwner) (Variables|Default|GetSpell%20Components))
      (else
        (goto _label Reset))))
  (:Ongoing
    (Class|ISpellcaster|HeldSpellIndicator(Message) (Components|GetOwner) (Variables|Default|GetSpell%20Components)))
  (:Canceled
    (bind _spell_count_2 (Class|ISpellcaster|GetSpellCount(Message) _returnvalue (Variables|Default|GetSpell%20Components)))
    (bind _can_cast_2 (Class|ISpellcaster|CanCast(Message) _returnvalue _spell_count_2))
    (if _can_cast_2
      (bind _spell_indicator (Class|ISpellcaster|GetSpellIndicator(Message) (Components|GetOwner)))
      (Utilities|IsValid _spell_indicator
        (:Is%20Valid
          (if (Variables|/Game/Spells/Indicators/Blueprints/BP_Spell_Indicator.BP_Spell_Indicator_C|GetIsValid? _spell_indicator)
            (Class|ISpellcaster|SpellcastingStopMontage(Message) _returnvalue_3 "/Game/FrogNomad/Animations/Standing_2H_Magic_Attack_01_Montage.Standing_2H_Magic_Attack_01_Montage")
            (Class|ISpellcaster|SpellcastingPlayMontage(Message) _returnvalue_3 "/Game/FrogNomad/Animations/Standing_2H_Magic_Attack_01_Montage.Standing_2H_Magic_Attack_01_Montage" 3.0)
            (CallFunction|ServerPlaySoundAttached "/Game/Sounds/Character/Magic/FreezeOrb/MS_Freeze_Orb.MS_Freeze_Orb" (Variables|/Script/Engine.Actor|GetRootComponent (Components|GetOwner)))
            (Class|ISpellcaster|CastActiveSpell(Message) (Components|GetOwner))
            (CallFunction|PostSpellCast)
            (else
              (Class|ISpellcaster|StopSpellIndicator(Message) (Components|GetOwner) :!label _label_2))))
        (:Is%20Not%20Valid
          (goto _label_2)))
      (else
        (Class|ISpellcaster|StopSpellIndicator(Message) (Components|GetOwner))))))