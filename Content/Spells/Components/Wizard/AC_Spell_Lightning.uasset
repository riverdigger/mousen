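; Lightning primary spell component for the Wizard, cast from the primary spell input.
; On initialization it caches whether the player state holds a RotateCube or Planetary item, either of which blocks the spell.
; On press, if the owner can attack and no spell is charging, it cancels other spells, plays a sped-up cast montage and casts through owner message calls.
; Release or cancel stops all spells and that montage.
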(event Input|EnhancedActionEvents|EnhancedInputActionIA_Magic_SpellPrimary
  (params (ActionValue :type Boolean) (ElapsedSeconds :type Float%20%28double-precision%29) (TriggeredSeconds :type Float%20%28double-precision%29) (InputAction :type Input%20Action%20Object%20Reference :default "/Game/Inputs/Magic/IA_Magic_SpellPrimary.IA_Magic_SpellPrimary"))
  (bind _returnvalue (Components|GetOwner))
  (bind _returnvalue_2 (Components|GetOwner))
  (:Started
    (Variables|Default|SetIsBlocked? false)
    (bind _can_attack (Class|ISpellcaster|CanAttack(Message) (Components|GetOwner)))
    (bind _is_charging (Class|ISpellcaster|GetIsChargingSpell(Message) (Components|GetOwner)))
    (if (and _can_attack (not _is_charging))
      (if (not (Variables|Default|GetHasItemsThatBlockPrimary?))
        (for _array_element (Actor|GetComponentsByClass (Components|GetOwner) "/Game/Spells/Components/AC_Spell.AC_Spell_C")
          (if (Variables|/Game/Spells/Components/AC_Spell.AC_Spell_C|GetIsCharging? _array_element)
            (Variables|Default|SetIsBlocked? true)))
        (if (not (Variables|Default|GetIsBlocked?))
          (Class|ISpellcaster|SpellcastingStopMontage(Message) _returnvalue "/Game/FrogNomad/Animations/Standing_2H_Magic_Attack_01_Montage.Standing_2H_Magic_Attack_01_Montage")
          (Class|ISpellcaster|SpellcastingPlayMontage(Message) _returnvalue "/Game/FrogNomad/Animations/Standing_2H_Magic_Attack_04_Montage.Standing_2H_Magic_Attack_04_Montage" 3.0)
          (Class|ISpellcaster|CancelAllSpells(Message) _returnvalue_2)
          (Class|ISpellcaster|SetActiveSpell(Message) _returnvalue_2 (Variables|Default|GetSpell%20Components))
          (Class|ISpellcaster|CastActiveSpell(Message) (Components|GetOwner))
          (CallFunction|PostSpellCast)))))
  (:Canceled
    (Class|ISpellcaster|CancelAllSpells(Message) (Components|GetOwner) :!label _label)
    (Class|ISpellcaster|SpellcastingStopMontage(Message) (Components|GetOwner) "/Game/FrogNomad/Animations/Standing_2H_Magic_Attack_04_Montage.Standing_2H_Magic_Attack_04_Montage"))
  (:Completed
    (goto _label)))

(event EventInitializeSpellComponent
  (bind _player_state (Class|ICharacter|GetPlayerState(Message) (Components|GetOwner)))
  (bind _asbp_ps_mousen (Utilities|Casting|CastToBP_PS_Mousen _player_state))
  (Variables|Default|SetHasItemsThatBlockPrimary? (or (Variables|/Game/ThirdPerson/Blueprints/Gameplay/BP_PS_Mousen.BP_PS_Mousen_C|GetHasRotateCube? _asbp_ps_mousen) (Variables|/Game/ThirdPerson/Blueprints/Gameplay/BP_PS_Mousen.BP_PS_Mousen_C|GetHasPlanetary? _asbp_ps_mousen))))