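; Wizard spell component that makes its owner briefly invisible when the movement-spell input starts.
; After a cast check through owner interface messages, it cancels other spells, casts itself, applies the Invisible status effect and stops attack montages.
; If the player state's NowYouSeeMe flag, cached at initialization, is set, a server-named event also spawns a BP_Spell_Invisibility actor at the owner's transform for greater invisibility.
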(event Custom|Server%20Spawn%20Greater%20Invisibility
  (bind _returnvalue (Components|GetOwner))
  (Game|SpawnActorfromClass "/Game/Spells/Blueprints/BP_Spell_Invisibility.BP_Spell_Invisibility_C" (Transformation|GetActorTransform _returnvalue) "Undefined" "OverrideRootScale" _returnvalue (.AsPawn (Utilities|Casting|CastToPawn _returnvalue))))

(event Input|EnhancedActionEvents|EnhancedInputActionIA_SpellMovement
  (params (ActionValue :type Boolean) (ElapsedSeconds :type Float%20%28double-precision%29) (TriggeredSeconds :type Float%20%28double-precision%29) (InputAction :type Input%20Action%20Object%20Reference :default "/Game/Inputs/IA_SpellMovement.IA_SpellMovement"))
  (bind _returnvalue (Components|GetOwner))
  (bind _returnvalue_2 (Components|GetOwner))
  (bind _returnvalue_3 (Components|GetOwner))
  (:Started
    (bind _spell_count (Class|ISpellcaster|GetSpellCount(Message) _returnvalue_3 (Variables|Default|GetSpell%20Components)))
    (bind _can_cast (Class|ISpellcaster|CanCast(Message) _returnvalue_3 _spell_count))
    (if _can_cast
      (Class|ISpellcaster|CancelAllSpells(Message) (Components|GetOwner))
      (Class|ISpellcaster|SetActiveSpell(Message) (Components|GetOwner) (Variables|Default|GetSpell%20Components))
      (Class|ISpellcaster|CastActiveSpell(Message) (Components|GetOwner))
      (bind _player_controller (Class|IPlayerState|GetPlayerController(Message) _returnvalue))
      (Class|IStatusInvisible|OnInvisible(Message) _returnvalue "/Game/Spells/StatusEffects/Blueprints/BP_Status_Effect_Invisible.BP_Status_Effect_Invisible_C" 3.0 _player_controller _returnvalue)
      (Class|ISpellcaster|SpellcastingStopMontage(Message) _returnvalue_2 "/Game/FrogNomad/Animations/Standing_2H_Magic_Attack_01_Montage.Standing_2H_Magic_Attack_01_Montage")
      (Class|ISpellcaster|SpellcastingStopMontage(Message) _returnvalue_2 "/Game/FrogNomad/Animations/Standing_2H_Magic_Attack_04_Montage.Standing_2H_Magic_Attack_04_Montage")
      (if (Variables|Default|GetHas%20Now%20You%20See%20Me?)
        (CallFunction|ServerSpawnGreaterInvisibility))
      (CallFunction|PostSpellCast))))

(event EventInitializeSpellComponent
  (bind _player_state (Class|ICharacter|GetPlayerState(Message) (Components|GetOwner)))
  (bind _asbp_ps_mousen (Utilities|Casting|CastToBP_PS_Mousen _player_state))
  (Variables|Default|SetHas%20Now%20You%20See%20Me? (Variables|/Game/ThirdPerson/Blueprints/Gameplay/BP_PS_Mousen.BP_PS_Mousen_C|GetHasNowYouSeeMe? _asbp_ps_mousen)))