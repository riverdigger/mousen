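; Wizard spell component for Fire Ball, a charge-to-cast spell driven by the secondary spell input action.
; Starting the input checks that the owner can attack and cast, then cancels other spells, slows movement, charges the HUD reticle and plays the casting montage.
; Ongoing input updates charge progress; completion casts it as the active spell if still valid, while cancellation resets the charge.
; All owner and HUD communication goes through interface messages.
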(event Input|EnhancedActionEvents|EnhancedInputActionIA_Magic_SpellSecondary
  (params (ActionValue :type Boolean) (ElapsedSeconds :type Float%20%28double-precision%29) (TriggeredSeconds :type Float%20%28double-precision%29) (InputAction :type Input%20Action%20Object%20Reference :default "/Game/Inputs/Magic/IA_Magic_SpellSecondary.IA_Magic_SpellSecondary"))
  (bind _returnvalue (Components|GetOwner))
  (bind _returnvalue_2 (Components|GetOwner))
  (bind _returnvalue_3 (Components|GetOwner))
  (:Started
    (Variables|Default|SetIsCharging? false)
    (bind _can_attack (Class|ISpellcaster|CanAttack(Message) (Components|GetOwner)))
    (if _can_attack
      (bind _spell_count (Class|ISpellcaster|GetSpellCount(Message) _returnvalue (Variables|Default|GetSpell%20Components)))
      (bind _can_cast (Class|ISpellcaster|CanCast(Message) _returnvalue _spell_count))
      (bind _output_get (Variables|Default|SetIsCharging? _can_cast))
      (if _output_get
        (bind _player_controller (Class|ICharacter|GetPlayerController(Message) (Components|GetOwner)))
        (Class|IHUD|ChargeSpellReticle(Message) (HUD|GetHUD _player_controller) "NewEnumerator2")
        (Class|ISpellcaster|CancelAllSpells(Message) _returnvalue_3)
        (Class|ISpellcaster|SetChargeSlowModifier(Message) _returnvalue_3 true 0.3)
        (Class|ISpellcaster|SpellcastingPlayMontage(Message) (Components|GetOwner) "/Game/FrogNomad/Animations/Casting_Spell_Montage.Casting_Spell_Montage" 0.0))))
  (:Ongoing
    (bind _can_attack_2 (Class|ISpellcaster|CanAttack(Message) (Components|GetOwner)))
    (Class|ISpellcaster|UpdateSpellChargePercentage(Message) (Components|GetOwner) (select (and (Variables|Default|GetIsCharging?) _can_attack_2) (/ ElapsedSeconds 1.0) 0.0)))
  (:Canceled
    (bind _player_controller_2 (Class|ICharacter|GetPlayerController(Message) (Components|GetOwner)))
    (Class|IHUD|UnchargeSpellReticle(Message) (HUD|GetHUD _player_controller_2) "NewEnumerator2")
    (Class|ISpellcaster|UpdateSpellChargePercentage(Message) (Components|GetOwner) 0.0)
    (Class|ISpellcaster|SpellcastingStopMontage(Message) (Components|GetOwner) "/Game/FrogNomad/Animations/Casting_Spell_Montage.Casting_Spell_Montage")
    (Variables|Default|SetIsCharging? false)
    (bind _has_charge_slow (Class|ISpellcaster|GetChargeSlowModifier(Message) (Components|GetOwner)))
    (if _has_charge_slow
      (Class|ISpellcaster|SetChargeSlowModifier(Message) (Components|GetOwner) false 0.3)))
  (:Completed
    (bind _can_attack_3 (Class|ISpellcaster|CanAttack(Message) (Components|GetOwner)))
    (bind _player_controller_3 (Class|ICharacter|GetPlayerController(Message) (Components|GetOwner)))
    (Class|IHUD|UnchargeSpellReticle(Message) (HUD|GetHUD _player_controller_3) "NewEnumerator2")
    (Class|ISpellcaster|SpellcastingStopMontage(Message) (Components|GetOwner) "/Game/FrogNomad/Animations/Casting_Spell_Montage.Casting_Spell_Montage")
    (if _can_attack_3
      (if (Variables|Default|GetIsCharging?)
        (Class|ISpellcaster|UpdateSpellChargePercentage(Message) (Components|GetOwner) 0.0)
        (Class|ISpellcaster|SetChargeSlowModifier(Message) (Components|GetOwner) false 0.3)
        (Variables|Default|SetIsCharging? false)
        (Class|ISpellcaster|SetActiveSpell(Message) _returnvalue_2 (Variables|Default|GetSpell%20Components))
        (Class|ISpellcaster|CastActiveSpell(Message) _returnvalue_2)
        (Class|ISpellcaster|SpellcastingPlayMontage(Message) (Components|GetOwner) "/Game/FrogNomad/Animations/Casting_Spell_End_Montage.Casting_Spell_End_Montage" 0.0)
        (CallFunction|PostSpellCast)
        (else
          (Variables|Default|SetIsCharging? false :!label _label)
          (Class|ISpellcaster|SetChargeSlowModifier(Message) (Components|GetOwner) false 0.3)))
      (else
        (goto _label)))))