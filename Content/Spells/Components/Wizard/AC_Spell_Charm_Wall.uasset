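; AC_Spell_Charm_Wall is a wizard spell component that starts the Charm Wall spell from the second spell input action.
; On input start, it asks the owner for the spell count and whether casting is allowed.
; If so, it cancels all spells, sets the active spell and casts it through messages to the owner.
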(event Input|EnhancedActionEvents|EnhancedInputActionIA_Magic_SpellTwo
  (params (ActionValue :type Boolean) (ElapsedSeconds :type Float%20%28double-precision%29) (TriggeredSeconds :type Float%20%28double-precision%29) (InputAction :type Input%20Action%20Object%20Reference :default "/Game/Inputs/Magic/IA_Magic_SpellTwo.IA_Magic_SpellTwo"))
  (bind _returnvalue (Components|GetOwner))
  (bind _returnvalue_2 (Components|GetOwner))
  (:Started
    (bind _spell_count (Class|ISpellcaster|GetSpellCount(Message) _returnvalue (Variables|Default|GetSpell%20Components)))
    (bind _can_cast (Class|ISpellcaster|CanCast(Message) _returnvalue _spell_count))
    (if _can_cast
      (Class|ISpellcaster|CancelAllSpells(Message) _returnvalue_2)
      (Class|ISpellcaster|SetActiveSpell(Message) _returnvalue_2 (Variables|Default|GetSpell%20Components))
      (Class|ISpellcaster|CastActiveSpell(Message) (Components|GetOwner)))))