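; AC_Status_Effect_Frozen is a status effect actor component that slows its owning actor while it is active.
; On BeginPlay, after running the parent logic, the server sends the owner a slowdown message with the Percentage value.
; Before destruction, the server sends a matching speedup message with Percentage to undo the slow.
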(event EventBeginPlay
  (|CallParentFunction)
  (if (Networking|IsServer)
    (Class|IStatusEffectOwner|Slowdown(Message) (Components|GetOwner) (Variables|Default|GetPercentage))))

(event EventBeforeDestroy
  (if (Networking|IsServer)
    (Class|IStatusEffectOwner|Speedup(Message) (Components|GetOwner) (Variables|Default|GetPercentage))))