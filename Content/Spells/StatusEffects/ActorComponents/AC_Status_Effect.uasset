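; Status effect actor component that lives on its owner for a set Lifespan, then destroys itself.
; BeginPlay starts the lifespan timer, whose expiry clears it, calls a BeforeDestroy hook and removes the component.
; If a Niagara system is set, it messages the owner on start and end.
; Separate server events multicast spawning that system at the owner's root component ("pelvis" attach point) and destroying it.
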(event Custom|Multicast%20Attach%20System
  (bind _returnvalue (Niagara|SpawnSystemAttached (Variables|Default|GetNiagaraSystem) (Variables|/Script/Engine.Actor|GetRootComponent (Components|GetOwner)) "pelvis" "0, 0, 0" "0, 0, 0" "SnapToTarget" false)))

(event Custom|Multicast%20Remove%20System
  (Components|DestroyComponent (stale Custom|Multicast%20Attach%20System _returnvalue)))

(event EventBeginPlay
  (bind _returnvalue (Utilities|Time|SetTimerbyEvent (delegate EventBeginDestroy) (Variables|Default|GetLifespan)))
  (Variables|Default|SetLifespanTimer _returnvalue)
  (Utilities|IsValid (Variables|Default|GetNiagaraSystem)
    (:Is%20Valid
      (Class|IStatusEffectOwner|AttachNS(Message) (Components|GetOwner) self))))

(event EventBeginDestroy
  (Utilities|Time|ClearandInvalidateTimerbyHandle (Variables|Default|GetLifespanTimer))
  (CallFunction|BeforeDestroy)
  (Utilities|IsValid (Variables|Default|GetNiagaraSystem)
    (:Is%20Valid
      (Class|IStatusEffectOwner|RemoveNS(Message) (Components|GetOwner) self))
    (:Is%20Not%20Valid
      _))
  (Components|DestroyComponent))

(event EventServerAddNS
  (CallFunction|MulticastAttachSystem))

(event EventServerRemoveNS
  (CallFunction|MulticastRemoveSystem))