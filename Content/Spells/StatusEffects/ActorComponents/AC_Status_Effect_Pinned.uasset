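; Status effect component that pins its owning character in place for as long as it is attached.
; On BeginPlay the server resets launch parameters and multicasts the pin, which zeroes gravity, stops movement and simulates physics below the pelvis with physical animation orientation drive.
; Before destruction, the server resets pinned parameters and multicasts the release, restoring falling movement and gravity and turning off the simulation.
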(event Custom|Pin%20Owner
  (Class|IStatusLaunch|ResetLaunchParameters(Message) (Components|GetOwner) true)
  (CallFunction|MulticastPinOwner))

(event Custom|Multicast%20Pin%20Owner
  (bind _returnvalue (Components|GetOwner))
  (bind _character_movement (Class|IStatusEffectOwner|GetCharacterMovement(Message) _returnvalue))
  (Variables|/Script/Engine.CharacterMovementComponent|SetGravityScale _character_movement 0.0)
  (Components|Movement|StopMovementImmediately _character_movement)
  (bind _physical_animation (Class|IStatusEffectOwner|GetPhysicalComponent(Message) _returnvalue))
  (Utilities|IsValid _physical_animation
    (:Is%20Valid
      (Class|PhysicalAnimationComponent|ApplyPhysicalAnimationSettingsBelow _physical_animation "pelvis" (Utilities|Struct|MakePhysicalAnimationData true 1e+03 1e+02 1e+03 1e+02 1e+02 1e+02) true)
      (bind _skeletal_mesh (Class|IStatusEffectOwner|GetSkeletalMesh(Message) (Components|GetOwner)))
      (Utilities|IsValid _skeletal_mesh
        (:Is%20Valid
          (Class|SkeletalMeshComponent|SetAllBodiesBelowSimulatePhysics _skeletal_mesh (Class|SkinnedMeshComponent|GetBoneName _skeletal_mesh (Class|SkinnedMeshComponent|GetBoneIndex _skeletal_mesh "pelvis")) true false))))))

(event Custom|Multicast%20Un%20Pin%20Owner
  (bind _character_movement (Class|IStatusEffectOwner|GetCharacterMovement(Message) (Components|GetOwner)))
  (Pawn|Components|CharacterMovement|SetMovementMode _character_movement "MOVE_Falling" 0)
  (Variables|/Script/Engine.CharacterMovementComponent|SetGravityScale _character_movement 1.75)
  (bind _physical_animation (Class|IStatusEffectOwner|GetPhysicalComponent(Message) (Components|GetOwner)))
  (Utilities|IsValid _physical_animation
    (:Is%20Valid
      (Class|PhysicalAnimationComponent|ApplyPhysicalAnimationSettingsBelow _physical_animation "None" (Utilities|Struct|MakePhysicalAnimationData true 0.0) true)
      (bind _skeletal_mesh (Class|IStatusEffectOwner|GetSkeletalMesh(Message) (Components|GetOwner)))
      (Utilities|IsValid _skeletal_mesh
        (:Is%20Valid
          (Class|SkeletalMeshComponent|SetAllBodiesBelowSimulatePhysics _skeletal_mesh (Class|SkinnedMeshComponent|GetBoneName _skeletal_mesh (Class|SkinnedMeshComponent|GetBoneIndex _skeletal_mesh "pelvis")) false false))))))

(event EventBeginPlay
  (|CallParentFunction)
  (if (Networking|IsServer)
    (CallFunction|PinOwner)))

(event EventBeforeDestroy
  (if (Networking|IsServer)
    (CallFunction|MulticastUnPinOwner)
    (Class|IStatusPin|ResetPinnedParameters(Message) (Components|GetOwner))))