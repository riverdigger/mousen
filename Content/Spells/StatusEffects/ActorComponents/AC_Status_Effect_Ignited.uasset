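; Status effect actor component for Ignited, which deals periodic fire-typed damage to the actor it is attached to.
; On the server, BeginPlay applies one tick immediately, then starts a looping timer at the tick rate.
; Each tick sends a point damage message to the owner with the Ignited damage type, crediting the effect's instigator and creator.
; The server clears the timer before the component is destroyed.
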(event Custom|Apply%20Tick%20%20Damage
  (bind _returnvalue (Components|GetOwner))
  (Class|IDamage|ApplyServerPointDamage(Message) :self _returnvalue :DamagedActor _returnvalue :BaseDamage (Variables|Default|GetDamage) :InstigatedBy (Variables|Default|GetInstigated%20By) :DamageCauser (Variables|Default|GetCreated%20By) :DamageType "/Game/Items/DT_Ignited.DT_Ignited_C"))

(event EventBeforeDestroy
  (if (Networking|IsServer)
    (Utilities|Time|ClearandInvalidateTimerbyHandle (stale EventBeginPlay _returnvalue))))

(event EventBeginPlay
  (|CallParentFunction)
  (if (Networking|IsServer)
    (CallFunction|ApplyTickDamage)
    (bind _returnvalue (Utilities|Time|SetTimerbyEvent (delegate Custom|Apply%20Tick%20%20Damage) (Variables|Default|GetTick%20Rate) true))))