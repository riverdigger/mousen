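; Status effect component for spells that launches its owning character while active.
; On BeginPlay the server zeroes ground friction and walking braking, applies ProjectileVector as a velocity-change impulse, and multicasts a partial ragdoll using physical animation and simulated bodies below the pelvis.
; Before destruction, a multicast sets friction and braking to high values and, unless HitSomething is set, switches to Falling and turns the ragdoll off.
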(event Custom|Launch%20Owner
  (bind _character_movement (Class|IStatusEffectOwner|GetCharacterMovement(Message) (Components|GetOwner)))
  (Variables|/Script/Engine.CharacterMovementComponent|SetGroundFriction _character_movement 0.0)
  (Variables|/Script/Engine.CharacterMovementComponent|SetBrakingDecelerationWalking _character_movement 0.0)
  (CallFunction|MulticastLaunchOwner)
  (if (> (Math|Vector|VectorLength (Variables|Default|GetProjectileVector)) 0.0)
    (Physics|AddImpulse _character_movement (Variables|Default|GetProjectileVector) true)))

(event Custom|Multicast%20Reset%20Launced
  (bind _returnvalue (Components|GetOwner))
  (bind _character_movement (Class|IStatusEffectOwner|GetCharacterMovement(Message) _returnvalue))
  (Variables|/Script/Engine.CharacterMovementComponent|SetGroundFriction _character_movement 1e+03)
  (Variables|/Script/Engine.CharacterMovementComponent|SetBrakingDecelerationWalking _character_movement 1e+06)
  (if (not (Variables|Default|GetHitSomething?))
    (Pawn|Components|CharacterMovement|SetMovementMode _character_movement "MOVE_Falling" 0)
    (bind _physical_animation (Class|IStatusEffectOwner|GetPhysicalComponent(Message) _returnvalue))
    (Utilities|IsValid _physical_animation
      (:Is%20Valid
        (Class|PhysicalAnimationComponent|ApplyPhysicalAnimationSettingsBelow _physical_animation "None" (Utilities|Struct|MakePhysicalAnimationData true 0.0) true)
        (bind _skeletal_mesh (Class|IStatusEffectOwner|GetSkeletalMesh(Message) (Components|GetOwner)))
        (Utilities|IsValid _skeletal_mesh
          (:Is%20Valid
            (Class|SkeletalMeshComponent|SetAllBodiesBelowSimulatePhysics _skeletal_mesh (Class|SkinnedMeshComponent|GetBoneName _skeletal_mesh (Class|SkinnedMeshComponent|GetBoneIndex _skeletal_mesh "pelvis")) false false)))))))

(event Custom|Multicast%20Launch%20Owner
  (bind _returnvalue (Components|GetOwner))
  (bind _character_movement (Class|IStatusEffectOwner|GetCharacterMovement(Message) _returnvalue))
  (Variables|/Script/Engine.CharacterMovementComponent|SetBrakingDecelerationWalking _character_movement 0.0)
  (bind _physical_animation (Class|IStatusEffectOwner|GetPhysicalComponent(Message) _returnvalue))
  (Utilities|IsValid _physical_animation
    (:Is%20Valid
      (Class|PhysicalAnimationComponent|ApplyPhysicalAnimationSettingsBelow _physical_animation "pelvis" (Utilities|Struct|MakePhysicalAnimationData true 1e+03 1e+02 1e+03 1e+02 1e+02 1e+02) true)
      (bind _skeletal_mesh (Class|IStatusEffectOwner|GetSkeletalMesh(Message) (Components|GetOwner)))
      (Utilities|IsValid _skeletal_mesh
        (:Is%20Valid
          (Class|SkeletalMeshComponent|SetAllBodiesBelowSimulatePhysics _skeletal_mesh (Class|SkinnedMeshComponent|GetBoneName _skeletal_mesh (Class|SkinnedMeshComponent|GetBoneIndex _skeletal_mesh "pelvis")) true false))))))

(event EventBeginPlay
  (|CallParentFunction)
  (if (Networking|IsServer)
    (CallFunction|LaunchOwner)))

(event EventBeforeDestroy
  (if (Networking|IsServer)
    (CallFunction|MulticastResetLaunced)))