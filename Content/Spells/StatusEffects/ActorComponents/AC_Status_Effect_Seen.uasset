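; Status effect actor component that marks its owner as Seen by showing an overlay material on its skeletal mesh.
; On the server, BeginPlay multicasts applying the overlay material, and BeforeDestroy multicasts clearing it.
; Both multicasts fetch the owner's mesh through a GetSkeletalMeshMessage call and check it is valid before changing the overlay.
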(event Custom|Multicast%20Remove%20Overlay
  (bind _skeletal_mesh (Class|IStatusEffectOwner|GetSkeletalMesh(Message) (Components|GetOwner)))
  (Utilities|IsValid _skeletal_mesh
    (:Is%20Valid
      (Rendering|Material|SetOverlayMaterial _skeletal_mesh 0 :!class /Script/Engine.MeshComponent))))

(event Custom|Multicast%20Apply%20Overlay
  (bind _skeletal_mesh (Class|IStatusEffectOwner|GetSkeletalMesh(Message) (Components|GetOwner)))
  (Utilities|IsValid _skeletal_mesh
    (:Is%20Valid
      (Rendering|Material|SetOverlayMaterial _skeletal_mesh (Variables|Default|GetOverlayMaterial) :!class /Script/Engine.MeshComponent))))

(event EventBeginPlay
  (|CallParentFunction)
  (if (Networking|IsServer)
    (CallFunction|MulticastApplyOverlay)))

(event EventBeforeDestroy
  (if (Networking|IsServer)
    (CallFunction|MulticastRemoveOverlay)))