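; Stunned status effect actor component that slows its owner and applies a stunned screen effect while active.
; On the server, BeginPlay sends slowdown and post-process messages to the owner, and BeforeDestroy reverses the slowdown.
; The screen material is removed only when the owner's "Stun" effect count is one or less, so overlapping stuns keep the visual.
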(event EventBeforeDestroy
  (bind _returnvalue (Components|GetOwner))
  (if (Networking|IsServer)
    (Class|IStatusEffectOwner|Speedup(Message) _returnvalue (Variables|Default|GetPercentage))
    (bind _count (Class|IStatusEffectOwner|GetStatusEffectCount(Message) _returnvalue "Stun"))
    (if (<= _count 1)
      (Class|IStatusEffectOwner|RemovePostProcess(Message) _returnvalue "/Game/Spells/StatusEffects/FX/M_Screen_Stunned.M_Screen_Stunned"))))

(event EventBeginPlay
  (bind _returnvalue (Components|GetOwner))
  (|CallParentFunction)
  (if (Networking|IsServer)
    (Class|IStatusEffectOwner|Slowdown(Message) _returnvalue (Variables|Default|GetPercentage))
    (Class|IStatusEffectOwner|AddPostProcess(Message) _returnvalue "/Game/Spells/StatusEffects/FX/M_Screen_Stunned.M_Screen_Stunned")))