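; Status effect actor component that makes its owner invisible and changes its speed while active.
; On begin play it messages the owner to apply separate materials for owner and others, and the server applies a percentage speedup.
; Before destruction it resets the material only when the owner's Invisible effect count is not above one, so overlapping effects keep it.
; The server reverses each instance's speedup with a matching slowdown message.
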(event EventBeginPlay
  (bind _returnvalue (Components|GetOwner))
  (|CallParentFunction)
  (Class|IStatusEffectOwner|SetMaterial(Message) _returnvalue _returnvalue (Variables|Default|GetOwnerMaterial) (Variables|Default|GetOthersMaterial))
  (if (Networking|IsServer)
    (Class|IStatusEffectOwner|Speedup(Message) (Components|GetOwner) (Variables|Default|GetPercentage))))

(event EventBeforeDestroy
  (bind _returnvalue (Components|GetOwner))
  (bind _count (Class|IStatusEffectOwner|GetStatusEffectCount(Message) _returnvalue "Invisible"))
  (if (> _count 1)
    _
    (else
      (Class|IStatusEffectOwner|ResetMaterial(Message) _returnvalue 0 _returnvalue)))
  (if (Networking|IsServer)
    (Class|IStatusEffectOwner|Slowdown(Message) (Components|GetOwner) (Variables|Default|GetPercentage))))