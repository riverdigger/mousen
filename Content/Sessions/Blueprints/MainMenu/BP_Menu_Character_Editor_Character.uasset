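; Preview character for the main menu's character editor that wears the player's saved cosmetics and can be rotated, shown or hidden.
; On BeginPlay it looks up the saved melee hat and skin IDs in cosmetic DataTables.
; Hat changes spawn and attach an actor, skin changes swap the mesh material, and both play montages.
; A show-only SceneCapture2D re-captures after cosmetic updates and exports a per-class PNG to the project's image folder.
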(event Custom|PlayAnimationMontgage
  (params (MontageToPlay :type Anim%20Montage%20Object%20Reference))
  (Utilities|FlowControl|Delay 0.1)
  (Animation|Montage|PlayMontage (Variables|Default|GetSkeletalMesh) MontageToPlay))

(event Custom|Show%20In%20Menu
  (Rendering|SetVisibility (Variables|Default|GetSkeletalMesh) true true))

(event Custom|SaveImageToDisk
  (params (bSuccess :type Boolean))
  (Development|PrintString (Utilities|String|Append "Saved image: " (Utilities|String|ToString(Boolean) bSuccess) (Utilities|String|Append (Class|KismetSystemLibrary|GetProjectDirectory) "/Images/Classes/" (Utilities|String|Append (Utilities|String|EnumtoString (Variables|Default|GetClass)) "Class.png")))))

(event Custom|Start%20Rotating%20Left
  (Variables|Default|SetIsRotating? true)
  (Variables|Default|SetDirection 1.0))

(event Custom|AttachCosmeticHat
  (params (Hat :type S%20DT%20Cosmetics%20Hat%20Structure))
  (bind (_displayname _socket _texture _actor) (Utilities|Struct|BreakS_DT_Cosmetics_Hat Hat))
  (if (!= _actor (Utilities|GetClass (Variables|Default|GetAttachedHat)))
    (CallFunction|ResetCosmeticHat)
    (bind _returnvalue (Game|SpawnActorfromClass _actor (Transformation|GetActorTransform) "Undefined" "MultiplyWithRoot" 0 0))
    (Class|ICosmetic|Attach(Message) _returnvalue (Variables|Default|GetSkeletalMesh) _socket)
    (bind _output_get (Variables|Default|SetAttachedHat _returnvalue))
    (Rendering|SceneCapture|ShowOnlyActorComponents (Variables|Default|GetSceneCaptureComponent2D) _output_get true)
    (CallFunction|SaveImage)
    (CallFunction|PlayAnimationMontgage (Variables|Default|GetMontageHat))
    (else
      (CallFunction|SaveImage)
      (CallFunction|PlayAnimationMontgage (Variables|Default|GetMontageHat)))))

(event Custom|Update%20Skin%20Material
  (params (Skin :type S%20DT%20Cosmetics%20Skin%20Structure))
  (Rendering|Material|SetMaterial (Variables|Default|GetSkeletalMesh) 0 (.Material (Utilities|Struct|BreakS_DT_Cosmetics_Skin Skin)))
  (CallFunction|SaveImage)
  (CallFunction|PlayAnimationMontgage (Variables|Default|GetMontageSkin)))

(event Custom|ResetCosmeticHat
  (Actor|DestroyActor (Variables|Default|GetAttachedHat))
  (Variables|Default|SetAttachedHat 0)
  (CallFunction|SaveImage)
  (CallFunction|PlayAnimationMontgage))

(event Custom|Hide%20In%20Menu
  (Rendering|SetVisibility (Variables|Default|GetSkeletalMesh) false true))

(event Custom|Start%20Rotating%20Right
  (Variables|Default|SetIsRotating? true)
  (Variables|Default|SetDirection -1.0))

(event Custom|Stop%20Rotating
  (Variables|Default|SetIsRotating? false))

(event Custom|AttachAllCosmetics
  (Utilities|FlowControl|Sequence
    (:then_0
      (bind _settings (Class|IGameInstance|GetSettings(Message) (Game|GetGameInstance)))
      (bind _returnvalue (Utilities|GetDataTableRow "/Game/Objects/Cosmetics/Hats/DT_Cosmetics_Hat.DT_Cosmetics_Hat" (Variables|/Game/ThirdPerson/Blueprints/Gameplay/BP_Settings_Save.BP_Settings_Save_C|GetMeleeHatCosmeticID _settings))
        (:then
          (CallFunction|AttachCosmeticHat _returnvalue))))
    (:then_1
      (bind _settings_2 (Class|IGameInstance|GetSettings(Message) (Game|GetGameInstance)))
      (bind _returnvalue_2 (Utilities|GetDataTableRow "/Game/Objects/Cosmetics/Skins/DT_Cosmetics_Skins.DT_Cosmetics_Skins" (Variables|/Game/ThirdPerson/Blueprints/Gameplay/BP_Settings_Save.BP_Settings_Save_C|GetMeleeSkinCosmeticID _settings_2))
        (:then
          (CallFunction|UpdateSkinMaterial _returnvalue_2))))
    (:then_2
      (CallFunction|SaveImage))))

(event Custom|SaveImage
  (Rendering|SceneCapture|CaptureScene (Variables|Default|GetSceneCaptureComponent2D) :!class /Script/Engine.SceneCaptureComponent2D)
  (Class|ImageWriteBlueprintLibrary|ExporttoDisk (Variables|/Script/Engine.SceneCaptureComponent2D|GetTextureTarget (Variables|Default|GetSceneCaptureComponent2D)) (Utilities|String|Append (Class|KismetSystemLibrary|GetProjectDirectory) "/Images/Classes/" (Utilities|String|Append (Utilities|String|EnumtoString (Variables|Default|GetClass)) "Class.png")) (Utilities|Struct|MakeImageWriteOptions "PNG" (delegate Custom|SaveImageToDisk))))

(event EventTick
  (params (DeltaSeconds :type Float%20%28single-precision%29))
  (if (Variables|Default|GetIsRotating?)
    (Transformation|AddActorLocalRotation (Math|Rotator|MakeRotator 0.0 0.0 (* (* (/ 3.6e+02 (Variables|Default|GetTimeToRotateFully)) DeltaSeconds) (Variables|Default|GetDirection))) false false)))

(event EventBeginPlay
  (CallFunction|AttachAllCosmetics))

(fn ConstructionScript
  (Rendering|SceneCapture|ShowOnlyComponent (Variables|Default|GetSceneCaptureComponent2D) (Variables|Default|GetSkeletalMesh)))