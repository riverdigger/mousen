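; Wizard character for the main menu character editor, previewing the saved hat and skin cosmetics.
; Looks up the game instance's cosmetic IDs in DataTables, then spawns and attaches the hat actor and swaps the skeletal mesh material.
; A new hat replaces the old one and joins the SceneCapture2D show-only list.
; Cosmetic changes call SaveImage and play a hat or skin montage; the character calls HideInMenu on BeginPlay.
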(event EventBeginPlay
  (|CallParentFunction)
  (CallFunction|HideinMenu))

(event Collision|EventActorBeginOverlap
  (params (OtherActor :type Actor%20Object%20Reference)))

(event EventTick
  (params (DeltaSeconds :type Float%20%28single-precision%29))
  (|CallParentFunction DeltaSeconds) ; This node is disabled and will not be called.\nDrag off pins to build functionality.
)

(event EventUpdateSkinMaterial
  (params (Skin :type S%20DT%20Cosmetics%20Skin%20Structure))
  (Rendering|Material|SetMaterial (Variables|Default|GetSkeletalMesh) 1 (.Material (Utilities|Struct|BreakS_DT_Cosmetics_Skin Skin)))
  (CallFunction|SaveImage)
  (CallFunction|PlayAnimationMontgage (Variables|Default|GetMontageSkin)))

(event EventAttachAllCosmetics
  (Utilities|FlowControl|Sequence
    (:then_0
      (bind _settings (Class|IGameInstance|GetSettings(Message) (Game|GetGameInstance)))
      (bind _returnvalue (Utilities|GetDataTableRow "/Game/Objects/Cosmetics/Hats/DT_Cosmetics_Hat.DT_Cosmetics_Hat" (Variables|/Game/ThirdPerson/Blueprints/Gameplay/BP_Settings_Save.BP_Settings_Save_C|GetWizardHatCosmeticID _settings))
        (:then
          (CallFunction|AttachCosmeticHat _returnvalue))))
    (:then_1
      (bind _settings_2 (Class|IGameInstance|GetSettings(Message) (Game|GetGameInstance)))
      (bind _returnvalue_2 (Utilities|GetDataTableRow "/Game/Objects/Cosmetics/Skins/DT_Cosmetics_Skins.DT_Cosmetics_Skins" (Variables|/Game/ThirdPerson/Blueprints/Gameplay/BP_Settings_Save.BP_Settings_Save_C|GetWizardSkinCosmeticID _settings_2))
        (:then
          (CallFunction|UpdateSkinMaterial _returnvalue_2))))
    (:then_2
      (CallFunction|SaveImage))))

(event EventAttachCosmeticHat
  (params (Hat :type S%20DT%20Cosmetics%20Hat%20Structure))
  (bind (_displayname _socket _texture _actor) (Utilities|Struct|BreakS_DT_Cosmetics_Hat Hat))
  (if (!= _actor (Utilities|GetClass (Variables|Default|GetAttachedHat)))
    (CallFunction|ResetCosmeticHat)
    (bind _returnvalue (Game|SpawnActorfromClass _actor (Transformation|GetActorTransform) "Undefined" "MultiplyWithRoot" 0 0))
    (Class|ICosmetic|Attach(Message) _returnvalue (Variables|Default|GetSkeletalMesh) _socket)
    (bind _output_get (Variables|Default|SetAttachedHat _returnvalue))
    (Rendering|SceneCapture|ShowOnlyActorComponents (Variables|Default|GetSceneCaptureComponent2D) _output_get true)
    (CallFunction|SaveImage)
    (CallFunction|PlayAnimationMontgage (Variables|Default|GetMontageHat))
    (else
      (CallFunction|SaveImage)
      (CallFunction|PlayAnimationMontgage (Variables|Default|GetMontageHat)))))

(event EventResetCosmeticHat
  (Actor|DestroyActor (Variables|Default|GetAttachedHat))
  (Variables|Default|SetAttachedHat 0)
  (CallFunction|SaveImage)
  (CallFunction|PlayAnimationMontgage (Variables|Default|GetMontageHat)))

(fn ConstructionScript
  (|CallParentFunction))