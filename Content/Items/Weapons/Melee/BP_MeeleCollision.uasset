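; Melee hit volume that deals fixed two-handed weapon damage to actors its sphere overlaps.
; Overlaps count only for I_Damage implementers other than the Instigator; I_Character targets also receive a blood splat particle.
; Hit direction and a synthetic hit result come from the sphere-to-target vector and target location.
; ServerApplyDamage forwards point damage through player controller 0, cached at BeginPlay as BP_PC_Mousen and passed as instigating controller.
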(event OnComponentBeginOverlap(Sphere)
  (params (OverlappedComponent :type Primitive%20Component%20Object%20Reference) (OtherActor :type Actor%20Object%20Reference) (OtherComp :type Primitive%20Component%20Object%20Reference) (OtherBodyIndex :type Integer) (bFromSweep :type Boolean) (SweepResult :type Hit%20Result%20Structure%20%28by%20ref%29))
  (bind _returnvalue (Transformation|GetActorLocation OtherActor))
  (bind _sphere (Variables|Default|GetSphere))
  (bind _returnvalue_2 (Transformation|GetWorldLocation _sphere))
  (bind _returnvalue_3 (- _returnvalue _returnvalue_2))
  (bind _returnvalue_4 (Math|Vector|Normalize _returnvalue_3))
  (if (Utilities|DoesObjectImplementInterface OtherActor "/Game/ThirdPerson/Blueprints/Gameplay/I_Damage.I_Damage_C")
    (if (!= OtherActor (Variables|Actor|GetInstigator))
      (if (Utilities|DoesObjectImplementInterface OtherActor "/Game/ThirdPerson/Blueprints/I_Character.I_Character_C")
        (Class|ICharacter|PassWeaponParticleSystem(Message) OtherActor "/Game/ExternalFreeContent/Realistic_Starter_VFX_Pack_Vol2/Particles/Blood/P_Blood_Splat_Cone.P_Blood_Splat_Cone"))
      (CallFunction|ServerApplyDamage OtherActor 5e+01 _returnvalue_4 (Collision|MakeHitResult false false 0.0 0.0 "0, 0, 0" _returnvalue "0,0,1" _returnvalue_4 0 OtherActor) (Variables|Default|GetAs%20BP%20PC%20Mousen) (Variables|Actor|GetInstigator) "/Game/Items/Weapons/DT_2HWeapon.DT_2HWeapon_C"))))

(event Custom|Server%20Apply%20Damage
  (params (DamagedActor :type Actor%20Object%20Reference) (Damage :type Float%20%28double-precision%29) (Hit%20Direction :type Vector) (Hit%20Info :type Hit%20Result%20Structure) (Instigated%20By :type Controller%20Object%20Reference) (DamageCauser :type Actor%20Object%20Reference) (Damage%20Type%20Class :type Damage%20Type%20Class%20Reference))
  (Default|ApplyPointDamage (Variables|Default|GetAs%20BP%20PC%20Mousen) DamagedActor Damage Hit%20Direction Hit%20Info Instigated%20By DamageCauser Damage%20Type%20Class))

(event EventBeginPlay
  (bind _asbp_pc_mousen (Utilities|Casting|CastToBP_PC_Mousen (Game|GetPlayerController 0)))
  (Variables|Default|SetAs%20BP%20PC%20Mousen _asbp_pc_mousen))

(fn ConstructionScript)