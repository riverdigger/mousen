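; Overcharged arrow projectile that damages and knocks back what it hits, with a brief trail after spawn.
; On box overlap with anything but its instigator, it stops, attaches to the target and pushes characters in Flying mode using scaled arrow velocity.
; I_Damage targets receive a Launched status and point damage routed through the Mousen player controller.
; Server-named events handle velocity, damage and multicast hit particles before a delayed destroy.
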(event OnComponentBeginOverlap(Box)
  (params (OverlappedComponent :type Primitive%20Component%20Object%20Reference) (OtherActor :type Actor%20Object%20Reference) (OtherComp :type Primitive%20Component%20Object%20Reference) (OtherBodyIndex :type Integer) (bFromSweep :type Boolean) (SweepResult :type Hit%20Result%20Structure%20%28by%20ref%29))
  (bind _lastknownvelocity (Variables|Default|GetLastKnownVelocity))
  (bind _projectilemovement (Variables|Default|GetProjectileMovement))
  (bind _lastknownvelocity_2 (Variables|Default|GetLastKnownVelocity))
  (bind _returnvalue (* _lastknownvelocity_2 0.3))
  (bind _returnvalue_2 (* _lastknownvelocity 0.3))
  ;[1 1 1] When Arrow hits, deal damage and attach the arrow to the target
  (if (!= OtherActor (Variables|Actor|GetInstigator))
    (CallFunction|ServerUpdateLastKnownVelocity (Variables|/Script/Engine.MovementComponent|GetVelocity (Variables|Default|GetProjectileMovement)))
    (Variables|Default|SetLastKnownVector (Transformation|GetActorForwardVector))
    (Components|Movement|StopMovementImmediately _projectilemovement)
    (Variables|/Script/Engine.ProjectileMovementComponent|SetProjectileGravityScale _projectilemovement 0.0)
    (Collision|SetCollisionEnabled (Variables|Default|GetBox) "NoCollision")
    (bind _ascharacter (Utilities|Casting|CastToCharacter OtherActor)
      (:then
        (Transformation|AttachComponentToComponent (Variables|/Script/Engine.Character|GetMesh _ascharacter) "pelvis" "SnapToTarget" "KeepWorld" "KeepWorld" true)
        (Pawn|Components|CharacterMovement|SetMovementMode (Variables|/Script/Engine.Character|GetCharacterMovement _ascharacter) "MOVE_Flying" 0)
        (if (AI|Components|NavMovement|IsFalling (Variables|/Script/Engine.Character|GetCharacterMovement _ascharacter))
          (Physics|AddImpulse (Variables|/Script/Engine.Character|GetCharacterMovement _ascharacter) (Math|Vector|MakeVector (.x _returnvalue_2) (.y _returnvalue_2) (+ (.z _returnvalue_2) 25.0)) true)
          (else
            (Physics|AddImpulse (Variables|/Script/Engine.Character|GetCharacterMovement _ascharacter) (Math|Vector|MakeVector (.x _returnvalue) (.y _returnvalue) 1.5e+02) true))))
      (:CastFailed
        (Transformation|AttachActorToActor OtherActor "None" "KeepWorld" "KeepWorld" "KeepWorld" true)))
    (if (Utilities|DoesObjectImplementInterface OtherActor "/Game/ThirdPerson/Blueprints/Gameplay/I_Damage.I_Damage_C")
      (Class|IStatusLaunch|OnLaunch(Message) OtherActor "/Game/Spells/StatusEffects/BP_Status_Effect_Launched.BP_Status_Effect_Launched_C" (Variables|Default|GetLaunchLifetime) (Variables|Default|GetLastKnownVector))
      (CallFunction|ServerApplyDamage :DamagedActor OtherActor :Damage (CallFunction|GetCurrentDamage) :Hit%20Direction (* (Math|Vector|Normalize (Math|Vector|GetForwardVector (Variables|Default|GetArrow))) "-1.000000,-1.000000,-1.000000") :Instigated%20By (Game|GetPlayerController 0) :DamageCauser (Variables|Actor|GetInstigator) :Damage%20Type%20Class "/Game/Items/Weapons/Ranged/DT_Ranged.DT_Ranged_C"))
    (CallFunction|ServerSpawnCollisionEmitter)
    (Utilities|FlowControl|Delay (Variables|Default|GetLifetime))
    (Actor|DestroyActor)))

(event Custom|Server%20Apply%20Damage
  (params (DamagedActor :type Actor%20Object%20Reference) (Damage :type Float%20%28double-precision%29) (Hit%20Direction :type Vector) (Hit%20Info :type Hit%20Result%20Structure) (Instigated%20By :type Controller%20Object%20Reference) (DamageCauser :type Actor%20Object%20Reference) (Damage%20Type%20Class :type Damage%20Type%20Class%20Reference))
  (Default|ApplyPointDamage (Variables|Default|GetAs%20BP%20PC%20Mousen) DamagedActor Damage Hit%20Direction Hit%20Info Instigated%20By DamageCauser Damage%20Type%20Class))

(event Custom|Multicast%20Spawn%20Collision%20Emitter
  (Effects|SpawnEmitteratLocation "/Game/ExternalFreeContent/FXVarietyPack/Particles/P_ky_hit2.P_ky_hit2" (Transformation|GetWorldLocation (Variables|Default|GetBox)) "0, 0, 0" "0.200000,0.200000,0.200000"))

(event Custom|Server%20Spawn%20Collision%20Emitter
  (CallFunction|MulticastSpawnCollisionEmitter))

(event Custom|Server%20Update%20Last%20Known%20Velocity
  (params (LastKnownVelocity :type Vector))
  ;[1 1 1] When Arrow hits, deal damage and attach the arrow to the target
  (Variables|Default|SetLastKnownVelocity LastKnownVelocity))

(event EventBeginPlay
  (bind _trail (Variables|Default|GetTrail))
  ;[1 1 1] Spawn Arrow and Set Owner and Effects
  (bind _asbp_pc_mousen (Utilities|Casting|CastToBP_PC_Mousen (Game|GetPlayerController 0)))
  (Variables|Default|SetAs%20BP%20PC%20Mousen _asbp_pc_mousen)
  (Effects|Particles|Trails|BeginTrails _trail "Trail1" "Trail2" "ETrailWidthMode_FromFirst" 5.0)
  (Utilities|FlowControl|Delay 0.2)
  (Effects|Particles|Trails|EndTrails _trail))

(fn ConstructionScript)

(fn GetCurrentDamage
  (return (Variables|Default|GetBaseDamage)))