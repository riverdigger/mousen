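; BP_Arrow is the projectile fired by BP_Bow, showing a trail from spawn.
; On capsule overlap, ignoring its owner and that owner's owner, it stops, attaches to the hit actor, disables collision and spawns a hit effect.
; Damage uses the bow's WeaponOutputDamage, applied through player 0's BP_ThirdPersonCharacter as causer, regardless of who fired.
; The EndTrails call is unconnected, so the trail is never explicitly ended.
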(event OnComponentBeginOverlap(Capsule)
  (params (OverlappedComponent :type Primitive%20Component%20Object%20Reference) (OtherActor :type Actor%20Object%20Reference) (OtherComp :type Primitive%20Component%20Object%20Reference) (OtherBodyIndex :type Integer) (bFromSweep :type Boolean) (SweepResult :type Hit%20Result%20Structure%20%28by%20ref%29))
  (bind _returnvalue (Game|GetPlayerCharacter 0))
  (bind _self self)
  (bind _projectilemovement (Variables|Default|GetProjectileMovement))
  (bind _returnvalue_2 (Components|GetOwner _self))
  (bind _asbp_third_person_character (Utilities|Casting|CastToBP_ThirdPersonCharacter _returnvalue))
  (if (and (and (!= OtherActor _self) (!= _returnvalue_2 OtherActor)) (!= OtherActor (Components|GetOwner _returnvalue_2)))
    (Components|Movement|StopMovementImmediately _projectilemovement)
    (Variables|/Script/Engine.ProjectileMovementComponent|SetProjectileGravityScale _projectilemovement 0.0)
    (Transformation|AttachActorToActor OtherActor "None" "KeepWorld" "KeepWorld" "KeepWorld" true)
    (Default|ApplyServerPointDamage :self _asbp_third_person_character :Damaged%20Actor OtherActor :Base%20Damage (Variables|/Game/Items/Weapons/Ranged/BP_Bow.BP_Bow_C|GetWeaponOutputDamage (.AsBP%20Bow (Utilities|Casting|CastToBP_Bow (Components|GetOwner)))) :Instigated%20By (Game|GetPlayerController 0) :Damage%20Causer _asbp_third_person_character :Damage%20Type "/Script/Engine.DamageType")
    (Collision|SetCollisionEnabled (Variables|Default|GetCapsule) "NoCollision")
    (Effects|SpawnEmitteratLocation "/Game/ExternalFreeContent/FXVarietyPack/Particles/P_ky_hit2.P_ky_hit2" (Transformation|GetWorldLocation (Variables|Default|GetCapsule)) "0, 0, 0" "0.200000,0.200000,0.200000")))

(event EventBeginPlay
  (Effects|Particles|Trails|BeginTrails (Variables|Default|GetTrail) "Trail1" "Trail2" "ETrailWidthMode_FromFirst" 1.0))

(event Collision|EventActorBeginOverlap
  (params (OtherActor :type Actor%20Object%20Reference)))

(event EventTick
  (params (DeltaSeconds :type Float%20%28single-precision%29)))

(fn ConstructionScript)