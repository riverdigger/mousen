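; BP_Spell_Tornado is a timed area-damage spell actor that destroys itself after its Lifespan.
; Capsule overlap starts tick damage on I_Damage actors via interface messages, and end overlap stops it.
; Unless DamagesCaster is set, it skips starting damage on the caster, found as the owner's owner.
; The instigator is always player controller 0.
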(event OnComponentEndOverlap(Capsule)
  (params (OverlappedComponent :type Primitive%20Component%20Object%20Reference) (OtherActor :type Actor%20Object%20Reference) (OtherComp :type Primitive%20Component%20Object%20Reference) (OtherBodyIndex :type Integer))
  (if (Utilities|DoesObjectImplementInterface OtherActor "/Game/ThirdPerson/Blueprints/Gameplay/I_Damage.I_Damage_C")
    (Class|IDamage|StopTickDamage(Message) OtherActor)))

(event OnComponentBeginOverlap(Capsule)
  (params (OverlappedComponent :type Primitive%20Component%20Object%20Reference) (OtherActor :type Actor%20Object%20Reference) (OtherComp :type Primitive%20Component%20Object%20Reference) (OtherBodyIndex :type Integer) (bFromSweep :type Boolean) (SweepResult :type Hit%20Result%20Structure%20%28by%20ref%29))
  (if (Utilities|DoesObjectImplementInterface OtherActor "/Game/ThirdPerson/Blueprints/Gameplay/I_Damage.I_Damage_C")
    (if (Variables|Default|GetDamagesCaster?)
      (Class|IDamage|ApplyTickDamage(Message) OtherActor (Variables|Default|GetDamage) (Variables|Default|GetTickRate) (Game|GetPlayerController 0) self :!label _label)
      (elif (not (== (Components|GetOwner (Components|GetOwner self)) OtherActor))
        (goto _label)))))

(event EventBeginPlay
  (Utilities|FlowControl|Delay (Variables|Default|GetLifespan))
  (Actor|DestroyActor))

(event Collision|EventActorBeginOverlap
  (params (OtherActor :type Actor%20Object%20Reference)))

(fn ConstructionScript)