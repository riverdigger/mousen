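; Team flag spawner for a capture-the-flag mode that spawns a BP_Flag above its spawn point when play begins on the server.
; Separate respawn and reclaim timers, each startable, pausable and cancellable, end in identical events that clear both timers and replace the flag.
; Tick prints both remaining times as debug output.
; ScorePoint is an empty stub, with its capture effect and reset logic left disconnected.
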(event Custom|Countdown%20Reclaim%20Flag
  (Utilities|Time|ClearandInvalidateTimerbyHandle (stale _returnvalue))
  (bind _returnvalue (Utilities|Time|SetTimerbyEvent (delegate Custom|Reclaim%20Flag) (Variables|Default|GetReclaimTime))))

(event Custom|Cancel%20Reclaim%20Flag
  (Utilities|Time|ClearandInvalidateTimerbyHandle (stale Custom|Countdown%20Reclaim%20Flag _returnvalue)))

(event Custom|Reclaim%20Flag
  (bind _spawnlocation (Variables|Default|GetSpawnLocation))
  (bind _returnvalue (Transformation|GetWorldLocation _spawnlocation))
  (Utilities|Time|ClearandInvalidateTimerbyHandle (stale Custom|Countdown%20Respawn%20Flag _returnvalue))
  (Utilities|Time|ClearandInvalidateTimerbyHandle (stale Custom|Countdown%20Reclaim%20Flag _returnvalue))
  (Utilities|IsValid (Variables|Default|GetFlag)
    (:Is%20Valid
      (Actor|DestroyActor (Variables|Default|GetFlag)))
    (:Is%20Not%20Valid
      _))
  (bind _returnvalue_2 (Game|SpawnActorfromClass "/Game/Items/Flags/BP_Flag.BP_Flag_C" (Math|Transform|MakeTransform (Math|Vector|MakeVector (.x _returnvalue) (.y _returnvalue) (+ (.z _returnvalue) 75.0)) "0, 0, 0" "1.000000,1.000000,1.000000") "Undefined" 0 self (Variables|Default|GetTeam) 0))
  (Variables|Default|SetHasFlag? true)
  (bind _output_get (Variables|Default|SetFlag _returnvalue_2))
  (Variables|/Game/Items/Flags/BP_Flag.BP_Flag_C|SetIsAway? _output_get false))

(event Custom|Pause%20Reclaim%20Timer
  (Utilities|Time|PauseTimerbyHandle (stale Custom|Countdown%20Reclaim%20Flag _returnvalue)))

(event Custom|UnPause%20Reclaim%20Timer
  (Utilities|Time|UnpauseTimerbyHandle (stale Custom|Countdown%20Reclaim%20Flag _returnvalue)))

(event Custom|UnPause%20Respawn%20Timer
  (Utilities|Time|UnpauseTimerbyHandle (stale Custom|Countdown%20Respawn%20Flag _returnvalue)))

(event Custom|Pause%20Respawn%20Timer
  (Utilities|Time|PauseTimerbyHandle (stale Custom|Countdown%20Respawn%20Flag _returnvalue)))

(event Custom|Countdown%20Respawn%20Flag
  (Utilities|Time|ClearandInvalidateTimerbyHandle (stale _returnvalue))
  (bind _returnvalue (Utilities|Time|SetTimerbyEvent (delegate Custom|Respawn%20Flag) (Variables|Default|GetRespawnTime))))

(event Custom|Cancel%20Respawn%20Flag
  (Utilities|Time|ClearandInvalidateTimerbyHandle (stale Custom|Countdown%20Respawn%20Flag _returnvalue)))

(event Custom|Respawn%20Flag
  (bind _spawnlocation (Variables|Default|GetSpawnLocation))
  (bind _returnvalue (Transformation|GetWorldLocation _spawnlocation))
  (Utilities|Time|ClearandInvalidateTimerbyHandle (stale Custom|Countdown%20Respawn%20Flag _returnvalue))
  (Utilities|Time|ClearandInvalidateTimerbyHandle (stale Custom|Countdown%20Reclaim%20Flag _returnvalue))
  (Utilities|IsValid (Variables|Default|GetFlag)
    (:Is%20Valid
      (Actor|DestroyActor (Variables|Default|GetFlag)))
    (:Is%20Not%20Valid
      _))
  (bind _returnvalue_2 (Game|SpawnActorfromClass "/Game/Items/Flags/BP_Flag.BP_Flag_C" (Math|Transform|MakeTransform (Math|Vector|MakeVector (.x _returnvalue) (.y _returnvalue) (+ (.z _returnvalue) 75.0)) "0, 0, 0" "1.000000,1.000000,1.000000") "Undefined" 0 self (Variables|Default|GetTeam) 0))
  (Variables|Default|SetHasFlag? true)
  (bind _output_get (Variables|Default|SetFlag _returnvalue_2))
  (Variables|/Game/Items/Flags/BP_Flag.BP_Flag_C|SetIsAway? _output_get false))

(event EventBeginPlay
  (if (Networking|IsServer)
    (CallFunction|RespawnFlag)))

(event EventTick
  (params (DeltaSeconds :type Float%20%28single-precision%29))
  (Development|PrintString (Utilities|String|Append "Respawn: " (Utilities|String|ToString(Float) (Utilities|Time|GetTimerRemainingTimebyHandle (stale Custom|Countdown%20Respawn%20Flag _returnvalue)))))
  (Development|PrintString (Utilities|String|Append "Reclaim: " (Utilities|String|ToString(Float) (Utilities|Time|GetTimerRemainingTimebyHandle (stale Custom|Countdown%20Reclaim%20Flag _returnvalue))))))

(fn ConstructionScript
  (Variables|Default|SetRespawnTimeRemaining (Variables|Default|GetRespawnTime)))

(fn ResetCountdown
  (Variables|Default|SetRespawnTimeRemaining (Variables|Default|GetRespawnTime)))

(fn ScorePoint
  (params (Flag :type %20Object%20Reference) (Player :type BP%20Third%20Person%20Character%20Object%20Reference)))

(fn GetRemainingRespawnTime
  (return (Class|KismetSystemLibrary|GetTimerRemainingTime 0 "Respawn Flag")))

(fn GetRemainingReclaimTime
  (return (Class|KismetSystemLibrary|GetTimerRemainingTime 0 "Reclaim Flag")))