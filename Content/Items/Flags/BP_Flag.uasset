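; BP_Flag is a carryable flag that a player picks up or drops through its Interact event.
; Pickup routes a server event to a multicast that snaps the flag to the player mesh's item_spine socket and sets IsHeld.
; Dropping detaches it through the same pattern.
; Physics toggling and the forward impulse on drop run directly in Interact, outside the multicasts.
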(event Custom|Multicast%20Pick%20Up%20Flag
  (params (ActorToAttach :type Actor%20Object%20Reference) (Parent :type Character%20Object%20Reference))
  (Transformation|AttachComponentToComponent (Variables|/Script/Engine.Character|GetMesh Parent) "item_spine" "SnapToTarget" "SnapToTarget" "KeepRelative" true)
  (Variables|Default|SetIsHeld? true))

(event Custom|Server%20Pick%20Up%20Flag
  (params (Parent :type Character%20Object%20Reference))
  (CallFunction|MulticastPickUpFlag 0 Parent))

(event Custom|Server%20Drop%20Flag
  (CallFunction|MulticastDropFlag))

(event Custom|Multicast%20Drop%20Flag
  (Transformation|DetachFromActor "KeepWorld" "KeepWorld" "KeepWorld")
  (Variables|Default|SetIsHeld? false))

(event EventInteract
  (params (Player :type Character%20Object%20Reference))
  (bind _flagmesh (Variables|Default|GetFlagMesh))
  (if (Variables|Default|GetIsHeld?)
    (CallFunction|ServerDropFlag)
    (Physics|SetSimulatePhysics (Variables|Default|GetFlagMesh) true)
    (Physics|SetPhysicsLinearVelocity _flagmesh "0, 0, 0" false "None")
    (Physics|AddImpulse _flagmesh (* (Transformation|GetActorForwardVector (Components|GetOwner)) 2e+02) "None" true)
    (else
      (Physics|SetSimulatePhysics (Variables|Default|GetFlagMesh) false)
      (CallFunction|ServerPickUpFlag Player))))

(fn ConstructionScript)