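; Martyrdom weapon actor, a timed explosive that launches forward on spawn and detonates after TimeToExplode.
; The explosion multicasts particles and hides the mesh, then damages I_Damage actors overlapping the Sphere, skipping those tagged with the instigator's team.
; Damage is routed through the instigator's BP_PC_Mousen controller as point damage, and the actor destroys itself one second after exploding.
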(event Custom|Server%20Apply%20Damage
  (params (DamagedActor :type Actor%20Object%20Reference) (Damage :type Float%20%28double-precision%29) (Hit%20Direction :type Vector) (Hit%20Info :type Hit%20Result%20Structure) (Instigated%20By :type Controller%20Object%20Reference) (DamageCauser :type Actor%20Object%20Reference) (Damage%20Type%20Class :type Damage%20Type%20Class%20Reference))
  (Default|ApplyPointDamage (.AsBP%20PC%20Mousen (Utilities|Casting|CastToBP_PC_Mousen (Game|GetInstigatorController))) DamagedActor Damage Hit%20Direction Hit%20Info Instigated%20By DamageCauser Damage%20Type%20Class))

(event Custom|Server%20Explode
  (CallFunction|MulticastActivateExplosion)
  (for _array_element (Collision|GetOverlappingActors (Variables|Default|GetSphere) "/Script/Engine.Actor" :!class /Script/Engine.PrimitiveComponent)
    (if (Utilities|DoesObjectImplementInterface _array_element "/Game/ThirdPerson/Blueprints/Gameplay/I_Damage.I_Damage_C")
      (if (not (Actor|ActorHasTag _array_element (Utilities|Name|EnumtoName (Variables|/Game/ThirdPerson/Blueprints/Gameplay/BP_PS_Mousen.BP_PS_Mousen_C|GetPlayerTeam (.AsBP%20PS%20Mousen (Utilities|Casting|CastToBP_PS_Mousen (Variables|/Script/Engine.Pawn|GetPlayerState (Variables|Actor|GetInstigator))))))))
        (CallFunction|ServerApplyDamage :DamagedActor _array_element :Damage (Variables|Default|GetDamage) :Instigated%20By (.AsBP%20PC%20Mousen (Utilities|Casting|CastToBP_PC_Mousen (Game|GetInstigatorController))) :DamageCauser self))))
  (Utilities|FlowControl|Delay 1.0)
  (Actor|DestroyActor))

(event Custom|Multicast%20Activate%20Explosion
  (Components|Activation|Activate (Variables|Default|GetExplosionParticles) false)
  (Rendering|SetVisibility (Variables|Default|GetStaticMesh) false false))

(event EventBeginPlay
  (Physics|AddImpulse (Variables|Default|GetStaticMesh) (* (Transformation|GetActorForwardVector) 1e+02) "None" true)
  (Utilities|Time|SetTimerbyEvent (delegate Custom|Server%20Explode) (Variables|Default|GetTimeToExplode)))

(fn ConstructionScript)