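; Melee weapon hitbox actor that follows its instigating melee character's MeleeSpawn point each tick, pushed forward along the camera.
; Capsule and sphere overlaps are handled on the server, hitting each I_Damage actor once via a multicast-updated HitActors list.
; Hits apply two-handed-weapon point damage and trigger an impact sound, plus blood particles and camera shake for characters.
; Damage is credited to player controller 0, cached at BeginPlay, rather than the instigator's controller.
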(event OnComponentBeginOverlap(Sphere1)
  (params (OverlappedComponent :type Primitive%20Component%20Object%20Reference) (OtherActor :type Actor%20Object%20Reference) (OtherComp :type Primitive%20Component%20Object%20Reference) (OtherBodyIndex :type Integer) (bFromSweep :type Boolean) (SweepResult :type Hit%20Result%20Structure%20%28by%20ref%29))
  (CallFunction|CollisionOverlap OtherActor))

(event OnComponentBeginOverlap(Capsule)
  (params (OverlappedComponent :type Primitive%20Component%20Object%20Reference) (OtherActor :type Actor%20Object%20Reference) (OtherComp :type Primitive%20Component%20Object%20Reference) (OtherBodyIndex :type Integer) (bFromSweep :type Boolean) (SweepResult :type Hit%20Result%20Structure%20%28by%20ref%29))
  (CallFunction|CollisionOverlap OtherActor))

(event Custom|Server%20Apply%20Damage
  (params (DamagedActor :type Actor%20Object%20Reference) (Damage :type Float%20%28double-precision%29) (Hit%20Direction :type Vector) (Hit%20Info :type Hit%20Result%20Structure) (Instigated%20By :type Controller%20Object%20Reference) (DamageCauser :type Actor%20Object%20Reference) (Damage%20Type%20Class :type Damage%20Type%20Class%20Reference))
  (Default|ApplyPointDamage (Variables|Default|GetAs%20BP%20PC%20Mousen) DamagedActor Damage Hit%20Direction Hit%20Info Instigated%20By DamageCauser Damage%20Type%20Class))

(event Custom|Multicast%20Add%20Actor%20to%20Hit%20Actors
  (params (Hit%20Actor :type Actor%20Object%20Reference))
  (Utilities|Array|Add (Variables|Default|GetHitActors) Hit%20Actor))

(event Custom|Collision%20Overlap
  (params (Other%20Actor :type Actor%20Object%20Reference))
  (bind _returnvalue (Transformation|GetActorLocation Other%20Actor))
  (bind _capsule (Variables|Default|GetCapsule))
  (bind _returnvalue_2 (Transformation|GetWorldLocation _capsule))
  (bind _returnvalue_3 (- _returnvalue _returnvalue_2))
  (bind _returnvalue_4 (Math|Vector|Normalize _returnvalue_3))
  (if (Networking|IsServer)
    (if (Utilities|DoesObjectImplementInterface Other%20Actor "/Game/ThirdPerson/Blueprints/Gameplay/I_Damage.I_Damage_C")
      (if (!= Other%20Actor (Variables|Actor|GetInstigator))
        (if (not (Utilities|Array|ContainsItem (Variables|Default|GetHitActors) Other%20Actor))
          (CallFunction|ServerAddActortoHitActors Other%20Actor)
          (if (Utilities|DoesObjectImplementInterface Other%20Actor "/Game/ThirdPerson/Blueprints/I_Character.I_Character_C")
            (Class|ICharacter|PassWeaponParticleSystem(Message) Other%20Actor "/Game/ExternalFreeContent/Realistic_Starter_VFX_Pack_Vol2/Particles/Blood/P_Blood_Splat_Cone.P_Blood_Splat_Cone")
            (Class|IDamage|ShakeCamera(Message) (Variables|Default|GetAs%20BP%20Third%20Person%20Melee)))
          (CallFunction|ServerApplyDamage Other%20Actor (Variables|Default|GetDamage) _returnvalue_4 (Collision|MakeHitResult false false 0.0 0.0 "0, 0, 0" _returnvalue "0,0,1" _returnvalue_4 0 Other%20Actor) (Variables|Default|GetAs%20BP%20PC%20Mousen) (Variables|Actor|GetInstigator) "/Game/Objects/Weapons/DT_2HWeapon.DT_2HWeapon_C")
          (CallFunction|ServerSpawnBlockImpactSound))))))

(event Custom|Server%20Add%20Actor%20to%20Hit%20Actors
  (params (Hit%20Actor :type Actor%20Object%20Reference))
  (CallFunction|MulticastAddActortoHitActors Hit%20Actor))

(event Custom|Server%20Spawn%20Block%20Impact%20Sound
  (CallFunction|MSSpawnBlockImpactSound))

(event Custom|MS%20Spawn%20Block%20Impact%20Sound
  (Audio|SpawnSoundAttached "/Game/Sounds/Character/Melee/Block/MS_Block_Impact.MS_Block_Impact" (Variables|Default|GetCapsule) "None" "0, 0, 0" "0, 0, 0" "KeepRelativeOffset" false 1.0 1.0 0.0 0 0))

(event EventBeginPlay
  (bind _asbp_pc_mousen (Utilities|Casting|CastToBP_PC_Mousen (Game|GetPlayerController 0)))
  (Variables|Default|SetAs%20BP%20PC%20Mousen _asbp_pc_mousen)
  (bind _asbp_third_person_melee (Utilities|Casting|CastToBP_ThirdPerson_Melee (Variables|Actor|GetInstigator)))
  (Variables|Default|SetAs%20BP%20Third%20Person%20Melee _asbp_third_person_melee))

(event EventTick
  (params (DeltaSeconds :type Float%20%28single-precision%29))
  (bind _as_bp_third_person_melee (Variables|Default|GetAs%20BP%20Third%20Person%20Melee))
  (bind _meleespawn (Variables|/Game/ThirdPerson/Blueprints/Melee/BP_ThirdPerson_Melee.BP_ThirdPerson_Melee_C|GetMeleeSpawn _as_bp_third_person_melee))
  (bind _camera (Default|GetCamera _as_bp_third_person_melee))
  (Transformation|SetActorTransform self (Math|Transform|MakeTransform (+ (Transformation|GetWorldLocation _meleespawn) (* (Math|Vector|GetForwardVector _camera) 125.0)) (Transformation|GetWorldRotation _meleespawn) "1.000000,1.000000,1.000000")))

(fn ConstructionScript)