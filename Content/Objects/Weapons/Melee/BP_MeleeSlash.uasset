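; BP_MeleeSlash is a melee weapon slash actor that follows its owner's position and rotation.
; Each Tick it does a swept move to the owner's location plus a forward step of DistanceToMoveForward over TimeToMoveForward, scaled by delta time, and copies the owner's rotation.
; The step is re-applied from the owner's location each frame, so it does not accumulate and the slash stays just ahead of the owner.
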(event EventBeginPlay)

(event Collision|EventActorBeginOverlap
  (params (OtherActor :type Actor%20Object%20Reference)))

(event EventTick
  (params (DeltaSeconds :type Float%20%28single-precision%29))
  (bind _returnvalue (Components|GetOwner))
  (Transformation|SetActorLocationAndRotation (+ (Transformation|GetActorLocation _returnvalue) (* (Transformation|GetActorForwardVector) (* (/ (Variables|Default|GetDistanceToMoveForward) (Variables|Default|GetTimeToMoveForward)) DeltaSeconds))) (Transformation|GetActorRotation _returnvalue) true))

(fn ConstructionScript)