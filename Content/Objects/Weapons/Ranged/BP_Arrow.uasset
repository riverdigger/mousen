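; Arrow projectile for the Ranger that shows a brief trail on spawn, sticks into what it hits and deals ranged damage.
; On overlap with anything but its instigator it stops, attaches to the actor (characters at the neck_01 socket), then destroys itself after Lifetime.
; Targets implementing I_Damage take the Ranger's base weapon damage through player controller 0 (BP_PC_Mousen).
; Server-named events handle damage and relay the hit particle to a multicast-named event.
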(event OnComponentBeginOverlap(Capsule)
  (params (OverlappedComponent :type Primitive%20Component%20Object%20Reference) (OtherActor :type Actor%20Object%20Reference) (OtherComp :type Primitive%20Component%20Object%20Reference) (OtherBodyIndex :type Integer) (bFromSweep :type Boolean) (SweepResult :type Hit%20Result%20Structure%20%28by%20ref%29))
  (bind _projectilemovement (Variables|Default|GetProjectileMovement))
  ;[1 1 1] When Arrow hits, deal damage and attach the arrow to the target
  (if (!= OtherActor (Variables|Actor|GetInstigator))
    (Components|Movement|StopMovementImmediately _projectilemovement)
    (Variables|/Script/Engine.ProjectileMovementComponent|SetProjectileGravityScale _projectilemovement 0.0)
    (Collision|SetCollisionEnabled (Variables|Default|GetCapsule) "NoCollision")
    (bind _ascharacter (Utilities|Casting|CastToCharacter OtherActor)
      (:then
        (Transformation|AttachComponentToComponent (Variables|/Script/Engine.Character|GetMesh _ascharacter) "neck_01" "KeepWorld" "KeepWorld" "KeepWorld" true))
      (:CastFailed
        (Transformation|AttachActorToActor OtherActor "None" "KeepWorld" "KeepWorld" "KeepWorld" true)))
    (if (Utilities|DoesObjectImplementInterface OtherActor "/Game/ThirdPerson/Blueprints/Gameplay/I_Damage.I_Damage_C")
      (CallFunction|ServerApplyDamage :DamagedActor OtherActor :Damage (CallFunction|GetCurrentDamage) :Hit%20Direction (* (Math|Vector|Normalize (Math|Vector|GetForwardVector (Variables|Default|GetArrow))) "-1.000000,-1.000000,-1.000000") :Instigated%20By (Game|GetPlayerController 0) :DamageCauser (Variables|Actor|GetInstigator) :Damage%20Type%20Class "/Game/Objects/Weapons/Ranged/DT_Ranged.DT_Ranged_C"))
    (CallFunction|ServerSpawnCollisionEmitter)
    (Utilities|FlowControl|Delay (Variables|Default|GetLifetime))
    (Actor|DestroyActor)))

(event Custom|Server%20Apply%20Damage
  (params (DamagedActor :type Actor%20Object%20Reference) (Damage :type Float%20%28double-precision%29) (Hit%20Direction :type Vector) (Hit%20Info :type Hit%20Result%20Structure) (Instigated%20By :type Controller%20Object%20Reference) (DamageCauser :type Actor%20Object%20Reference) (Damage%20Type%20Class :type Damage%20Type%20Class%20Reference))
  (Default|ApplyPointDamage (Variables|Default|GetAs%20BP%20PC%20Mousen) DamagedActor Damage Hit%20Direction Hit%20Info Instigated%20By DamageCauser Damage%20Type%20Class))

(event Custom|Multicast%20Spawn%20Collision%20Emitter
  (Effects|SpawnEmitteratLocation "/Game/ExternalFreeContent/FXVarietyPack/Particles/P_ky_hit2.P_ky_hit2" (Transformation|GetWorldLocation (Variables|Default|GetCapsule)) "0, 0, 0" "0.200000,0.200000,0.200000"))

(event Custom|Server%20Spawn%20Collision%20Emitter
  (CallFunction|MulticastSpawnCollisionEmitter))

(event EventBeginPlay
  (bind _trail (Variables|Default|GetTrail))
  ;[1 1 1] Spawn Arrow and Set Owner and Effects
  (bind _asbp_pc_mousen (Utilities|Casting|CastToBP_PC_Mousen (Game|GetPlayerController 0)))
  (Variables|Default|SetAs%20BP%20PC%20Mousen _asbp_pc_mousen)
  (Effects|Particles|Trails|BeginTrails _trail "Trail1" "Trail2" "ETrailWidthMode_FromFirst" 5.0)
  (Utilities|FlowControl|Delay 0.2)
  (Effects|Particles|Trails|EndTrails _trail))

(fn ConstructionScript)

(fn GetCurrentDamage
  (return (.weaponbasedamage (Variables|/Game/ThirdPerson/Blueprints/Ranger/BP_ThirdPerson_Ranger.BP_ThirdPerson_Ranger_C|GetWeaponInfo (.AsBP%20Third%20Person%20Ranger (Utilities|Casting|CastToBP_ThirdPerson_Ranger (Variables|Actor|GetInstigator)))))))