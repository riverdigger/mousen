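; Overcharged arrow projectile that launches and pins the enemy it hits, dealing ranged point damage.
; On spawn it turns homing on from the shooter's auto-aimer flag and starts a lifespan timer.
; On overlap it stops; the server attaches it to non-teammate characters' pelvises, setting them flying, or to other actors.
; Damageable targets get a launch status along the last velocity; others get a multicast impact effect.
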(event OnComponentBeginOverlap(Box)
  (params (OverlappedComponent :type Primitive%20Component%20Object%20Reference) (OtherActor :type Actor%20Object%20Reference) (OtherComp :type Primitive%20Component%20Object%20Reference) (OtherBodyIndex :type Integer) (bFromSweep :type Boolean) (SweepResult :type Hit%20Result%20Structure%20%28by%20ref%29))
  (bind _returnvalue (Transformation|GetActorLocation))
  (bind _projectilemovement (Variables|Default|GetProjectileMovement))
  (bind (_x _y) (Math|Vector|BreakVector _returnvalue))
  ;[1 1 1] When Arrow hits, deal damage and attach the arrow to the target
  (if (!= OtherActor (Variables|Actor|GetInstigator))
    (CallFunction|ServerUpdateLastKnownVelocity (Variables|/Script/Engine.MovementComponent|GetVelocity (Variables|Default|GetProjectileMovement)))
    (Variables|Default|SetLastKnownVector (Transformation|GetActorForwardVector))
    (Components|Movement|StopMovementImmediately _projectilemovement)
    (Variables|/Script/Engine.ProjectileMovementComponent|SetProjectileGravityScale _projectilemovement 0.0)
    (Collision|SetCollisionEnabled (Variables|Default|GetBox) "NoCollision")
    (if (Networking|IsServer)
      (bind _ascharacter (Utilities|Casting|CastToCharacter OtherActor)
        (:then
          (if (Actor|ActorHasTag OtherActor (Utilities|Name|EnumtoName (Variables|/Game/ThirdPerson/Blueprints/Gameplay/BP_PS_Mousen.BP_PS_Mousen_C|GetPlayerTeam (.AsBP%20PS%20Mousen (Utilities|Casting|CastToBP_PS_Mousen (Variables|/Script/Engine.Pawn|GetPlayerState (Variables|Actor|GetInstigator)))))))
            _
            (else
              (Transformation|AttachComponentToComponent (Variables|/Script/Engine.Character|GetMesh _ascharacter) "pelvis" "SnapToTarget" "KeepWorld" "KeepWorld" true)
              (Pawn|Components|CharacterMovement|SetMovementMode (Variables|/Script/Engine.Character|GetCharacterMovement _ascharacter) "MOVE_Flying" 0)
              (if (Utilities|DoesObjectImplementInterface OtherActor "/Game/ThirdPerson/Blueprints/Gameplay/I_Damage.I_Damage_C") :!label _label
                (Class|IStatusLaunch|OnLaunch(Message) OtherActor "/Game/Spells/StatusEffects/Blueprints/BP_Status_Effect_Launched.BP_Status_Effect_Launched_C" (Variables|Default|GetLaunchLifetime) (* (Math|Vector|Normalize (Variables|Default|GetLastKnownVelocity)) 3e+03) true self)
                (Class|ICharacter|PassWeaponParticleSystem(Message) OtherActor "/Game/ExternalFreeContent/FXVarietyPack/Particles/P_ky_hit2.P_ky_hit2")
                (CallFunction|ServerApplyDamage OtherActor (Variables|Default|GetDamage) (* (Math|Vector|Normalize (Math|Vector|GetForwardVector (Variables|Default|GetArrow))) "-1.000000,-1.000000,-1.000000") (Collision|MakeHitResult false false 0.0 0.0 "0, 0, 0" (Math|Vector|MakeVector _x _y (.z (Transformation|GetActorLocation))) "0,0,1" (* (Math|Vector|Normalize (Transformation|GetActorForwardVector)) -1.0) 0 0) (Game|GetPlayerController 0) (Variables|Actor|GetInstigator) "/Game/Objects/Weapons/Ranged/DT_Ranged.DT_Ranged_C")
                (else
                  (CallFunction|ServerSpawnCollisionEmitter)))
              (Utilities|FlowControl|Delay (Variables|Default|GetLifetime)))))
        (:CastFailed
          (Transformation|AttachActorToActor OtherActor "None" "KeepWorld" "KeepWorld" "KeepWorld" true)
          (goto _label)))
      (Actor|DestroyActor))))

(event Custom|Server%20Apply%20Damage
  (params (DamagedActor :type Actor%20Object%20Reference) (Damage :type Float%20%28double-precision%29) (Hit%20Direction :type Vector) (Hit%20Info :type Hit%20Result%20Structure) (Instigated%20By :type Controller%20Object%20Reference) (DamageCauser :type Actor%20Object%20Reference) (Damage%20Type%20Class :type Damage%20Type%20Class%20Reference))
  (Default|ApplyPointDamage (Variables|Default|GetAs%20BP%20PC%20Mousen) DamagedActor Damage Hit%20Direction Hit%20Info Instigated%20By DamageCauser Damage%20Type%20Class))

(event Custom|Multicast%20Spawn%20Collision%20Emitter
  (Effects|SpawnEmitteratLocation "/Game/ExternalFreeContent/FXVarietyPack/Particles/P_ky_hit2.P_ky_hit2" (Transformation|GetWorldLocation (Variables|Default|GetBox)) "0, 0, 0" "0.200000,0.200000,0.200000"))

(event Custom|Server%20Spawn%20Collision%20Emitter
  (CallFunction|MulticastSpawnCollisionEmitter))

(event Custom|Break%20Self
  ;[1 1 1] Spawn Arrow and Set Owner and Effects
  (Actor|DestroyActor))

(event Custom|Server%20Update%20Last%20Known%20Velocity
  (params (LastKnownVelocity :type Vector))
  ;[1 1 1] When Arrow hits, deal damage and attach the arrow to the target
  (Variables|Default|SetLastKnownVelocity LastKnownVelocity))

(event EventBeginPlay
  ;[1 1 1] Spawn Arrow and Set Owner and Effects
  (bind _asbp_pc_mousen (Utilities|Casting|CastToBP_PC_Mousen (Game|GetPlayerController 0)))
  (Variables|Default|SetAs%20BP%20PC%20Mousen _asbp_pc_mousen)
  (bind _output_get (Variables|Default|SetAs%20BP%20PS%20Mousen (.AsBP%20PS%20Mousen (Utilities|Casting|CastToBP_PS_Mousen (Variables|/Script/Engine.Pawn|GetPlayerState (Variables|Actor|GetInstigator))))))
  (Variables|/Script/Engine.ProjectileMovementComponent|SetbIsHomingProjectile (Variables|Default|GetProjectileMovement) (Variables|/Game/ThirdPerson/Blueprints/Gameplay/BP_PS_Mousen.BP_PS_Mousen_C|GetHasAutoAimer? _output_get))
  (Utilities|Time|SetTimerbyEvent (delegate Custom|Break%20Self) (Variables|/Game/ThirdPerson/Blueprints/Gameplay/BP_PS_Mousen.BP_PS_Mousen_C|GetArrowLifespan (Variables|Default|GetAs%20BP%20PS%20Mousen))))

(fn ConstructionScript)