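; Vision arrow projectile for the Ranger that damages what it hits, sticks to it, then reveals nearby enemies.
; Player state sets starting gravity and homing, with gravity rising after a delay.
; A cone overlap picks an enemy homing target, and Tick stops homing once distance grows.
; On impact, an expanding sphere pulses, highlighting opposing-team characters before the arrow destroys itself; Hunter's Mark also highlights the struck enemy.
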(event OnComponentBeginOverlap(Box)
  (params (OverlappedComponent :type Primitive%20Component%20Object%20Reference) (OtherActor :type Actor%20Object%20Reference) (OtherComp :type Primitive%20Component%20Object%20Reference) (OtherBodyIndex :type Integer) (bFromSweep :type Boolean) (SweepResult :type Hit%20Result%20Structure%20%28by%20ref%29))
  (bind _returnvalue (Transformation|GetActorLocation OtherActor))
  (bind _projectilemovement (Variables|Default|GetProjectileMovement))
  (bind _instigator (Variables|Actor|GetInstigator))
  (bind _visionsphere (Variables|Default|GetVisionSphere))
  (bind (_x _y) (Class|KismetMathLibrary|BreakVector3f _returnvalue))
  (bind _playerstate (Variables|/Script/Engine.Pawn|GetPlayerState _instigator))
  (bind _asbp_ps_mousen (Utilities|Casting|CastToBP_PS_Mousen _playerstate))
  ;[1 1 1] When Arrow hits, deal damage and attach the arrow to the target
  (if (!= OtherActor (Variables|Actor|GetInstigator))
    (Components|Movement|StopMovementImmediately _projectilemovement)
    (Variables|/Script/Engine.ProjectileMovementComponent|SetProjectileGravityScale _projectilemovement 0.0)
    (Collision|SetCollisionEnabled (Variables|Default|GetBox) "NoCollision")
    (bind _ascharacter (Utilities|Casting|CastToCharacter OtherActor)
      (:then
        (Transformation|AttachComponentToComponent (Variables|/Script/Engine.Character|GetMesh _ascharacter) "neck_01" "KeepWorld" "KeepWorld" "KeepWorld" true))
      (:CastFailed
        (Transformation|AttachActorToActor OtherActor "None" "KeepWorld" "KeepWorld" "KeepWorld" true)))
    (if (Utilities|DoesObjectImplementInterface OtherActor "/Game/ThirdPerson/Blueprints/Gameplay/I_Damage.I_Damage_C")
      (Class|ICharacter|PassWeaponParticleSystem(Message) OtherActor "/Game/ExternalFreeContent/Realistic_Starter_VFX_Pack_Vol2/Particles/Blood/P_Blood_Splat_Cone.P_Blood_Splat_Cone")
      (CallFunction|ServerApplyDamage OtherActor (CallFunction|GetCurrentDamage) (* (Math|Vector|Normalize (Math|Vector|GetForwardVector (Variables|Default|GetArrow))) "-1.000000,-1.000000,-1.000000") (Collision|MakeHitResult false false 0.0 0.0 "0, 0, 0" (Math|Vector|MakeVector _x _y (.z (Transformation|GetActorLocation))) "0,0,1" (* (Math|Vector|Normalize (Transformation|GetActorForwardVector)) -1.0) 0 OtherActor) (Game|GetPlayerController 0) (Variables|Actor|GetInstigator) "/Game/Objects/Weapons/Ranged/DT_Ranged.DT_Ranged_C")
      (if (Variables|/Game/ThirdPerson/Blueprints/Gameplay/BP_PS_Mousen.BP_PS_Mousen_C|GetHasHuntersMark? _asbp_ps_mousen)
        (if (!= (Math|Conversions|ToInteger(Byte) (Variables|/Game/ThirdPerson/Blueprints/Gameplay/BP_PS_Mousen.BP_PS_Mousen_C|GetPlayerTeam _asbp_ps_mousen)) (Math|Conversions|ToInteger(Byte) (Variables|/Game/ThirdPerson/Blueprints/Gameplay/BP_PS_Mousen.BP_PS_Mousen_C|GetPlayerTeam (.AsBP%20PS%20Mousen (Utilities|Casting|CastToBP_PS_Mousen (Variables|/Script/Engine.Pawn|GetPlayerState (.AsBP%20Third%20Person%20Character (Utilities|Casting|CastToBP_ThirdPersonCharacter OtherActor))))))))
          (Class|IStatusSeen|OnSeen(Message) OtherActor 0 "/Game/Spells/FX/MI_Overlay.MI_Overlay" 4.0)))
      (else
        (CallFunction|ServerSpawnCollisionEmitter "/Game/ExternalFreeContent/FXVarietyPack/Particles/P_ky_hit2.P_ky_hit2" "0.200000,0.200000,0.200000")))
    (Collision|SetCollisionEnabled (Variables|Default|GetVisionSphere) "QueryAndPhysics")
    (bind _counter (Utilities|FlowControl|DoN (Variables|Default|GetPulses) :!label _label)
      (:Exit
        (bind _scale (Timeline|Pulse%20Timeline PlayFromStart)
          (:Update
            (Transformation|SetWorldScale3D _visionsphere (Math|Vector|Lerp(Vector) (Transformation|GetWorldScale _visionsphere) "75.000000,75.000000,75.000000" _scale)))
          (:Finished
            (if (<= _counter (- (Variables|Default|GetPulses) 1))
              (Transformation|SetWorldScale3D (Variables|Default|GetVisionSphere) "0, 0, 0")
              (Utilities|FlowControl|Delay 0.5)
              (goto _label)
              (else
                (Actor|DestroyActor)))))))))

(event OnComponentBeginOverlap(Cone)
  (params (OverlappedComponent :type Primitive%20Component%20Object%20Reference) (OtherActor :type Actor%20Object%20Reference) (OtherComp :type Primitive%20Component%20Object%20Reference) (OtherBodyIndex :type Integer) (bFromSweep :type Boolean) (SweepResult :type Hit%20Result%20Structure%20%28by%20ref%29))
  ;[1 1 1 1 80] Homing Missile
  (Utilities|IsValid (Variables|/Script/Engine.ProjectileMovementComponent|GetHomingTargetComponent (Variables|Default|GetProjectileMovement))
    (:Is%20Not%20Valid
      (if (Utilities|Enum|NotEqual(Enum) (Variables|/Game/ThirdPerson/Blueprints/Gameplay/BP_PS_Mousen.BP_PS_Mousen_C|GetPlayerTeam (.AsBP%20PS%20Mousen (Utilities|Casting|CastToBP_PS_Mousen (Variables|/Script/Engine.Pawn|GetPlayerState (.AsBP%20Third%20Person%20Character (Utilities|Casting|CastToBP_ThirdPersonCharacter OtherActor)))))) (Variables|/Game/ThirdPerson/Blueprints/Gameplay/BP_PS_Mousen.BP_PS_Mousen_C|GetPlayerTeam (Variables|Default|GetAs%20BP%20PS%20Mousen)))
        (if (!= OtherActor (Variables|Actor|GetInstigator))
          (Variables|/Script/Engine.ProjectileMovementComponent|SetHomingTargetComponent (Variables|Default|GetProjectileMovement) (Variables|/Script/Engine.Actor|GetRootComponent OtherActor)))))))

(event OnComponentBeginOverlap(VisionSphere)
  (params (OverlappedComponent :type Primitive%20Component%20Object%20Reference) (OtherActor :type Actor%20Object%20Reference) (OtherComp :type Primitive%20Component%20Object%20Reference) (OtherBodyIndex :type Integer) (bFromSweep :type Boolean) (SweepResult :type Hit%20Result%20Structure%20%28by%20ref%29))
  (if (!= (Math|Conversions|ToInteger(Byte) (Variables|/Game/ThirdPerson/Blueprints/Gameplay/BP_PS_Mousen.BP_PS_Mousen_C|GetPlayerTeam (.AsBP%20PS%20Mousen (Utilities|Casting|CastToBP_PS_Mousen (Variables|/Script/Engine.Pawn|GetPlayerState (Variables|Actor|GetInstigator)))))) (Math|Conversions|ToInteger(Byte) (Variables|/Game/ThirdPerson/Blueprints/Gameplay/BP_PS_Mousen.BP_PS_Mousen_C|GetPlayerTeam (.AsBP%20PS%20Mousen (Utilities|Casting|CastToBP_PS_Mousen (Variables|/Script/Engine.Pawn|GetPlayerState (.AsBP%20Third%20Person%20Character (Utilities|Casting|CastToBP_ThirdPersonCharacter OtherActor))))))))
    (Class|IStatusSeen|OnSeen(Message) OtherActor 0 "/Game/Spells/FX/MI_Overlay.MI_Overlay" 1.0)))

(event Custom|Server%20Apply%20Damage
  (params (DamagedActor :type Actor%20Object%20Reference) (Damage :type Float%20%28double-precision%29) (Hit%20Direction :type Vector) (Hit%20Info :type Hit%20Result%20Structure) (Instigated%20By :type Controller%20Object%20Reference) (DamageCauser :type Actor%20Object%20Reference) (Damage%20Type%20Class :type Damage%20Type%20Class%20Reference))
  (Default|ApplyPointDamage (Variables|Default|GetAs%20BP%20PC%20Mousen) DamagedActor Damage Hit%20Direction Hit%20Info Instigated%20By DamageCauser Damage%20Type%20Class))

(event Custom|Multicast%20Spawn%20Collision%20Emitter
  (params (EmitterTemplate :type Particle%20System%20Object%20Reference) (Scale :type Vector))
  (Effects|SpawnEmitteratLocation EmitterTemplate (Transformation|GetWorldLocation (Variables|Default|GetBox)) "0, 0, 0" Scale))

(event Custom|Server%20Spawn%20Collision%20Emitter
  (params (EmitterTemplate :type Particle%20System%20Object%20Reference) (Scale :type Vector))
  (CallFunction|MulticastSpawnCollisionEmitter EmitterTemplate Scale))

(event Custom|Change%20Gravity
  ;[1 1 1] Spawn Arrow and Set Owner and Effects
  (Variables|/Script/Engine.ProjectileMovementComponent|SetProjectileGravityScale (Variables|Default|GetProjectileMovement) 4.0))

(event EventBeginPlay
  ;[1 1 1] Spawn Arrow and Set Owner and Effects
  (Transformation|SetWorldScale3D (Variables|Default|GetVisionSphere) "0, 0, 0")
  (bind _asbp_pc_mousen (Utilities|Casting|CastToBP_PC_Mousen (Game|GetPlayerController 0)))
  (Variables|Default|SetAs%20BP%20PC%20Mousen _asbp_pc_mousen)
  (bind _output_get (Variables|Default|SetAs%20BP%20PS%20Mousen (.AsBP%20PS%20Mousen (Utilities|Casting|CastToBP_PS_Mousen (Variables|/Script/Engine.Pawn|GetPlayerState (Variables|Actor|GetInstigator))))))
  (Variables|/Script/Engine.ProjectileMovementComponent|SetbIsHomingProjectile (Variables|Default|GetProjectileMovement) (Variables|/Game/ThirdPerson/Blueprints/Gameplay/BP_PS_Mousen.BP_PS_Mousen_C|GetHasAutoAimer? _output_get))
  (bind _output_get_2 (Variables|/Script/Engine.ProjectileMovementComponent|SetProjectileGravityScale (Variables|Default|GetProjectileMovement) (Variables|/Game/ThirdPerson/Blueprints/Gameplay/BP_PS_Mousen.BP_PS_Mousen_C|GetArrowGravity (Variables|Default|GetAs%20BP%20PS%20Mousen))))
  (Utilities|Time|SetTimerbyEvent (delegate Custom|Change%20Gravity) (Math|Float|SelectFloat 0.4 0.8 (== _output_get_2 1.0))))

(event EventTick
  (params (DeltaSeconds :type Float%20%28single-precision%29))
  (bind _projectilemovement (Variables|Default|GetProjectileMovement))
  (bind _homingtargetcomponent (Variables|/Script/Engine.ProjectileMovementComponent|GetHomingTargetComponent _projectilemovement))
  ;[1 1 1 1 80] Homing Missile
  (Utilities|IsValid _homingtargetcomponent
    (:Is%20Valid
      (bind _output_get (Variables|Default|SetCurrentDistanceTo (Transformation|GetDistanceTo (Components|GetOwner _homingtargetcomponent))))
      (if (> (Variables|Default|GetCurrentDistanceTo) (Variables|Default|GetLastDistanceTo))
        (Variables|/Script/Engine.ProjectileMovementComponent|SetbIsHomingProjectile (Variables|Default|GetProjectileMovement) false)
        (else
          (Variables|Default|SetLastDistanceTo _output_get))))))

(fn ConstructionScript)

(fn GetCurrentDamage
  (return (.weaponbasedamage (Variables|/Game/ThirdPerson/Blueprints/Ranger/BP_ThirdPerson_Ranger.BP_ThirdPerson_Ranger_C|GetWeaponInfo (.AsBP%20Third%20Person%20Ranger (Utilities|Casting|CastToBP_ThirdPerson_Ranger (Variables|Actor|GetInstigator)))))))