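; Team flag for a capture-the-flag mode that opposing players pick up, carry and drop through instant interaction.
; Server-to-multicast events attach it to the carrier's spine socket or detach it; dropping enables physics with an impulse.
; While dropped away from its spawner, overlapping teammates and enemies drive FlagSpawner's reclaim and respawn timers, with enemies pausing both.
; A team-colored crystal bobs and rotates when unheld, alongside icon and timer widgets.
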(event OnComponentBeginOverlap(Cylinder)
  (params (OverlappedComponent :type Primitive%20Component%20Object%20Reference) (OtherActor :type Actor%20Object%20Reference) (OtherComp :type Primitive%20Component%20Object%20Reference) (OtherBodyIndex :type Integer) (bFromSweep :type Boolean) (SweepResult :type Hit%20Result%20Structure%20%28by%20ref%29))
  (bind _asbp_third_person_character (Utilities|Casting|CastToBP_ThirdPersonCharacter OtherActor))
  (Utilities|IsValid (Variables|Default|GetFlagSpawner)
    (:Is%20Valid
      (if (not (Variables|/Game/Objects/Flags/BP_FlagSpawner.BP_FlagSpawner_C|GetHasFlag? (Variables|Default|GetFlagSpawner)))
        (if (not (Variables|Default|GetIsHeld?))
          (if (Utilities|ClassIsChildOf (Utilities|GetClass OtherActor) "/Game/ThirdPerson/Blueprints/BP_ThirdPersonCharacter.BP_ThirdPersonCharacter_C")
            (if (not (Variables|/Game/ThirdPerson/Blueprints/Gameplay/BP_PS_Mousen.BP_PS_Mousen_C|GetIsPlayerDead? (.AsBP%20PS%20Mousen (Utilities|Casting|CastToBP_PS_Mousen (Variables|/Script/Engine.Pawn|GetPlayerState _asbp_third_person_character)))))
              (if (== (Math|Conversions|ToInteger(Byte) (Variables|Default|GetTeam)) (Variables|/Game/ThirdPerson/Blueprints/Gameplay/BP_PS_Mousen.BP_PS_Mousen_C|GetPlayerTeam (.AsBP%20PS%20Mousen (Utilities|Casting|CastToBP_PS_Mousen (Variables|/Script/Engine.Pawn|GetPlayerState _asbp_third_person_character)))))
                (Utilities|Array|AddUnique (Variables|Default|GetOverlappingTeammates) _asbp_third_person_character)
                (CallFunction|RecheckTimers)
                (else
                  (Utilities|Array|AddUnique (Variables|Default|GetOverlappingEnemies) _asbp_third_person_character)
                  (CallFunction|RecheckTimers)))
              (else
                (Utilities|Array|RemoveItem (Variables|Default|GetOverlappingTeammates) _asbp_third_person_character)
                (Utilities|Array|RemoveItem (Variables|Default|GetOverlappingEnemies) _asbp_third_person_character)
                (CallFunction|RecheckTimers)))))))))

(event OnComponentEndOverlap(Cylinder)
  (params (OverlappedComponent :type Primitive%20Component%20Object%20Reference) (OtherActor :type Actor%20Object%20Reference) (OtherComp :type Primitive%20Component%20Object%20Reference) (OtherBodyIndex :type Integer))
  (bind _asbp_third_person_character (Utilities|Casting|CastToBP_ThirdPersonCharacter OtherActor))
  (Utilities|IsValid (Variables|Default|GetFlagSpawner)
    (:Is%20Valid
      (if (not (Variables|/Game/Objects/Flags/BP_FlagSpawner.BP_FlagSpawner_C|GetHasFlag? (Variables|Default|GetFlagSpawner)))
        (if (not (Variables|Default|GetIsHeld?))
          (if (Utilities|ClassIsChildOf (Utilities|GetClass OtherActor) "/Game/ThirdPerson/Blueprints/BP_ThirdPersonCharacter.BP_ThirdPersonCharacter_C")
            (if (not (Variables|/Game/ThirdPerson/Blueprints/Gameplay/BP_PS_Mousen.BP_PS_Mousen_C|GetIsPlayerDead? (.AsBP%20PS%20Mousen (Utilities|Casting|CastToBP_PS_Mousen (Variables|/Script/Engine.Pawn|GetPlayerState _asbp_third_person_character)))))
              (if (== (Math|Conversions|ToInteger(Byte) (Variables|Default|GetTeam)) (Variables|/Game/ThirdPerson/Blueprints/Gameplay/BP_PS_Mousen.BP_PS_Mousen_C|GetPlayerTeam (.AsBP%20PS%20Mousen (Utilities|Casting|CastToBP_PS_Mousen (Variables|/Script/Engine.Pawn|GetPlayerState _asbp_third_person_character)))))
                (Utilities|Array|RemoveItem (Variables|Default|GetOverlappingTeammates) _asbp_third_person_character)
                (CallFunction|RecheckTimers)
                (else
                  (Utilities|Array|RemoveItem (Variables|Default|GetOverlappingEnemies) _asbp_third_person_character)
                  (CallFunction|RecheckTimers)))
              (else
                (Utilities|Array|RemoveItem (Variables|Default|GetOverlappingTeammates) _asbp_third_person_character)
                (Utilities|Array|RemoveItem (Variables|Default|GetOverlappingEnemies) _asbp_third_person_character)
                (CallFunction|RecheckTimers)))))))))

(event OnComponentBeginOverlap(InteractCylinder)
  (params (OverlappedComponent :type Primitive%20Component%20Object%20Reference) (OtherActor :type Actor%20Object%20Reference) (OtherComp :type Primitive%20Component%20Object%20Reference) (OtherBodyIndex :type Integer) (bFromSweep :type Boolean) (SweepResult :type Hit%20Result%20Structure%20%28by%20ref%29))
  (bind _asbp_third_person_character (Utilities|Casting|CastToBP_ThirdPersonCharacter OtherActor))
  (bind _can_interact (Default|CanInteract self _asbp_third_person_character))
  (if _can_interact
    (Utilities|IsValid (Pawn|GetLocalViewingPlayerController _asbp_third_person_character)
      (:Is%20Valid
        (if (Variables|Default|GetCanInteract?)
          (Default|ShowInteract (.AsBP%20HUD%20Mousen (Utilities|Casting|CastToBP_HUD_Mousen (HUD|GetHUD (Pawn|GetLocalViewingPlayerController _asbp_third_person_character)))) "0, 0, 0"))))))

(event OnComponentEndOverlap(InteractCylinder)
  (params (OverlappedComponent :type Primitive%20Component%20Object%20Reference) (OtherActor :type Actor%20Object%20Reference) (OtherComp :type Primitive%20Component%20Object%20Reference) (OtherBodyIndex :type Integer))
  (if (Variables|Default|GetCanInteract?)
    (bind _asbp_third_person_character (Utilities|Casting|CastToBP_ThirdPersonCharacter OtherActor))
    (Utilities|IsValid (Pawn|GetLocalViewingPlayerController _asbp_third_person_character)
      (:Is%20Valid
        (Default|HideInteract (.AsBP%20HUD%20Mousen (Utilities|Casting|CastToBP_HUD_Mousen (HUD|GetHUD (Pawn|GetLocalViewingPlayerController _asbp_third_person_character)))))))))

(event Custom|Recheck%20Timers
  (bind _flagspawner (Variables|Default|GetFlagSpawner))
  (bind _flagspawner_2 (Variables|Default|GetFlagSpawner))
  (bind _flagspawner_3 (Variables|Default|GetFlagSpawner))
  (if (<= (Class|KismetSystemLibrary|GetTimerElapsedTime _flagspawner "Respawn Flag") 0.0)
    (Default|CountdownRespawnFlag _flagspawner))
  (if (> (Utilities|Array|Length (Variables|Default|GetOverlappingTeammates)) 0)
    (if (> (Utilities|Array|Length (Variables|Default|GetOverlappingEnemies)) 0)
      (Default|PauseRespawnTimer _flagspawner_3)
      (Default|PauseReclaimTimer _flagspawner_3)
      (else
        (Default|CountdownReclaimFlag _flagspawner_3)
        (if (Class|KismetSystemLibrary|IsTimerPaused _flagspawner_3 "Respawn Flag")
          (Default|UnPauseRespawnTimer _flagspawner_3))))
    (elif (> (Utilities|Array|Length (Variables|Default|GetOverlappingEnemies)) 0)
      (Default|PauseRespawnTimer _flagspawner_2)
      (Default|PauseReclaimTimer _flagspawner_2)
      (Default|CancelReclaimFlag _flagspawner_2)
      (else
        (Default|CancelReclaimFlag _flagspawner_2)
        (if (Class|KismetSystemLibrary|IsTimerPaused _flagspawner_2 "Respawn Flag")
          (Default|UnPauseRespawnTimer _flagspawner_2))))))

(event Custom|Server%20Set%20Widget
  (CallFunction|MulticastSetWidget))

(event Custom|MC%20Update%20Zipliner
  (params (CanZipline? :type Boolean))
  (Variables|/Game/ThirdPerson/Blueprints/Gameplay/MapObjects/Zipline/AC_Zipliner.AC_Zipliner_C|SetCanZipline? (Variables|Default|GetAC_Zipliner) CanZipline?))

(event Custom|Server%20Update%20Zipliner
  (params (CanZipline? :type Boolean))
  (CallFunction|MCUpdateZipliner CanZipline?))

(event Custom|Multicast%20Pick%20Up%20Flag
  (params (ActorToAttach :type Actor%20Object%20Reference) (Parent :type Character%20Object%20Reference))
  (Transformation|AttachComponentToComponent (Variables|/Script/Engine.Character|GetMesh Parent) "spine_item" "SnapToTarget" "SnapToTarget" "KeepRelative" true)
  (Variables|Default|SetIsHeld? true)
  (Rendering|SetVisibility (Variables|Default|GetFlagIconWidget) false false)
  (Rendering|SetVisibility (Variables|Default|GetFlagTimerWidget) false false))

(event Custom|Server%20Pick%20Up%20Flag
  (params (Parent :type Character%20Object%20Reference))
  (CallFunction|MulticastPickUpFlag 0 Parent))

(event Custom|Server%20Update%20Can%20Interact
  (Variables|Default|SetCanInteract? true))

(event Custom|Server%20Reset%20Materials
  (CallFunction|MulticastResetMaterials))

(event Custom|Multicast%20Reset%20Materials
  (Rendering|Material|SetMaterial (Variables|Default|GetCrystalMesh) 0 "/Game/Objects/Flags/MI_Crystal_Base_White.MI_Crystal_Base_White")
  (Rendering|Material|SetVectorParameterValueonMaterials (Variables|Default|GetCrystalMesh) "Emissive Color" (Math|Conversions|ToVector(LinearColor) (Default|GetTeamUIColor (.AsBP%20PS%20Mousen (Utilities|Casting|CastToBP_PS_Mousen (Game|GetPlayerState 0))) (Variables|Default|GetTeam)))))

(event Custom|Multicast%20Set%20Widget
  (bind _output_get (Variables|Default|SetAs%20WB%20Flag%20Timer (.AsWB%20Flag%20Timer (Utilities|Casting|CastToWB_Flag_Timer (UserInterface|GetWidget (Variables|Default|GetFlagTimerWidget))))))
  (Default|UpdateTeam _output_get (Variables|Default|GetTeam)))

(event Custom|Server%20Drop%20Flag
  (CallFunction|MulticastDropFlag)
  (Utilities|Time|SetTimerbyEvent (delegate Custom|Server%20Update%20Can%20Interact) 0.5))

(event Custom|Settings%20Updated
  (CallFunction|ServerResetMaterials))

(event Custom|Bindings
  (EventDispatchers|BindEventtoSettingsSaved (.AsBP%20GI%20Mousen (Utilities|Casting|CastToBP_GI_Mousen (Game|GetGameInstance))) (delegate Custom|Settings%20Updated)))

(event Custom|Multicast%20Drop%20Flag
  (Transformation|DetachFromActor "KeepWorld" "KeepWorld" "KeepWorld")
  (Variables|Default|SetIsHeld? false)
  (Rendering|SetVisibility (Variables|Default|GetFlagIconWidget) true false)
  (Rendering|SetVisibility (Variables|Default|GetFlagTimerWidget) true false))

(event EventBeginPlay
  (Rendering|Components|Light|SetLightColor (Variables|Default|GetPointLight) (Default|GetTeamUIColor (.AsBP%20PS%20Mousen (Utilities|Casting|CastToBP_PS_Mousen (Game|GetPlayerState 0))) (Variables|Default|GetTeam)) true)
  (Components|StaticMesh|SetStaticMesh (Variables|Default|GetCrystalMesh) "/Game/DreamscapeSeries/DreamscapeTower/Meshes/Crystals/SM_Crystal_01_Red.SM_Crystal_01_Red")
  (CallFunction|ServerResetMaterials)
  (CallFunction|Bindings)
  (Components|StaticMesh|SetStaticMesh (Variables|Default|GetFlagMesh) "/Game/Fantastic_Village_Pack/meshes/props/deco/SM_PROP_flag_04.SM_PROP_flag_04")
  (Variables|/Game/ThirdPerson/UI/Widgets/Flag/WB_Flag_Icon.WB_Flag_Icon_C|SetTeam (.AsWB%20Flag%20Icon (Utilities|Casting|CastToWB_Flag_Icon (UserInterface|GetUserWidgetObject (Variables|Default|GetFlagIconWidget)))) (Variables|Default|GetTeam))
  (CallFunction|ServerSetWidget))

(event EventTick
  (params (DeltaSeconds :type Float%20%28single-precision%29))
  (bind _output_get (Variables|Default|SetRunningTime (+ DeltaSeconds (Variables|Default|GetRunningTime))))
  (if (not (Variables|Default|GetIsHeld?))
    (Transformation|SetRelativeLocationAndRotation (Variables|Default|GetCrystalMesh) (Math|Vector|Lerp(Vector) "0.000000,0.000000,160.000000" "0.000000,0.000000,120.000000" (+ (* (Math|Trig|Sin(Radians) _output_get) 0.5) 0.5)) (Math|Rotator|MakeRotator 0.0 0.0 (* (+ (* (Math|Trig|Sin(Radians) _output_get) 0.5) 0.5) 1.8e+02)) false false)
    (else
      (Transformation|SetRelativeLocationAndRotation (Variables|Default|GetCrystalMesh) "0, 0, 0" (Math|Rotator|MakeRotator 0.0 0.0 0.0) false false))))

(event EventTouchedKillZone
  (Default|ResetFlag (Variables|Default|GetFlagSpawner)))

(event EventInteract
  (params (Player :type Character%20Object%20Reference))
  (if (!= (Math|Conversions|ToInteger(Byte) (Variables|Default|GetTeam)) (Variables|/Game/ThirdPerson/Blueprints/Gameplay/BP_PS_Mousen.BP_PS_Mousen_C|GetPlayerTeam (.AsBP%20PS%20Mousen (Utilities|Casting|CastToBP_PS_Mousen (Variables|/Script/Engine.Pawn|GetPlayerState Player)))))
    (if (Variables|Default|GetIsHeld?)
      (CallFunction|DropFlag Player)
      (elif (Variables|Default|GetCanInteract?)
        (CallFunction|PickUpFlag Player)))))

(fn ConstructionScript)

(fn DropFlag
  (params (Character :type Character%20Object%20Reference))
  (bind _returnvalue (Components|GetOwner))
  (bind _flagmesh (Variables|Default|GetFlagMesh))
  (CallFunction|ServerUpdateZipliner true)
  (CallFunction|ServerDropFlag)
  (Collision|SetCollisionEnabled (Variables|Default|GetCylinder) "QueryOnly")
  (Collision|SetCollisionEnabled (Variables|Default|GetInteractCylinder) "QueryOnly")
  (Collision|SetCollisionResponsetoChannel (Variables|Default|GetCapsule) "ECC_GameTraceChannel3" "ECR_Overlap")
  (Physics|SetSimulatePhysics (Variables|Default|GetFlagMesh) true)
  (Physics|SetPhysicsLinearVelocity _flagmesh "0, 0, 0" false "None")
  (Physics|AddImpulse _flagmesh (* (Transformation|GetActorForwardVector _returnvalue) (* (Math|Float|Clamp(Float) (Math|Vector|VectorLength (Transformation|GetVelocity _returnvalue)) 0.0 3.0) 1e+02)) "None" true)
  (Default|ServerUpdateHeldFlag (.AsBP%20Third%20Person%20Character (Utilities|Casting|CastToBP_ThirdPersonCharacter Character)))
  (Rendering|SetVisibility (Variables|Default|GetFlagCircle) true false))

(fn PickUpFlag
  (params (Character :type Character%20Object%20Reference))
  (bind _flagspawner (Variables|Default|GetFlagSpawner))
  (CallFunction|ServerUpdateZipliner false)
  (Variables|Default|SetIsAway? true)
  (Variables|Default|SetCanInteract? false)
  (Default|ServerUpdateRatMode (.AsBP%20Third%20Person%20Character (Utilities|Casting|CastToBP_ThirdPersonCharacter Character)) false)
  (Rendering|SetVisibility (Variables|Default|GetFlagCircle) false false)
  (Physics|SetSimulatePhysics (Variables|Default|GetFlagMesh) false)
  (Collision|SetCollisionEnabled (Variables|Default|GetCylinder) "NoCollision")
  (Collision|SetCollisionEnabled (Variables|Default|GetInteractCylinder) "NoCollision")
  (Collision|SetCollisionResponsetoChannel (Variables|Default|GetCapsule) "ECC_GameTraceChannel3" "ECR_Ignore")
  (CallFunction|ServerPickUpFlag Character)
  (Default|CancelRespawnFlag _flagspawner)
  (Default|CancelReclaimFlag _flagspawner)
  (if (Variables|/Game/Objects/Flags/BP_FlagSpawner.BP_FlagSpawner_C|GetHasFlag? _flagspawner)
    (Default|ServerLowerGates _flagspawner))
  (Variables|/Game/Objects/Flags/BP_FlagSpawner.BP_FlagSpawner_C|SetHasFlag? _flagspawner false)
  (Default|ServerUpdateHeldFlag (.AsBP%20Third%20Person%20Character (Utilities|Casting|CastToBP_ThirdPersonCharacter Character)) self))

(fn CanInteract
  (params (Player%20Character :type Character%20Object%20Reference))
  (bind _asbp_third_person_character (Utilities|Casting|CastToBP_ThirdPersonCharacter Player%20Character))
  (bind _asbp_ps_mousen (Utilities|Casting|CastToBP_PS_Mousen (Variables|/Script/Engine.Pawn|GetPlayerState _asbp_third_person_character)))
  (if (Utilities|Enum|NotEqual(Enum) (Variables|/Game/ThirdPerson/Blueprints/Gameplay/BP_PS_Mousen.BP_PS_Mousen_C|GetPlayerTeam _asbp_ps_mousen) (Variables|Default|GetTeam))
    (return (or (Variables|Default|GetCanInteract?) (== Player%20Character (.AsCharacter (Utilities|Casting|CastToCharacter (Components|GetOwner))))))
    (else
      (return false))))

(fn GetInteractTimeSeconds
  (return 0.0 true))

(fn GetIsDead
  (return false))