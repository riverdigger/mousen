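; BP_FlagCapture is a team-owned capture zone that scores flag captures in a capture-the-flag mode.
; When a BP_ThirdPersonCharacter holding a flag overlaps its Cylinder, it checks that the player's team matches the zone's.
; It then scans all BP_Flag actors for the team's own flag, which must not be away.
; A valid capture respawns the carried flag through its spawner and awards points through BP_GM_Mousen.
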(event OnComponentBeginOverlap(Cylinder)
  (params (OverlappedComponent :type Primitive%20Component%20Object%20Reference) (OtherActor :type Actor%20Object%20Reference) (OtherComp :type Primitive%20Component%20Object%20Reference) (OtherBodyIndex :type Integer) (bFromSweep :type Boolean) (SweepResult :type Hit%20Result%20Structure%20%28by%20ref%29))
  (bind _asbp_third_person_character (Utilities|Casting|CastToBP_ThirdPersonCharacter OtherActor))
  (bind _heldflag (Variables|/Game/ThirdPerson/Blueprints/BP_ThirdPersonCharacter.BP_ThirdPersonCharacter_C|GetHeldFlag _asbp_third_person_character))
  (bind _playerstate (Variables|/Script/Engine.Pawn|GetPlayerState _asbp_third_person_character))
  (bind _asbp_ps_mousen (Utilities|Casting|CastToBP_PS_Mousen _playerstate))
  (bind _playerteam (Variables|/Game/ThirdPerson/Blueprints/Gameplay/BP_PS_Mousen.BP_PS_Mousen_C|GetPlayerTeam _asbp_ps_mousen))
  (if (Utilities|ClassIsChildOf (Utilities|GetClass OtherActor) "/Game/ThirdPerson/Blueprints/BP_ThirdPersonCharacter.BP_ThirdPersonCharacter_C")
    (Utilities|IsValid _heldflag
      (:Is%20Valid
        (if (== (Variables|Default|GetTeam) (Math|Conversions|ToInteger(Byte) _playerteam))
          ;[1 1 1] Can only capture when you flag is not away
          (bind _outactors (Actor|GetAllActorsOfClass "/Game/Objects/Flags/BP_Flag.BP_Flag_C"))
          (for _array_element _outactors
            (if (== (Variables|Default|GetTeam) (Math|Conversions|ToInteger(Byte) (Variables|/Game/Objects/Flags/BP_Flag.BP_Flag_C|GetTeam _array_element)))
              (if (not (Variables|/Game/Objects/Flags/BP_Flag.BP_Flag_C|GetIsAway? _array_element))
                (Default|RespawnFlag (Variables|/Game/Objects/Flags/BP_Flag.BP_Flag_C|GetFlagSpawner _heldflag))
                (Default|ScorePointsbyCaptures (.AsBP%20GM%20Mousen (Utilities|Casting|CastToBP_GM_Mousen (Game|GetGameMode))) _playerteam _asbp_ps_mousen)))))))))

(event EventBeginPlay)

(event Collision|EventActorBeginOverlap
  (params (OtherActor :type Actor%20Object%20Reference)))

(fn ConstructionScript)