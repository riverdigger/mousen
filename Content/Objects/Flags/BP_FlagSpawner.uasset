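; Team flag spawner for a capture-the-flag mode that spawns BP_Flag on the server and replaces it on respawn, reclaim or round change.
; Pausable, cancellable respawn and reclaim timers destroy the old flag, spawn a new one and raise the team's BP_Gate actors; round resets skip the gates.
; While either timer runs, server Tick multicasts both progress fractions to the flag's timer widget.
; ScorePoint is empty, with its capture logic disconnected.
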(event Custom|Server%20Update%20Respawn%20Widget
  (params (Outer%20Value :type Float%20%28double-precision%29) (Inner%20Value :type Float%20%28double-precision%29) (Team :type ENUM_Teams%20Enum :default "NewEnumerator4"))
  (CallFunction|MulticastUpdateRespawnWidget Outer%20Value Inner%20Value Team))

(event Custom|Cancel%20Reclaim%20Flag
  (Utilities|Time|ClearandInvalidateTimerbyHandle (Variables|Default|GetReclaim%20Timer)))

(event Custom|Reclaim%20Flag
  (bind _flag (Variables|Default|GetFlag))
  (bind _spawnlocation (Variables|Default|GetSpawnLocation))
  (bind _returnvalue (Transformation|GetWorldLocation _spawnlocation))
  (Utilities|Time|ClearandInvalidateTimerbyHandle (Variables|Default|GetRespawn%20Timer))
  (Utilities|Time|ClearandInvalidateTimerbyHandle (Variables|Default|GetReclaim%20Timer))
  (Utilities|IsValid _flag
    (:Is%20Valid
      (Actor|DestroyActor _flag))
    (:Is%20Not%20Valid
      _))
  (bind _returnvalue_2 (Game|SpawnActorfromClass "/Game/Objects/Flags/BP_Flag.BP_Flag_C" (Math|Transform|MakeTransform (Math|Vector|MakeVector (.x _returnvalue) (.y _returnvalue) (+ (.z _returnvalue) 75.0)) "0, 0, 0" "1.000000,1.000000,1.000000") "Undefined" "OverrideRootScale" 0 self (Variables|Default|GetTeam) 0))
  (Variables|Default|SetHasFlag? true)
  (CallFunction|MulticastSetFlag _returnvalue_2)
  (Variables|/Game/Objects/Flags/BP_Flag.BP_Flag_C|SetIsAway? _returnvalue_2 false)
  (CallFunction|ServerRaiseGates))

(event Custom|Pause%20Reclaim%20Timer
  (Utilities|Time|PauseTimerbyHandle (Variables|Default|GetReclaim%20Timer)))

(event Custom|UnPause%20Reclaim%20Timer
  (Utilities|Time|UnpauseTimerbyHandle (Variables|Default|GetReclaim%20Timer)))

(event Custom|UnPause%20Respawn%20Timer
  (Utilities|Time|UnpauseTimerbyHandle (Variables|Default|GetRespawn%20Timer)))

(event Custom|Pause%20Respawn%20Timer
  (Utilities|Time|PauseTimerbyHandle (Variables|Default|GetRespawn%20Timer)))

(event Custom|Reset%20Flag
  (bind _flag (Variables|Default|GetFlag))
  (bind _spawnlocation (Variables|Default|GetSpawnLocation))
  (bind _returnvalue (Transformation|GetWorldLocation _spawnlocation))
  (Utilities|Time|ClearandInvalidateTimerbyHandle (Variables|Default|GetRespawn%20Timer))
  (Utilities|Time|ClearandInvalidateTimerbyHandle (Variables|Default|GetReclaim%20Timer))
  (Utilities|IsValid _flag
    (:Is%20Valid
      (Actor|DestroyActor _flag))
    (:Is%20Not%20Valid
      _))
  (bind _returnvalue_2 (Game|SpawnActorfromClass "/Game/Objects/Flags/BP_Flag.BP_Flag_C" (Math|Transform|MakeTransform (Math|Vector|MakeVector (.x _returnvalue) (.y _returnvalue) (+ (.z _returnvalue) 75.0)) "0, 0, 0" "1.000000,1.000000,1.000000") "Undefined" "OverrideRootScale" 0 self (Variables|Default|GetTeam) 0))
  (Variables|Default|SetHasFlag? true)
  (CallFunction|MulticastSetFlag _returnvalue_2)
  (Variables|/Game/Objects/Flags/BP_Flag.BP_Flag_C|SetIsAway? _returnvalue_2 false))

(event Custom|Multicast%20Update%20Respawn%20Widget
  (params (Outer%20Value :type Float%20%28double-precision%29) (Innter%20Value :type Float%20%28double-precision%29) (Team :type ENUM_Teams%20Enum :default "NewEnumerator4"))
  (Default|UpdatePercent (Variables|/Game/Objects/Flags/BP_Flag.BP_Flag_C|GetAs%20WB%20Flag%20Timer (Variables|Default|GetFlag)) Outer%20Value Innter%20Value Team))

(event Custom|Countdown%20Reclaim%20Flag
  (Utilities|Time|ClearandInvalidateTimerbyHandle (Variables|Default|GetReclaim%20Timer))
  (bind _returnvalue (Utilities|Time|SetTimerbyEvent (delegate Custom|Reclaim%20Flag) (Variables|Default|GetReclaimTime)))
  (Variables|Default|SetReclaim%20Timer _returnvalue))

(event Custom|Multicast%20Set%20Flag
  (params (Flag :type BP%20Flag%20Object%20Reference))
  (Variables|Default|SetFlag Flag))

(event Custom|Countdown%20Respawn%20Flag
  (Utilities|Time|ClearandInvalidateTimerbyHandle (Variables|Default|GetRespawn%20Timer))
  (bind _returnvalue (Utilities|Time|SetTimerbyEvent (delegate Custom|Respawn%20Flag) (Variables|Default|GetRespawnTime)))
  (Variables|Default|SetRespawn%20Timer _returnvalue))

(event Custom|Cancel%20Respawn%20Flag
  (Utilities|Time|ClearandInvalidateTimerbyHandle (Variables|Default|GetRespawn%20Timer)))

(event Custom|Respawn%20Flag
  (bind _spawnlocation (Variables|Default|GetSpawnLocation))
  (bind _flag (Variables|Default|GetFlag))
  (bind _returnvalue (Transformation|GetWorldLocation _spawnlocation))
  (Utilities|Time|ClearandInvalidateTimerbyHandle (Variables|Default|GetRespawn%20Timer))
  (Utilities|Time|ClearandInvalidateTimerbyHandle (Variables|Default|GetReclaim%20Timer))
  (Utilities|IsValid _flag
    (:Is%20Valid
      (Actor|DestroyActor _flag))
    (:Is%20Not%20Valid
      _))
  (bind _returnvalue_2 (Game|SpawnActorfromClass "/Game/Objects/Flags/BP_Flag.BP_Flag_C" (Math|Transform|MakeTransform (Math|Vector|MakeVector (.x _returnvalue) (.y _returnvalue) (+ (.z _returnvalue) 75.0)) "0, 0, 0" "1.000000,1.000000,1.000000") "Undefined" "OverrideRootScale" 0 self (Variables|Default|GetTeam) 0))
  (Variables|Default|SetHasFlag? true)
  (CallFunction|MulticastSetFlag _returnvalue_2)
  (Variables|/Game/Objects/Flags/BP_Flag.BP_Flag_C|SetIsAway? _returnvalue_2 false)
  (CallFunction|ServerRaiseGates))

(event Custom|Server%20Lower%20Gates
  (bind _outactors (Actor|GetAllActorsOfClass "/Game/ThirdPerson/Maps/Environmental/Gate/BP_Gate.BP_Gate_C"))
  (for _array_element _outactors
    (if (Utilities|Enum|Equal(Enum) (Variables|/Game/ThirdPerson/Maps/Environmental/Gate/BP_Gate.BP_Gate_C|GetTeam _array_element) (Variables|Default|GetTeam))
      (Default|ServerLowerGate _array_element))))

(event Custom|Server%20Raise%20Gates
  (bind _outactors (Actor|GetAllActorsOfClass "/Game/ThirdPerson/Maps/Environmental/Gate/BP_Gate.BP_Gate_C"))
  (for _array_element _outactors
    (if (Utilities|Enum|Equal(Enum) (Variables|/Game/ThirdPerson/Maps/Environmental/Gate/BP_Gate.BP_Gate_C|GetTeam _array_element) (Variables|Default|GetTeam))
      (Default|ServerRaiseGate _array_element))))

(event EventBeginPlay
  (if (Networking|IsServer)
    (CallFunction|RespawnFlag)
    (EventDispatchers|BindEventtoGMMovetoNextRound (.AsBP%20GM%20Mousen (Utilities|Casting|CastToBP_GM_Mousen (Game|GetGameMode))) (delegate Custom|Reset%20Flag))))

(event EventTick
  (params (DeltaSeconds :type Float%20%28single-precision%29))
  (bind _respawn_timer (Variables|Default|GetRespawn%20Timer))
  (bind _reclaim_timer (Variables|Default|GetReclaim%20Timer))
  (if (Networking|IsServer)
    (if (or (Utilities|Time|IsTimerActivebyHandle _reclaim_timer) (Utilities|Time|IsTimerActivebyHandle _respawn_timer))
      (CallFunction|GetPercentages (Class|KismetSystemLibrary|GetTimerElapsedTimeHandle _respawn_timer) (Class|KismetSystemLibrary|GetTimerElapsedTimeHandle _reclaim_timer)))))

(fn ConstructionScript
  (Variables|Default|SetRespawnTimeRemaining (Variables|Default|GetRespawnTime)))

(fn ResetCountdown
  (Variables|Default|SetRespawnTimeRemaining (Variables|Default|GetRespawnTime)))

(fn ScorePoint
  (params (Flag :type %20Object%20Reference) (Player :type BP%20Third%20Person%20Character%20Object%20Reference)))

(fn GetRemainingRespawnTime
  (return (Utilities|Time|GetTimerRemainingTimebyHandle (Variables|Default|GetRespawn%20Timer))))

(fn GetRemainingReclaimTime
  (return (Utilities|Time|GetTimerRemainingTimebyHandle (Variables|Default|GetReclaim%20Timer))))

(fn GetPercentages
  (params (Outer%20Value :type Float%20%28double-precision%29) (Inner%20Value :type Float%20%28double-precision%29))
  (Utilities|FlowControl|Sequence
    (:then_0
      (if (Utilities|Time|IsTimerActivebyHandle (Variables|Default|GetRespawn%20Timer))
        (LocalVariables|SetOuter%20Percentage (/ Outer%20Value (Variables|Default|GetRespawnTime)))))
    (:then_1
      (if (Utilities|Time|IsTimerActivebyHandle (Variables|Default|GetReclaim%20Timer))
        (LocalVariables|SetInner%20Percentage (/ Inner%20Value (Variables|Default|GetReclaimTime)))))
    (:then_2
      (CallFunction|ServerUpdateRespawnWidget (LocalVariables|GetOuter%20Percentage) (LocalVariables|GetInner%20Percentage) (Variables|Default|GetTeam)))))