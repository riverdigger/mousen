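; BP_OnScreenWidget puts the Stylized Egypt Pack demo's controls hint on screen.
; On BeginPlay it creates WBP_Demo, adds it to the viewport and enables its own input through player controller 0.
; Hard-bound key events swap the widget's ControlsText: Gamepad Right Shoulder shows the gamepad controls, and Tab shows the mouse and keyboard controls.
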(event EventBeginPlay
  ;[0.05098 0.05098 0.05098] OnScreen Widget
  (bind _returnvalue (UserInterface|CreateWidget "/Game/StylizedEgyptPack/Widgets/WBP_Demo.WBP_Demo_C"))
  (bind _output_get (Variables|Default|SetControlsHintWidget _returnvalue))
  (UserInterface|Viewport|AddtoViewport _output_get 0)
  (Input|EnableInput (Game|GetPlayerController 0)))

(event Input|GamepadEvents|GamepadRightShoulder
  (params (Key :type Key%20Structure))
  ;[0.05098 0.05098 0.05098] Gamepad/Keyboard Controls Switch
  (:Pressed
    (Rendering|Components|TextRender|SetText (Variables|/Game/StylizedEgyptPack/Widgets/WBP_Demo.WBP_Demo_C|GetControlsText (Variables|Default|GetControlsHintWidget)) "Keyboard Tab Key - Show Mouse/Keyboard Controls 
 
Right Stick - Look Around 
Right Thumb Stick Button - Camera distance 
A - Jump / Swim Up 
B - Slow Down / Swim Down")))

(event Input|KeyboardEvents|Tab
  (params (Key :type Key%20Structure))
  ;[0.05098 0.05098 0.05098] Gamepad/Keyboard Controls Switch
  (:Pressed
    (Rendering|Components|TextRender|SetText (Variables|/Game/StylizedEgyptPack/Widgets/WBP_Demo.WBP_Demo_C|GetControlsText (Variables|Default|GetControlsHintWidget)) "Gamepad Right Shoulder - Show Gamepad Controls 
 
Mouse - Look Around 
Mouse Wheel - Camera distance 
Space - Jump / Swim Up 
L Ctrl - Slow Down / Swim Down")))

(fn ConstructionScript)