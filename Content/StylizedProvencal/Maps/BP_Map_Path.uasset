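; BP_Map_Path is a camera path actor in the StylizedProvencal maps that flies a camera along a spline in a continuous loop.
; Each Tick advances the distance by SplineSpeed times delta time and resets it to zero past the spline's end.
; The spline's location and rotation at that distance are sampled in world space but applied as the Camera's relative transform.
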(event EventBeginPlay)

(event Collision|EventActorBeginOverlap
  (params (OtherActor :type Actor%20Object%20Reference)))

(event EventTick
  (params (DeltaSeconds :type Float%20%28single-precision%29))
  (bind _output_get (Variables|Default|SetDistanceAlongSpline (+ (* DeltaSeconds (Variables|Default|GetSplineSpeed)) (Variables|Default|GetDistanceAlongSpline))))
  (if (> _output_get (Spline|GetSplineLength (Variables|Default|GetSpline)))
    (Variables|Default|SetDistanceAlongSpline 0.0))
  (Transformation|SetRelativeTransform (Variables|Default|GetCamera) (Math|Transform|MakeTransform (.location (Spline|GetTransformatDistanceAlongSpline (Variables|Default|GetSpline) (Variables|Default|GetDistanceAlongSpline) "World" false)) (.rotation (Spline|GetTransformatDistanceAlongSpline (Variables|Default|GetSpline) (Variables|Default|GetDistanceAlongSpline) "World" false)) "1.000000,1.000000,1.000000") false false))

(fn ConstructionScript)