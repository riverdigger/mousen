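; Rotating crystal actor that spins two crystal meshes every tick and changes its look when the post-round phase starts.
; On BeginPlay it casts the game mode to BP_GM_Mousen, retrying on a delay with a DoN-limited loop if that fails.
; It then binds to the GM's post-round event, which swaps the material on the first crystal mesh only.
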(event Custom|Server%20Add%20Bindings
  (EventDispatchers|BindEventtoGMStartPostRound (Variables|Default|GetAs%20BP%20GM%20Mousen) (delegate Custom|ChangeCrystalTextures)))

(event Custom|ChangeCrystalTextures
  (Rendering|Material|SetMaterial (Variables|Default|GetSM_crystal_01) 0 "/Game/Crystal_cave/Materials/MI_crystal_02.MI_crystal_02"))

(event EventBeginPlay
  (bind _returnvalue (Math|Float|Truncate 1e+01))
  ;[1 1 1] Make sure BP_GS_Mousen is valid on construct
  (Utilities|FlowControl|Sequence
    (:then_0
      (bind _asbp_gm_mousen (Utilities|Casting|CastToBP_GM_Mousen (Game|GetGameMode) :!label _label)
        (:then
          (Variables|Default|SetAs%20BP%20GM%20Mousen _asbp_gm_mousen)
          (CallFunction|ServerAddBindings))
        (:CastFailed
          (Utilities|FlowControl|Delay 1.0)
          (bind _counter (Utilities|FlowControl|DoN _returnvalue :!label _label_2)
            (:Exit
              (if (not (== _counter _returnvalue))
                (goto _label)))))))
    (:then_1
      (goto _label_2 Reset))))

(event EventTick
  (params (DeltaSeconds :type Float%20%28single-precision%29))
  (bind _delta_rotation (Variables|Default|GetDelta%20Rotation))
  (Transformation|AddLocalRotation (Variables|Default|GetSM_crystal_01) _delta_rotation false false)
  (Transformation|AddLocalRotation (Variables|Default|GetSM_crystal_02) _delta_rotation false false))

(event Collision|EventActorBeginOverlap
  (params (OtherActor :type Actor%20Object%20Reference)))

(fn ConstructionScript)