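; BP_Weather_Controller is a server-driven controller that picks a random weather ID between rounds.
; On BeginPlay the server casts the game mode to BP_GM_Mousen, with a delayed DoN retry path on failure, then binds to its round begin and end events.
; Round end randomizes WeatherID from five presets.
; StartWeather, bound to round start, and the WeatherID OnRep are empty stubs, so no weather is applied here.
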(event Custom|RandomizeWeather
  (Variables|Default|SetWeatherID (.OutItem (Utilities|Array|Random (Utilities|Array|MakeArray "Weather 1" "Weather 2" "Weather 3" "Weather 4" "Weather 5")))))

(event Custom|StartWeather)

(event Custom|Server%20Bind%20Rounds
  (EventDispatchers|BindEventtoGMBeginNewRound (Variables|Default|GetAs%20BP%20GM%20Mousen) (delegate Custom|StartWeather))
  (EventDispatchers|BindEventtoGMEndRound (Variables|Default|GetAs%20BP%20GM%20Mousen) (delegate Custom|RandomizeWeather)))

(event EventBeginPlay
  (bind _returnvalue (Math|Float|Truncate 0.0))
  (if (Networking|IsServer)
    (Utilities|FlowControl|Sequence
      (:then_0
        (bind _asbp_gm_mousen (Utilities|Casting|CastToBP_GM_Mousen (Game|GetGameMode) :!label _label)
          (:then
            (Variables|Default|SetAs%20BP%20GM%20Mousen _asbp_gm_mousen))
          (:CastFailed
            (Utilities|FlowControl|Delay 1.0)
            (bind _counter (Utilities|FlowControl|DoN _returnvalue :!label _label_2)
              (:Exit
                (if (== _counter _returnvalue)
                  (Variables|Default|SetAs%20BP%20GM%20Mousen 0)
                  (else
                    (goto _label)))))))
        (CallFunction|ServerBindRounds))
      (:then_1
        (goto _label_2 Reset)))))

(fn ConstructionScript)

(fn OnRepWeatherID)