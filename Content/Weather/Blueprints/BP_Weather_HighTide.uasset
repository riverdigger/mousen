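; High-tide weather effect that raises weather-affected damage zones while active.
; BeginPlay and CleanUp call server begin and end functions, with MCBeginEffect and MCEndEffect handling the changes.
; Begin moves each BP_DamageZone tagged AffectedByWeather to a fixed Z height, saving its transform in one shared variable.
; End applies that last saved transform to every tagged zone, then destroys the effect after a short delay.
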(event EventBeginPlay
  (CallFunction|ServerBeginEffect))

(event EventCleanUp
  (CallFunction|ServerEndEffect))

(event EventMCBeginEffect
  (bind _outactors (Actor|GetAllActorsOfClasswithTag "/Game/ThirdPerson/Maps/Environmental/BP_DamageZone.BP_DamageZone_C" "AffectedByWeather"))
  (for _array_element _outactors
    (bind _output_get (Variables|Default|SetOriginalTransform (Transformation|GetActorTransform _array_element)))
    (bind _output_get_2 (Variables|Default|SetNewTransform (Math|Transform|MakeTransform (Math|Vector|MakeVector (.x (.Location (Math|Transform|BreakTransform _output_get))) (.y (.Location (Math|Transform|BreakTransform _output_get))) 154.0) (.Rotation (Math|Transform|BreakTransform _output_get)) (.Scale (Math|Transform|BreakTransform _output_get)))))
    (Transformation|SetActorTransform _array_element _output_get_2)))

(event EventMCEndEffect
  (bind _outactors (Actor|GetAllActorsOfClasswithTag "/Game/ThirdPerson/Maps/Environmental/BP_DamageZone.BP_DamageZone_C" "AffectedByWeather"))
  (for _array_element _outactors
    (Transformation|SetActorTransform _array_element (Variables|Default|GetOriginalTransform)))
  (Utilities|FlowControl|Delay 0.2)
  (CallFunction|BeginDestroy))

(fn ConstructionScript
  (|CallParentFunction))